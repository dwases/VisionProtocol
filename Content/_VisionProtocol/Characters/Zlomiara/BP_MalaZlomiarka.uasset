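; Scripted NPC MalaZlomiarka, who moves along preset waypoints between conversations, opening with an in-motion monologue widget at BeginPlay.
; CheckStage finds the first unfinished stage, selects its dialogue table, runs its movement event and hides the two spinning marker meshes.
; Most stages use AIMoveTo; stages 3 and 6 lerp into a hole, then teleport onward.
; Arrival re-enables talking and shows the markers; waypoints derive from actor-relative offsets.
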(event `CheckStage`
  (bind _returnvalue (`KismetArrayLibrary.Array_Find` (`self.Stage`)))
  (switch `int` _returnvalue
    (:`Default`
      (set `self.Dialogue Ref` "/Game/_VisionProtocol/Core/DialogSystem/Dialogs/MalaZlomiarka/DT_MalaZlomiarkaDialog6.DT_MalaZlomiarkaDialog6"))
    (:`0`
      (set `self.Dialogue Ref` "/Game/_VisionProtocol/Core/DialogSystem/Dialogs/MalaZlomiarka/DT_MalaZlomiarkaMonolog2.DT_MalaZlomiarkaMonolog2")
      (`self.Stage 1` _returnvalue)
      (`SceneComponent.SetHiddenInGame` (`self.StaticMesh1`) true false :!label _label)
      (`SceneComponent.SetHiddenInGame` (`self.StaticMesh`) true false))
    (:`1`
      (set `self.Dialogue Ref` "/Game/_VisionProtocol/Core/DialogSystem/Dialogs/MalaZlomiarka/DT_MalaZlomiarkaDialog3.DT_MalaZlomiarkaDialog3")
      (`self.Stage 2` _returnvalue)
      (goto _label))
    (:`2`
      (set `self.Dialogue Ref` "/Game/_VisionProtocol/Core/DialogSystem/Dialogs/MalaZlomiarka/DT_MalaZlomiarkaMonolog3.DT_MalaZlomiarkaMonolog3")
      (`self.Stage 3` _returnvalue)
      (goto _label))
    (:`3`
      (set `self.Dialogue Ref` "/Game/_VisionProtocol/Core/DialogSystem/Dialogs/MalaZlomiarka/DT_MalaZlomiarkaDialog4.DT_MalaZlomiarkaDialog4")
      (`self.Stage 4` _returnvalue)
      (goto _label))
    (:`4`
      (set `self.Dialogue Ref` "/Game/_VisionProtocol/Core/DialogSystem/Dialogs/MalaZlomiarka/DT_MalaZlomiarkaDialog5.DT_MalaZlomiarkaDialog5")
      (`self.Stage 5` _returnvalue)
      (goto _label))
    (:`5`
      (set `self.Dialogue Ref` "/Game/_VisionProtocol/Core/DialogSystem/Dialogs/MalaZlomiarka/DT_MalaZlomiarkaDialog5.DT_MalaZlomiarkaDialog5")
      (`self.Stage 6` _returnvalue)
      (goto _label))
    (:`6`
      (set `self.Dialogue Ref` "/Game/_VisionProtocol/Core/DialogSystem/Dialogs/MalaZlomiarka/DT_MalaZlomiarkaDialog5.DT_MalaZlomiarkaDialog5")
      (`self.Stage 7` _returnvalue)
      (goto _label))))

(event `MoveTo`
  (bind _mesh (`self.Mesh`))
  (`SkeletalMeshComponent.PlayAnimation` _mesh "/Game/_VisionProtocol/Characters/Zlomiara/ZłomiaraRunning.ZłomiaraRunning" true)
  (`|AIMoveTo` self (`|GetArrayItem` (`self.WorldArrayLocations`) (`self.Current_I_Location`)) null 50.0
    (:`OnSuccess`
      (`/Engine/EditorBlueprintResources/StandardMacros.IncrementInt` (`self.Current_I_Location`)
        (:`  `
          (`SkeletalMeshComponent.Stop` _mesh)
          (`MovementComponent.StopMovementImmediately` (`self.CharacterMovement`))
          (set `self.IsReadyToSpeak` true)
          (`SceneComponent.SetHiddenInGame` (`self.StaticMesh1`) false false)
          (`SceneComponent.SetHiddenInGame` (`self.StaticMesh`) false false))))))

(event `Stage 3`
  (params (Index :type Integer))
  (`KismetSystemLibrary.Delay` 2.0) ; Czas, zanim wejdzie do dziury.
  (set `self.Base Location` (`self.K2_GetActorLocation`))
  (bind (_direction _1s) (`Timeline|Timeline_0` :!via `PlayFromStart`)
    (:`Update`
      (`self.K2_SetActorLocation` (`KismetMathLibrary.VLerp` (`self.Base Location`) (`|GetArrayItem` (`self.WorldArrayLocations`) (`self.Current_I_Location`)) _1s) false true))
    (:`Finished`
      (bind _result (`/Engine/EditorBlueprintResources/StandardMacros.IncrementInt` (`self.Current_I_Location`))
        (:`  `
          (`self.K2_SetActorLocation` (`|GetArrayItem` (`self.WorldArrayLocations`) _result) false true)
          (`/Engine/EditorBlueprintResources/StandardMacros.IncrementInt` (`self.Current_I_Location`)
            (:`  `
              (`KismetArrayLibrary.Array_Set` (`self.Stage`) Index true)
              (set `self.IsReadyToSpeak` true)
              (`SceneComponent.SetHiddenInGame` (`self.StaticMesh1`) false false)
              (`SceneComponent.SetHiddenInGame` (`self.StaticMesh`) false false))))))))

(event `Stage 1`
  (params (Index :type Integer))
  (`self.MoveTo`)
  (`KismetArrayLibrary.Array_Set` (`self.Stage`) Index true))

(event `JumpEvent`
  (set `self.Base Location` (`self.K2_GetActorLocation`))
  (bind (_direction _1_5s) (`Timeline|Timeline` :!via `PlayFromStart`)
    (:`Update`
      (`self.K2_SetActorLocation` (`KismetMathLibrary.VLerp` (`self.Base Location`) (`|GetArrayItem` (`self.WorldArrayLocations`) (`self.Current_I_Location`)) _1_5s) false true))
    (:`Finished`
      (`/Engine/EditorBlueprintResources/StandardMacros.IncrementInt` (`self.Current_I_Location`)))))

(event `Stage 2`
  (params (Index :type Integer))
  (`self.MoveTo`)
  (`KismetArrayLibrary.Array_Set` (`self.Stage`) Index true))

(event `Stage 4`
  (params (Index :type Integer))
  (`self.MoveTo`)
  (`KismetArrayLibrary.Array_Set` (`self.Stage`) Index true))

(event `Stage 5`
  (params (Index :type Integer))
  (`self.MoveTo`)
  (`KismetArrayLibrary.Array_Set` (`self.Stage`) Index true))

(event `Stage 6`
  (params (Index :type Integer))
  (`KismetSystemLibrary.Delay` 2.0) ; Czas, zanim wejdzie do dziury.
  (set `self.Base Location` (`self.K2_GetActorLocation`))
  (bind (_direction _1s) (`Timeline|Timeline_1` :!via `PlayFromStart`)
    (:`Update`
      (`self.K2_SetActorLocation` (`KismetMathLibrary.VLerp` (`self.Base Location`) (`|GetArrayItem` (`self.WorldArrayLocations`) (`self.Current_I_Location`)) _1s) false true))
    (:`Finished`
      (bind _result (`/Engine/EditorBlueprintResources/StandardMacros.IncrementInt` (`self.Current_I_Location`))
        (:`  `
          (`self.K2_SetActorLocation` (`|GetArrayItem` (`self.WorldArrayLocations`) _result) false true)
          (`/Engine/EditorBlueprintResources/StandardMacros.IncrementInt` (`self.Current_I_Location`)
            (:`  `
              (`KismetArrayLibrary.Array_Set` (`self.Stage`) Index true)
              (set `self.IsReadyToSpeak` true)
              (`SceneComponent.SetHiddenInGame` (`self.StaticMesh1`) false false)
              (`SceneComponent.SetHiddenInGame` (`self.StaticMesh`) false false))))))))

(event `self.ReceiveBeginPlay`
  (`parent.ReceiveBeginPlay`)
  (`self.RotateLogo`)
  (bind _returnvalue (`|CreateWidget` "/Game/_VisionProtocol/Widgets/Dialogues/WBP_DialogInMotion.WBP_DialogInMotion_C" (`GameplayStatics.GetPlayerController` 0) "/Game/_VisionProtocol/Core/DialogSystem/Dialogs/MalaZlomiarka/DT_MalaZlomiarkaMonolog1.DT_MalaZlomiarkaMonolog1"))
  (`UserWidget.AddToViewport` _returnvalue 0)
  (for _array_element (`self.RelativeArrayLocations`)
    (`KismetArrayLibrary.Array_Add` (`self.WorldArrayLocations`) (+ (`self.K2_GetActorLocation`) (`KismetMathLibrary.GreaterGreater_VectorRotator` _array_element (`self.K2_GetActorRotation`)))))
  (add `self.OnStartTalking` (`|CreateDelegate` :!event `CheckStage`))
  (for _ (`self.WorldArrayLocations`)
    (`KismetArrayLibrary.Array_Add` (`self.Stage`))))

(event `Stage 7`
  (params (Index :type Integer))
  (`self.MoveTo`)
  (`KismetArrayLibrary.Array_Set` (`self.Stage`) Index true)
  (`/Engine/EditorBlueprintResources/StandardMacros.IncrementInt` (`self.Current_I_Location`)))

(event `/Game/_VisionProtocol/Core/AI/BPI_Enemy.SpecialAttack1`)

(event `RotateLogo`
  (bind (_direction _newtrack_0) (`Timeline|Timeline_2` :!via `PlayFromStart`)
    (:`Update`
      (bind _returnvalue (* (struct :`Yaw` 360.0) _newtrack_0))
      (`SceneComponent.K2_SetRelativeRotation` (`self.StaticMesh`) _returnvalue false false)
      (`SceneComponent.K2_SetRelativeRotation` (`self.StaticMesh1`) (`KismetMathLibrary.MakeRotator` 0.0 0.0 (+ (.yaw _returnvalue) 180.0)) false false))
    (:`Finished`
      (`self.RotateLogo`))))

(fn `GetPatrolRoute`
  (returns (PatrolRoute :type "/Game/_VisionProtocol/Core/AI/BP_PatrolPath1 Object Reference"))
  (return null))

(fn `SetMovementSpeed`
  (params (Speed :type "/Game/_VisionProtocol/Core/AI/Enums/E_MovementSpeed Enum" :default "NewEnumerator0"))
  (returns (SpeedValue :type "Float (double-precision)"))
  (return 0.0))

(fn `UserConstructionScript`
  (`parent.UserConstructionScript`))
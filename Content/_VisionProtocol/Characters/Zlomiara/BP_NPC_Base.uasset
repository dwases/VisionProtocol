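; Base NPC Blueprint that lets the player talk to a character through a "Talk" interaction.
; Interact checks the DialogueRef row struct: monolog data opens a WBP_DialogInMotion widget, other data starts dialog on the interactor's BPC_DialogSystem.
; Both paths signal talk start, then restore IsReadyToSpeak immediately, except for BP_MalaZlomiarka, which stays unavailable.
; Combat, health, movement and patrol functions are empty stubs.
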(event `/Game/_VisionProtocol/Core/InteractionFramework/BPI_Interactable.Interact`
  (params (Interactor :type "Actor Object Reference") (InteracteeComponent :type "PrimitiveComponent Object Reference"))
  (bind _returnvalue (`self.GetComponentByClass` Interactor "/Game/_VisionProtocol/Core/DialogSystem/BPC_DialogSystem.BPC_DialogSystem_C"))
  (bind _dialogue_ref (`self.Dialogue Ref`))
  (if (`self.IsReadyToSpeak`)
    (set `self.IsReadyToSpeak` false)
    (if (`KismetStringLibrary.EqualEqual_StrStr` (`KismetSystemLibrary.GetDisplayName` (`DataTableFunctionLibrary.GetDataTableRowStruct` _dialogue_ref)) "ST_MonologData")
      (bind _returnvalue_2 (`|CreateWidget` "/Game/_VisionProtocol/Widgets/Dialogues/WBP_DialogInMotion.WBP_DialogInMotion_C" (`GameplayStatics.GetPlayerController` 0) _dialogue_ref))
      (`UserWidget.AddToViewport` _returnvalue_2 0)
      (`self.OnStartTalking`)
      (cast `/Game/_VisionProtocol/Characters/Zlomiara/BP_MalaZlomiarka` self
        (:`CastFailed`
          (set `self.IsReadyToSpeak` true)))
      (else
        (`/Engine/EditorBlueprintResources/StandardMacros.IsValid` _returnvalue
          (:`Is Valid`
            (`/Game/_VisionProtocol/Core/DialogSystem/BPC_DialogSystem.BeginDialog` _returnvalue _dialogue_ref)
            (`self.OnStartTalking`)
            (cast `/Game/_VisionProtocol/Characters/Zlomiara/BP_MalaZlomiarka` self
              (:`CastFailed`
                (set `self.IsReadyToSpeak` true)))))))))

(event `/Game/_VisionProtocol/Core/AI/BPI_Enemy.Attack1`)

(event `/Game/_VisionProtocol/Core/AI/BPI_Enemy.SpecialAttack1`)

(event `/Game/_VisionProtocol/Core/AI/BPI_Enemy.SpecialAttack2`)

(event `/Game/_VisionProtocol/Core/AI/BPI_Enemy.SpecialAttack3`)

(fn `GetCurrentHealth`
  (returns (Health :type "Float (double-precision)"))
  (return 0.0))

(fn `GetIdealRange`
  (returns (AttackRadius :type "Float (double-precision)") (DefenseRadius :type "Float (double-precision)"))
  (return 0.0 0.0))

(fn `GetInteractionName`
  (returns (InteractionName :type Text))
  (return "Talk"))

(fn `GetIsInteractKeyWidgetVisible`
  (returns (IsInteractKeyWidgetVisible :type Boolean))
  (return true))

(fn `GetLocation`
  (returns (Location :type "Vector Structure"))
  (return (0.0 0.0 0.0)))

(fn `GetMaxHealth`
  (returns (MaxHealth :type "Float (double-precision)"))
  (return 0.0))

(fn `GetPatrolRoute`
  (returns (PatrolRoute :type "/Game/_VisionProtocol/Core/AI/BP_PatrolPath1 Object Reference"))
  (return null))

(fn `Heal`
  (params (HP_Amount :type "Float (double-precision)"))
  (returns (`New Health` :type "Float (double-precision)"))
  (return 0.0))

(fn `IsDead`
  (returns (Dead :type Boolean))
  (return false))

(fn `SetMovementSpeed`
  (params (Speed :type "/Game/_VisionProtocol/Core/AI/Enums/E_MovementSpeed Enum" :default "NewEnumerator0"))
  (returns (SpeedValue :type "Float (double-precision)"))
  (return 0.0))

(fn `TakeDamage`
  (params (Amount :type "Float (double-precision)"))
  (returns (`Was Damaged` :type Boolean))
  (return false))

(fn `UserConstructionScript`
  (`parent.UserConstructionScript`))
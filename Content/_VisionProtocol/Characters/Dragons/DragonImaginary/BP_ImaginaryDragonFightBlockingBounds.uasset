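; Blocking box that bounds the Imaginary Dragon (BP_SmokUrojony) fight, with collision active from the dragon's start until its death.
; After a short delay on BeginPlay it finds the dragon, binds to its OnStart and OnDead events, and turns the box's collision off.
; OnStart enables query and physics collision, and OnDead disables it.
; A separate ToggleCollision function flips all channel responses between Block and Ignore but is not called here.
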(event `self.ReceiveBeginPlay`
  (`KismetSystemLibrary.Delay` 1.0)
  (bind _returnvalue (`GameplayStatics.GetActorOfClass` "/Game/_VisionProtocol/TestingPlayground/Filip/Urojony_Smok/BP_SmokUrojony.BP_SmokUrojony_C"))
  (`/Engine/EditorBlueprintResources/StandardMacros.IsValid` _returnvalue
    (:`Is Valid`
      (bind _output_get (set `self.Dragon` _returnvalue))
      (add `/Game/_VisionProtocol/TestingPlayground/Filip/Urojony_Smok/BP_SmokUrojony.OnStart` _output_get (delegate `EnableCollision`))
      (add `/Game/_VisionProtocol/TestingPlayground/Filip/Urojony_Smok/BP_SmokUrojony.OnDead` _output_get (delegate `DisableCollision`))
      (`PrimitiveComponent.SetCollisionEnabled` (`self.Box`) "NoCollision"))))

(event `EnableCollision`
  (`PrimitiveComponent.SetCollisionEnabled` (`self.Box`) "QueryAndPhysics"))

(event `DisableCollision`
  (`PrimitiveComponent.SetCollisionEnabled` (`self.Box`) "NoCollision"))

(fn `ToggleCollision`
  (if (`self.CollisionEnabled`)
    (`PrimitiveComponent.SetCollisionResponseToAllChannels` (`self.Box`) "ECR_Ignore")
    (set `self.CollisionEnabled` false)
    (else
      (`PrimitiveComponent.SetCollisionResponseToAllChannels` (`self.Box`) "ECR_Block")
      (set `self.CollisionEnabled` true))))

(fn `UserConstructionScript`)
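; BP_RobotCorpseEnd is an interactable robot corpse that shows a "Przeszukaj" (Search) prompt with a visible key widget.
; Its Interact event is empty, so interacting runs no logic in this Blueprint.
; A disconnected chain would show a rocket-boots popup, make the mesh ignore Visibility, add the DoubleJump gameplay tag to the player's parkour component and call HideLogo, but it never runs.
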(event `self.Interact`
  (params (Interactor :type "Actor Object Reference") (InteracteeComponent :type "PrimitiveComponent Object Reference")))

(fn `GetInteractionName`
  (returns (InteractionName :type Text))
  (return "Przeszukaj"))

(fn `GetIsInteractKeyWidgetVisible`
  (returns (IsInteractKeyWidgetVisible :type Boolean))
  (return true))

(fn `UserConstructionScript`)
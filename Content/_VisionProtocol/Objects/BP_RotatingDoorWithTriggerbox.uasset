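; A door Blueprint with a trigger box, named as a rotating door, that reacts once to the player character.
; The construction script places and sizes the Box from the TriggerboxLocation and BoxExtent variables.
; The first overlap by a BP_VPPlayerCharacter plays the TL_DoorMovementUp timeline from the start through a DoOnce.
; No timeline update is wired to move the door, and the Lerp and GetActorLocation nodes are unused.
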(event `self.Box.OnComponentBeginOverlap`
  (params (OverlappedComponent :type "PrimitiveComponent Object Reference") (OtherActor :type "Actor Object Reference") (OtherComp :type "PrimitiveComponent Object Reference") (OtherBodyIndex :type Integer) (bFromSweep :type Boolean) (SweepResult :type "HitResult Structure (by ref)"))
  (cast `/Game/_VisionProtocol/Core/BP_VPPlayerCharacter` OtherActor)
  (`/Engine/EditorBlueprintResources/StandardMacros.DoOnce` false
    (:`Completed`
      (bind (_direction _positionalpha) (`Timeline|TL_DoorMovementUp` :!via `PlayFromStart`)))))

(fn `UserConstructionScript`
  (`SceneComponent.K2_SetRelativeLocation` (`self.Box`) (`self.TriggerboxLocation`) false false)
  (`BoxComponent.SetBoxExtent` (`self.Box`) (`self.BoxExtent`) true))
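; BP_ExplosiveBarrel is an explosive barrel that detonates when damaged or interacted with.
; Positive damage triggers a sphere overlap that sends linearly falling-off, rounded damage to nearby actors, then fires a radial impulse, sound and particles before destroying itself.
; An IsExploding flag blocks re-entry, but is set even by non-positive damage.
; Interact only fires impulse and sound, then destroys the barrel; other health functions are stubs.
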(event `self.Interact`
  (params (Interactor :type "Actor Object Reference") (InteracteeComponent :type "PrimitiveComponent Object Reference"))
  (`RadialForceComponent.FireImpulse` (`self.RadialForce`))
  (`GameplayStatics.PlaySoundAtLocation` "/Game/StarterContent/Audio/Explosion_Cue.Explosion_Cue" (`self.K2_GetActorLocation`) (struct) 1.0 1.0 0.0 null null null null)
  (`self.K2_DestroyActor`))

(fn `GetCurrentHealth`
  (returns (Health :type "Float (double-precision)"))
  (return 0.0))

(fn `GetInteractionName`
  (returns (InteractionName :type Text))
  (return "EXPLODE!"))

(fn `GetMaxHealth`
  (returns (MaxHealth :type "Float (double-precision)"))
  (return 0.0))

(fn `Heal`
  (params (HP_Amount :type "Float (double-precision)"))
  (returns (`New Health` :type "Float (double-precision)"))
  (return 0.0))

(fn `IsDead`
  (returns (Dead :type Boolean))
  (return false))

(fn `TakeDamage`
  (params (Amount :type "Float (double-precision)"))
  (returns (`Was Damaged` :type Boolean))
  (bind _returnvalue (`self.K2_GetActorLocation`))
  (bind _returnvalue_2 (`self.K2_GetActorLocation`))
  (bind _explosionradius (`self.ExplosionRadius`))
  (if (not (`self.isExploding`))
    (set `self.isExploding` true)
    (if (> Amount 0.0)
      (bind _outactors (`KismetSystemLibrary.SphereOverlapActors` _returnvalue_2 (`self.ExplosionRadius`) (`|MakeArray` "ObjectTypeQuery1" "ObjectTypeQuery2" "ObjectTypeQuery3" "ObjectTypeQuery4" "ObjectTypeQuery6" "ObjectTypeQuery1" "ObjectTypeQuery5" "ObjectTypeQuery7" :!type "EObjectTypeQuery Enum") null (`|MakeArray` self :!type "Actor Object Reference")))
      (for _array_element _outactors
        (`/Engine/EditorBlueprintResources/StandardMacros.IsValid` _array_element
          (:`Is Valid`
            (bind _returnvalue_3 (`KismetMathLibrary.Conv_IntToDouble` (`KismetMathLibrary.Round` (* (`self.ExplosionDamage`) (`KismetMathLibrary.FClamp` (/ (- _explosionradius (`KismetMathLibrary.Vector_Distance` _returnvalue_2 (`self.K2_GetActorLocation` _array_element))) _explosionradius))))))
            (if (not (== _returnvalue_3 0.0))
              (message `/Game/_VisionProtocol/Core/DMG-HP/BPI_Damageable.TakeDamage` _array_element _returnvalue_3)))))
      (`RadialForceComponent.FireImpulse` (`self.RadialForce`))
      (`GameplayStatics.PlaySoundAtLocation` "/Game/StarterContent/Audio/Explosion_Cue.Explosion_Cue" _returnvalue (struct) 1.0 1.0 0.0 null null null null)
      (`GameplayStatics.SpawnEmitterAtLocation` "/Game/StarterContent/Particles/P_Explosion.P_Explosion" _returnvalue (struct) (5.0 5.0 5.0))
      (`self.K2_DestroyActor`)
      (return true)
      (else
        (return false)))))

(fn `UserConstructionScript`)
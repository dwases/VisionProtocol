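; BP_MechanicsUnlock is an interactable "Pick Up" actor that unlocks a player mechanic.
; On interact, a Visor flag selects between setting the character's visor unlock state and adding a gameplay tag to its parkour component.
; It then signals the unlock, pushes its notifications to the HUD pop-up widget and destroys itself.
; A self-restarting timeline continuously spins the logo widget until pickup.
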(event `RotateLogo`
  (bind (_direction _newtrack_0) (`Timeline|Timeline` :!via `PlayFromStart`)
    (:`Update`
      (`SceneComponent.K2_SetRelativeRotation` (`self.VPWidget`) (* (struct :`Yaw` 360.0) _newtrack_0) false false))
    (:`Finished`
      (`self.RotateLogo`))))

(event `self.ReceiveBeginPlay`
  (`self.RotateLogo`))

(event `/Game/_VisionProtocol/Core/InteractionFramework/BPI_Interactable.Interact`
  (params (Interactor :type "Actor Object Reference") (InteracteeComponent :type "PrimitiveComponent Object Reference"))
  (bind _asbp_vpplayer_character (cast `/Game/_VisionProtocol/Core/BP_VPPlayerCharacter` Interactor))
  (if (`self.Visor`)
    (set `/Game/_VisionProtocol/Core/Visors/C_Visors.IsVisorUnlocked` (`self.UnlockVisors`) (`/Game/_VisionProtocol/Core/BP_VPPlayerCharacter.C_Visors` _asbp_vpplayer_character))
    (else
      (`BlueprintGameplayTagLibrary.AddGameplayTag` (`/Game/_VisionProtocol/Core/Parkour/BP_CharacterParkourComponent.ParkourTags` (`/Game/_VisionProtocol/Core/BP_VPPlayerCharacter.BP_CharacterParkourComponent` _asbp_vpplayer_character)) (`self.AddGameplayTag`))))
  (`self.NewMechanicUnlocked`)
  (bind _asplayer_hud (cast `/Game/_VisionProtocol/Core/PlayerHUD` (`PlayerController.GetHUD` (`GameplayStatics.GetPlayerController` 0))))
  (for _array_element (`self.Notification`)
    (`/Game/_VisionProtocol/Widgets/Dialogues/WBP_PopUp.AddPopUp` (`/Game/_VisionProtocol/Core/PlayerHUD.PopUpWidget` _asplayer_hud) _array_element))
  (`self.K2_DestroyActor`))

(fn `GetInteractionName`
  (returns (InteractionName :type Text))
  (return "Pick Up"))

(fn `GetIsInteractKeyWidgetVisible`
  (returns (IsInteractKeyWidgetVisible :type Boolean))
  (return true))

(fn `UserConstructionScript`)
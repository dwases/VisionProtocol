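; BP_NewLevelBound is a level transition trigger that moves the player to another map.
; When BP_VPPlayerCharacter overlaps its Box, it gets the save struct from the player's BP_PlayerSaveLoadComponent and resets the stored transform to identity.
; It saves that synchronously through BP_GameInstance, then loads MapName with a "Start=" option carrying the PlayerStart value.
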(event `self.Box.OnComponentBeginOverlap`
  (params (OverlappedComponent :type "PrimitiveComponent Object Reference") (OtherActor :type "Actor Object Reference") (OtherComp :type "PrimitiveComponent Object Reference") (OtherBodyIndex :type Integer) (bFromSweep :type Boolean) (SweepResult :type "HitResult Structure (by ref)"))
  (bind _asbp_vpplayer_character (cast `/Game/_VisionProtocol/Core/BP_VPPlayerCharacter` OtherActor))
  (bind _asbp_game_instance (cast `/Game/_VisionProtocol/Core/SaveLoadSystem/BP_GameInstance` (`GameplayStatics.GetGameInstance`)))
  (bind _returnvalue (`self.GetComponentByClass` _asbp_vpplayer_character "/Game/_VisionProtocol/Core/SaveLoadSystem/BP_PlayerSaveLoadComponent.BP_PlayerSaveLoadComponent_C"))
  (`/Engine/EditorBlueprintResources/StandardMacros.IsValid` _returnvalue
    (:`Is Valid`
      (bind _playersave (`/Game/_VisionProtocol/Core/SaveLoadSystem/BP_PlayerSaveLoadComponent.GetPlayerSave` _returnvalue))
      (bind _newparam (`self.RestartTransform` _playersave))
      (`/Game/_VisionProtocol/Core/SaveLoadSystem/BPI_SaveGame.SavePlayer` _asbp_game_instance _newparam false)
      (`/Game/_VisionProtocol/Core/SaveLoadSystem/BP_GameInstance.LoadLevel` _asbp_game_instance (`self.Map Name`) (`KismetTextLibrary.Conv_TextToString` (`|FormatText` "Start={start}" (`self.PlayerStart`)))))))

(fn `RestartTransform`
  (params (NewParam1 :type "/Game/_VisionProtocol/Core/SaveLoadSystem/SPlayerSave2 Structure"))
  (returns (NewParam :type "/Game/_VisionProtocol/Core/SaveLoadSystem/SPlayerSave2 Structure"))
  (bind _structout (setmembers `/Game/_VisionProtocol/Core/SaveLoadSystem/SPlayerSave2` :`StructRef` NewParam1 :`Transform` (`KismetMathLibrary.MakeTransform` (0.0 0.0 0.0))))
  (return _structout))

(fn `UserConstructionScript`)
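; BP_RobotCorpse is a searchable robot corpse that tells the player, in Polish, that they found rocket boots for jumping in mid-air.
; Interact shows that message through the PlayerHUD pop-up widget and sets ConditionRobot on the first BP_PopUpTrigger found in the level.
; It then makes the mesh ignore the Visibility channel; the boots ability itself is not granted here.
; GetInteractionName supplies the "Przeszukaj" (Search) prompt.
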(event `/Game/_VisionProtocol/Core/InteractionFramework/BPI_Interactable.Interact`
  (params (Interactor :type "Actor Object Reference") (InteracteeComponent :type "PrimitiveComponent Object Reference"))
  (bind _asplayer_hud (cast `/Game/_VisionProtocol/Core/PlayerHUD` (`PlayerController.GetHUD` (`GameplayStatics.GetPlayerController` 0))))
  (`/Game/_VisionProtocol/Widgets/Dialogues/WBP_PopUp.AddPopUp` (`/Game/_VisionProtocol/Core/PlayerHUD.PopUpWidget` _asplayer_hud) "Gratulacje, zdobyłeś nową część – buty rakietowe. Pozwalają na skakanie w powietrzu.")
  (bind _returnvalue (`GameplayStatics.GetActorOfClass` "/Game/_VisionProtocol/Objects/BP_PopUpTrigger.BP_PopUpTrigger_C"))
  (set `/Game/_VisionProtocol/Objects/BP_PopUpTrigger.ConditionRobot` true _returnvalue)
  (`PrimitiveComponent.SetCollisionResponseToChannel` (`self.StaticMesh`) "ECC_Visibility" "ECR_Ignore"))

(fn `GetInteractionName`
  (returns (InteractionName :type Text))
  (return "Przeszukaj"))

(fn `UserConstructionScript`)
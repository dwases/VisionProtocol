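; BP_drabina is an interactable ladder that acts as a level transition.
; Its construction script stacks instanced mesh segments from Height and SegmentHeight, with query and physics collision.
; On Interact, it gets the player's save from BP_PlayerSaveLoadComponent, saves it synchronously through BP_GameInstance, then loads the NewMapName level.
; The interaction prompt reads "Use".
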(event `/Game/_VisionProtocol/Core/InteractionFramework/BPI_Interactable.Interact`
  (params (Interactor :type "Actor Object Reference") (InteracteeComponent :type "PrimitiveComponent Object Reference"))
  (bind _asbp_vpplayer_character (cast `/Game/_VisionProtocol/Core/BP_VPPlayerCharacter` Interactor))
  (bind _asbp_game_instance (cast `/Game/_VisionProtocol/Core/SaveLoadSystem/BP_GameInstance` (`GameplayStatics.GetGameInstance`)))
  (bind _returnvalue (`self.GetComponentByClass` _asbp_vpplayer_character "/Game/_VisionProtocol/Core/SaveLoadSystem/BP_PlayerSaveLoadComponent.BP_PlayerSaveLoadComponent_C"))
  (`/Engine/EditorBlueprintResources/StandardMacros.IsValid` _returnvalue
    (:`Is Valid`
      (bind _playersave (`/Game/_VisionProtocol/Core/SaveLoadSystem/BP_PlayerSaveLoadComponent.GetPlayerSave` _returnvalue))
      (`/Game/_VisionProtocol/Core/SaveLoadSystem/BPI_SaveGame.SavePlayer` _asbp_game_instance _playersave false)
      (`/Game/_VisionProtocol/Core/SaveLoadSystem/BP_GameInstance.LoadLevel` _asbp_game_instance (`self.NewMapName`)))))

(fn `GetInteractionName`
  (returns (InteractionName :type Text))
  (return "Use"))

(fn `UserConstructionScript`
  (bind _instancedstaticmesh (`self.InstancedStaticMesh`))
  (`InstancedStaticMeshComponent.ClearInstances` _instancedstaticmesh)
  (for _index (range (`self.Height`))
    (`InstancedStaticMeshComponent.AddInstance` _instancedstaticmesh (`KismetMathLibrary.Conv_VectorToTransform` (`KismetMathLibrary.MakeVector` 0.0 0.0 (* _index (`self.SegmentHeight`)))) false)
    (`PrimitiveComponent.SetCollisionEnabled` (`self.InstancedStaticMesh`) "QueryAndPhysics")
    (`PrimitiveComponent.SetCollisionEnabled` _instancedstaticmesh "QueryAndPhysics")))
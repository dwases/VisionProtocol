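; BP_RagingVortex is a Zero Dragon arena hazard that flings the player upward and damages them on contact.
; Static mesh hits launch BP_VPPlayerCharacter straight up with a very large velocity override, then apply fixed damage through BPI_Damageable.
; When ToDisappear is set, BeginPlay finds BP_SmokZerowy and binds to its OnDestroyed, so the vortex destroys itself along with that actor.
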(event `self.ReceiveBeginPlay`
  (if (`self.ToDisappear`)
    (bind _returnvalue (`GameplayStatics.GetActorOfClass` "/Game/_VisionProtocol/TestingPlayground/Filip/Zerowy_Smok/BP_SmokZerowy.BP_SmokZerowy_C"))
    (add `self.OnDestroyed` _returnvalue (delegate `DestroySelf`))))

(event `DestroySelf` :!signature `self.OnDestroyed`
  (params (DestroyedActor :type "Actor Object Reference"))
  (`self.K2_DestroyActor`))

(event `self.StaticMeshComponent.OnComponentHit`
  (params (HitComponent :type "PrimitiveComponent Object Reference") (OtherActor :type "Actor Object Reference") (OtherComp :type "PrimitiveComponent Object Reference") (NormalImpulse :type "Vector Structure") (Hit :type "HitResult Structure (by ref)"))
  (bind _asbp_vpplayer_character (cast `/Game/_VisionProtocol/Core/BP_VPPlayerCharacter` OtherActor))
  (`Character.LaunchCharacter` _asbp_vpplayer_character (0.0 0.0 45000.0) true true)
  (bind _asbpi_damageable (cast `/Game/_VisionProtocol/Core/DMG-HP/BPI_Damageable` OtherActor))
  (`/Game/_VisionProtocol/Core/DMG-HP/BPI_Damageable.TakeDamage` _asbpi_damageable 20.0))

(fn `UserConstructionScript`)
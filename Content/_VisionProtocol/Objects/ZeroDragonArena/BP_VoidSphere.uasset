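; BP_VoidSphere is a boundary for the Zero Dragon arena that keeps the player inside a large spherical radius.
; On Tick it measures and prints the player's distance from the sphere mesh's center.
; At or beyond the hard-coded radius, it launches the player toward the center and applies damage through BPI_Damageable.
; The check uses distance rather than collision; overlap and hit events are empty, and an older launch chain is disconnected.
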(event `self.StaticMeshComponent.OnComponentEndOverlap`
  (params (OverlappedComponent :type "PrimitiveComponent Object Reference") (OtherActor :type "Actor Object Reference") (OtherComp :type "PrimitiveComponent Object Reference") (OtherBodyIndex :type Integer)))

(event `self.StaticMeshComponent.OnComponentHit`
  (params (HitComponent :type "PrimitiveComponent Object Reference") (OtherActor :type "Actor Object Reference") (OtherComp :type "PrimitiveComponent Object Reference") (NormalImpulse :type "Vector Structure") (Hit :type "HitResult Structure (by ref)")))

(event `self.ReceiveTick`
  (params (DeltaSeconds :type "Float (single-precision)"))
  (bind _returnvalue (`SceneComponent.K2_GetComponentLocation` (`self.StaticMeshComponent`)))
  (bind _asbp_vpplayer_character (cast `/Game/_VisionProtocol/Core/BP_VPPlayerCharacter` (`GameplayStatics.GetPlayerPawn` 0)))
  (bind _returnvalue_2 (`self.K2_GetActorLocation` _asbp_vpplayer_character))
  (bind _returnvalue_3 (`KismetMathLibrary.Vector_Distance` _returnvalue_2 _returnvalue))
  (`KismetSystemLibrary.PrintString` (`KismetStringLibrary.Conv_DoubleToString` _returnvalue_3))
  (if (>= _returnvalue_3 49748.0)
    (`Character.LaunchCharacter` _asbp_vpplayer_character (* (`KismetMathLibrary.Normal` (- _returnvalue _returnvalue_2)) 45000.0) true true)
    (bind _asbpi_damageable (cast `/Game/_VisionProtocol/Core/DMG-HP/BPI_Damageable` _asbp_vpplayer_character))
    (`/Game/_VisionProtocol/Core/DMG-HP/BPI_Damageable.TakeDamage` _asbpi_damageable 15.0)))

(fn `UserConstructionScript`)
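; Elevator platform with a child pressure plate that sends it along its target locations and back, alternating on each accepted trigger.
; Construction places the plate at ButtonLocation; on BeginPlay it stays attached or detaches via ButtonFollow, and is destroyed if at zero offset.
; The plate's interaction event starts forward or reverse movement only for ActorToActivate while the elevator is idle.
; The stopped event clears the running flag.
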(event `self.ReceiveBeginPlay`
  (bind _pressureplate (`self.PressurePlate`))
  (if (not (`self.ButtonFollow`))
    (bind _asbp_pressure_plate (cast `/Game/_VisionProtocol/Objects/BP_PressurePlate` (`ChildActorComponent.ChildActor` (`self.PressurePlate`))))
    (`self.K2_DetachFromActor` _asbp_pressure_plate "KeepWorld" "KeepWorld" "KeepWorld"))
  (add `self.OnStopped` (delegate `ElevatorStopped`))
  (set `self.BaseLocation` (`SceneComponent.K2_GetComponentLocation` (`self.DefaultSceneRoot`)))
  (bind _asbp_pressure_plate_2 (cast `/Game/_VisionProtocol/Objects/BP_PressurePlate` (`ChildActorComponent.ChildActor` (`self.PressurePlate`))))
  (add `/Game/_VisionProtocol/Objects/BP_PressurePlate.OnInteracted` _asbp_pressure_plate_2 (delegate `ActivateMovement`))
  (if (== (`SceneComponent.RelativeLocation` _pressureplate) (0.0 0.0 0.0))
    (`self.K2_DestroyActor` (`ChildActorComponent.ChildActor` _pressureplate))))

(event `ActivateMovement`
  (params (Interactor :type "Actor Object Reference"))
  (if (== Interactor (`self.ActorToActivate`))
    (`KismetSystemLibrary.PrintString` "Hello")
    (if (`self.IsRunning`)
      (`KismetSystemLibrary.PrintString` "Winda jest w trakcie jazdy")
      (else
        (if (`self.AtBeggining`)
          (`self.Move` 0)
          (set `self.AtBeggining` false)
          (set `self.IsRunning` true)
          (else
            (`self.MoveReverse` (- (`KismetArrayLibrary.Array_Length` (`self.TargetLocations`)) 1))
            (set `self.AtBeggining` true)
            (set `self.IsRunning` true)))
        (if (`self.ButtonFollow`)
          _)))))

(event `ElevatorStopped`
  (set `self.IsRunning` false))

(fn `UserConstructionScript`
  (`parent.UserConstructionScript`)
  (`SceneComponent.K2_SetRelativeLocation` (`self.PressurePlate`) (`self.ButtonLocation`) false false))
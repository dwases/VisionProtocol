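; BP_ElevatorPlatform is an elevator platform that a child-actor BP_ElevatorButton sends back and forth along target locations.
; Button interaction, ignored while running, alternates Move and MoveReverse, and the stopped event clears the running flag.
; Construction positions the button from ButtonLocation; at start it detaches unless ButtonFollow is set, and is destroyed if its relative location is zero.
; Debug prints remain in the activation event.
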(event `self.ReceiveBeginPlay`
  (bind _activationbutton (`self.ActivationButton`))
  (if (not (`self.ButtonFollow`))
    (bind _asbp_elevator_button (cast `/Game/_VisionProtocol/Objects/BP_ElevatorButton` (`ChildActorComponent.ChildActor` (`self.ActivationButton`))))
    (`self.K2_DetachFromActor` _asbp_elevator_button "KeepWorld" "KeepWorld" "KeepWorld"))
  (add `self.OnStopped` (delegate `ElevatorStopped`))
  (set `self.BaseLocation` (`SceneComponent.K2_GetComponentLocation` (`self.DefaultSceneRoot`)))
  (bind _asbp_elevator_button_2 (cast `/Game/_VisionProtocol/Objects/BP_ElevatorButton` (`ChildActorComponent.ChildActor` (`self.ActivationButton`))))
  (add `/Game/_VisionProtocol/Objects/BP_ElevatorButton.OnInteracted` _asbp_elevator_button_2 (delegate `ActivateMovement`))
  (if (== (`SceneComponent.RelativeLocation` _activationbutton) (0.0 0.0 0.0))
    (`self.K2_DestroyActor` (`ChildActorComponent.ChildActor` _activationbutton))))

(event `ActivateMovement`
  (params (Interactor :type "Actor Object Reference"))
  (`KismetSystemLibrary.PrintString` "Hello")
  (if (`self.IsRunning`)
    (`KismetSystemLibrary.PrintString` "Winda jest w trakcie jazdy")
    (else
      (if (`self.AtBeggining`)
        (`self.Move` 0)
        (set `self.AtBeggining` false)
        (set `self.IsRunning` true)
        (else
          (`self.MoveReverse` (- (`KismetArrayLibrary.Array_Length` (`self.TargetLocations`)) 1))
          (set `self.AtBeggining` true)
          (set `self.IsRunning` true)))
      (if (`self.ButtonFollow`)
        _))))

(event `ElevatorStopped`
  (set `self.IsRunning` false))

(fn `UserConstructionScript`
  (`parent.UserConstructionScript`)
  (`SceneComponent.K2_SetRelativeLocation` (`self.ActivationButton`) (`self.ButtonLocation`) false false))
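; One-arm factory press hazard: the upper plate closes on the lower and kills the player when a second press overlap occurs while CanKill is set.
; Four chained timelines wait, close, wait and open, moving PressUp and listed attached actors with sound cues.
; Timeline play rates derive from durations, scale down for visor slow, and drop to zero on power off.
; Loop setup and start are unwired, so Poweron never starts the cycle.
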(event `self.PressUp.OnComponentBeginOverlap`
  (params (OverlappedComponent :type "PrimitiveComponent Object Reference") (OtherActor :type "Actor Object Reference") (OtherComp :type "PrimitiveComponent Object Reference") (OtherBodyIndex :type Integer) (bFromSweep :type Boolean) (SweepResult :type "HitResult Structure (by ref)"))
  ;[1 1 1] Kill Mechanic
  (bind _asbp_vpplayer_character (cast `/Game/_VisionProtocol/Core/BP_VPPlayerCharacter` OtherActor))
  (`/Engine/EditorBlueprintResources/StandardMacros.IsValid` _asbp_vpplayer_character
    (:`Is Valid`
      (if (`self.KillTrigger`)
        (if (`self.CanKill`)
          (`/Game/_VisionProtocol/Core/DMG-HP/C_DMG-HP.TakeDamage` (`/Game/_VisionProtocol/Core/BP_VPPlayerCharacter.C_DMG-HP` _asbp_vpplayer_character) 1000000.0))
        (else
          (set `self.KillTrigger` true))))))

(event `self.PressDown.OnComponentBeginOverlap`
  (params (OverlappedComponent :type "PrimitiveComponent Object Reference") (OtherActor :type "Actor Object Reference") (OtherComp :type "PrimitiveComponent Object Reference") (OtherBodyIndex :type Integer) (bFromSweep :type Boolean) (SweepResult :type "HitResult Structure (by ref)"))
  ;[1 1 1] Kill Mechanic
  (bind _asbp_vpplayer_character (cast `/Game/_VisionProtocol/Core/BP_VPPlayerCharacter` OtherActor))
  (`/Engine/EditorBlueprintResources/StandardMacros.IsValid` _asbp_vpplayer_character
    (:`Is Valid`
      (if (`self.KillTrigger`)
        (if (`self.CanKill`)
          (`/Game/_VisionProtocol/Core/DMG-HP/C_DMG-HP.TakeDamage` (`/Game/_VisionProtocol/Core/BP_VPPlayerCharacter.C_DMG-HP` _asbp_vpplayer_character) 1000000.0))
        (else
          (set `self.KillTrigger` true))))))

(event `self.PressUp.OnComponentEndOverlap`
  (params (OverlappedComponent :type "PrimitiveComponent Object Reference") (OtherActor :type "Actor Object Reference") (OtherComp :type "PrimitiveComponent Object Reference") (OtherBodyIndex :type Integer))
  ;[1 1 1] Kill Mechanic
  (bind _asbp_vpplayer_character (cast `/Game/_VisionProtocol/Core/BP_VPPlayerCharacter` OtherActor))
  (`/Engine/EditorBlueprintResources/StandardMacros.IsValid` _asbp_vpplayer_character
    (:`Is Valid`
      (if (`self.KillTrigger`) :!label _label
        (set `self.KillTrigger` false)
        (else
          (`KismetSystemLibrary.PrintString` "ERROR  - Press collision"))))))

(event `self.PressDown.OnComponentEndOverlap`
  (params (OverlappedComponent :type "PrimitiveComponent Object Reference") (OtherActor :type "Actor Object Reference") (OtherComp :type "PrimitiveComponent Object Reference") (OtherBodyIndex :type Integer))
  ;[1 1 1] Kill Mechanic
  (bind _asbp_vpplayer_character (cast `/Game/_VisionProtocol/Core/BP_VPPlayerCharacter` OtherActor))
  (`/Engine/EditorBlueprintResources/StandardMacros.IsValid` _asbp_vpplayer_character
    (:`Is Valid`
      (goto _label))))

(event `self.Power On`
  (`self.NormalSpeed`)
  (`/Engine/EditorBlueprintResources/StandardMacros.DoOnce` false
    (:`Completed`
      (`GameplayStatics.PlaySoundAtLocation` "/Game/_VisionProtocol/Audio/SFX/NewSFX/shotgun.shotgun" (`self.K2_GetActorLocation`) (struct) 0.3 0.6 0.0 "/Game/_VisionProtocol/Audio/BasicSoundAttenuation.BasicSoundAttenuation" null null null)
      (`KismetSystemLibrary.Delay` (`self.SpawnDelay`))
      ;[1 1 1] Save start position
      (set `self.StartLocationUp` (`SceneComponent.RelativeLocation` (`self.PressUp`))))))

(event `PressLoop`
  (bind _wait1 (`self.Wait1`))
  (bind _close2 (`self.Close2`))
  (bind _wait3 (`self.Wait3`))
  (bind _open4 (`self.Open4`))
  (bind _startlocationup (`self.StartLocationUp`))
  (bind _startlocationup_2 (`self.StartLocationUp`))
  (bind _returnvalue (`KismetMathLibrary.MultiplyMultiply_FloatFloat` (`self.CloseDuration`) -1.0))
  (bind _returnvalue_2 (`KismetMathLibrary.MultiplyMultiply_FloatFloat` (`self.BeforeOpenDelay`) -1.0))
  (bind _returnvalue_3 (`KismetMathLibrary.MultiplyMultiply_FloatFloat` (`self.BeforeCloseDelay`) -1.0))
  (bind _returnvalue_4 (`KismetMathLibrary.MultiplyMultiply_FloatFloat` (`self.OpenDuration`) -1.0))
  (if (not (`self.ActivelySlowed`))
    (`TimelineComponent.SetPlayRate` _wait1 _returnvalue_3)
    (`Timeline|Wait1` :!via `PlayFromStart` :!label _label_2
      (:`Finished`
        (if (not (`self.ActivelySlowed`))
          (`TimelineComponent.SetPlayRate` _close2 _returnvalue)
          (bind (_direction _open_animation) (`Timeline|Close2` :!via `PlayFromStart` :!label _label_3)
            (:`Update`
              (`SceneComponent.K2_SetRelativeLocation` (`self.PressUp`) (`KismetMathLibrary.VLerp` _startlocationup_2 (- _startlocationup_2 (`KismetMathLibrary.MakeVector` 0.0 0.0 (`self.DistanceFromCenter`))) _open_animation) false false)
              (for (_array_element _array_index) (`self.PressUpObjectList`)
                (`/Engine/EditorBlueprintResources/StandardMacros.IsValid` _array_element
                  (:`Is Valid`
                    (bind _output (`|GetArrayItem` (`self.PressUpLocations`) _array_index))
                    (`self.K2_SetActorLocation` _array_element (`KismetMathLibrary.VLerp` _output (- _output (`KismetMathLibrary.GreaterGreater_VectorRotator` (`KismetMathLibrary.MakeVector` 0.0 0.0 (`self.DistanceFromCenter`)) (`self.K2_GetActorRotation`))) _open_animation) false false)))))
            (:`Finished`
              (`GameplayStatics.PlaySoundAtLocation` "/Game/_VisionProtocol/Audio/SFX/explosion.explosion" (`self.K2_GetActorLocation`) (struct) 1.0 0.5 0.0 "/Game/_VisionProtocol/Audio/BasicSoundAttenuation.BasicSoundAttenuation" null null null)
              (if (not (`self.ActivelySlowed`))
                (`TimelineComponent.SetPlayRate` _wait3 _returnvalue_2)
                (`Timeline|Wait3` :!via `PlayFromStart` :!label _label_4
                  (:`Finished`
                    (if (not (`self.ActivelySlowed`))
                      (`TimelineComponent.SetPlayRate` _open4 _returnvalue_4)
                      (else
                        (`TimelineComponent.SetPlayRate` _open4 (/ _returnvalue_4 (`self.SlowStrength`)))))
                    (`GameplayStatics.PlaySoundAtLocation` null (`self.K2_GetActorLocation`) (struct) 1.0 1.0 0.0 null null null null)
                    (bind (_direction_2 _close_animation) (`Timeline|Open4` :!via `PlayFromStart`)
                      (:`Update`
                        (`SceneComponent.K2_SetRelativeLocation` (`self.PressUp`) (`KismetMathLibrary.VLerp` (- _startlocationup (`KismetMathLibrary.MakeVector` 0.0 0.0 (`self.DistanceFromCenter`))) _startlocationup _close_animation) false false)
                        (for (_array_element_2 _array_index_2) (`self.PressUpObjectList`)
                          (`/Engine/EditorBlueprintResources/StandardMacros.IsValid` _array_element_2
                            (:`Is Valid`
                              (bind _output_2 (`|GetArrayItem` (`self.PressUpLocations`) _array_index_2))
                              (`self.K2_SetActorLocation` _array_element_2 (`KismetMathLibrary.VLerp` (- _output_2 (`KismetMathLibrary.GreaterGreater_VectorRotator` (`KismetMathLibrary.MakeVector` 0.0 0.0 (`self.DistanceFromCenter`)) (`self.K2_GetActorRotation`))) _output_2 _close_animation) false false)))))
                      (:`Finished`
                        (`self.OnLoopEnd`)))))
                (else
                  (`TimelineComponent.SetPlayRate` _wait3 (/ _returnvalue_2 (`self.SlowStrength`)))
                  (goto _label_4 :!via `PlayFromStart`)))))
          (else
            (`TimelineComponent.SetPlayRate` _close2 (/ _returnvalue (`self.SlowStrength`)))
            (goto _label_3 :!via `PlayFromStart`)))))
    (else
      (`TimelineComponent.SetPlayRate` _wait1 (/ _returnvalue_3 (`self.SlowStrength`)))
      (goto _label_2 :!via `PlayFromStart`))))

(event `SlowDown`
  (`TimelineComponent.SetPlayRate` (`self.Wait1`) (/ (`KismetMathLibrary.MultiplyMultiply_FloatFloat` (`self.BeforeCloseDelay`) -1.0) (`self.SlowStrength`)))
  (`TimelineComponent.SetPlayRate` (`self.Close2`) (/ (`KismetMathLibrary.MultiplyMultiply_FloatFloat` (`self.CloseDuration`) -1.0) (`self.SlowStrength`)))
  (`TimelineComponent.SetPlayRate` (`self.Wait3`) (/ (`KismetMathLibrary.MultiplyMultiply_FloatFloat` (`self.BeforeOpenDelay`) -1.0) (`self.SlowStrength`)))
  (`TimelineComponent.SetPlayRate` (`self.Open4`) (/ (`KismetMathLibrary.MultiplyMultiply_FloatFloat` (`self.OpenDuration`) -1.0) (`self.SlowStrength`))))

(event `VisorSlowActivated`
  (params (SlowDown :type Boolean))
  (if SlowDown
    (if (not (`self.ActivelySlowed`))
      (set `self.ActivelySlowed` true)
      (`self.SlowDown`))
    (elif (`self.ActivelySlowed`)
      (set `self.ActivelySlowed` false)
      (`self.NormalSpeed`))))

(event `NormalSpeed`
  (`TimelineComponent.SetPlayRate` (`self.Wait1`) (`KismetMathLibrary.MultiplyMultiply_FloatFloat` (`self.BeforeCloseDelay`) -1.0))
  (`TimelineComponent.SetPlayRate` (`self.Close2`) (`KismetMathLibrary.MultiplyMultiply_FloatFloat` (`self.CloseDuration`) -1.0))
  (`TimelineComponent.SetPlayRate` (`self.Wait3`) (`KismetMathLibrary.MultiplyMultiply_FloatFloat` (`self.BeforeOpenDelay`) -1.0))
  (`TimelineComponent.SetPlayRate` (`self.Open4`) (`KismetMathLibrary.MultiplyMultiply_FloatFloat` (`self.OpenDuration`) -1.0)))

(event `self.Power Off`
  (`TimelineComponent.SetPlayRate` (`self.Wait1`) 0.0)
  (`TimelineComponent.SetPlayRate` (`self.Close2`) 0.0)
  (`TimelineComponent.SetPlayRate` (`self.Wait3`) 0.0)
  (`TimelineComponent.SetPlayRate` (`self.Open4`) 0.0))

(fn `UserConstructionScript`)
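; BP_PressControlSwitch is an interactable switch that toggles power for a set of factory machines.
; On Interact it sends PowerOff or PowerOn through BPI_Powerable to each entry in ControlledMashines, based on its PowerIsOn flag, then inverts that flag.
; Its interaction prompt reads "Power off" or "Power on" to match the flag, and the interact key widget is always visible.
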(event `/Game/_VisionProtocol/Core/InteractionFramework/BPI_Interactable.Interact`
  (params (Interactor :type "Actor Object Reference") (InteracteeComponent :type "PrimitiveComponent Object Reference"))
  (for _array_element (`self.ControlledMashines`)
    (bind _asbpi_powerable (cast `/Game/_VisionProtocol/Objects/Factory/BPI_Powerable` _array_element))
    (if (`self.PowerIsOn`)
      (`/Game/_VisionProtocol/Objects/Factory/BPI_Powerable.Power Off` _asbpi_powerable)
      (else
        (`/Game/_VisionProtocol/Objects/Factory/BPI_Powerable.Power On` _asbpi_powerable))))
  (set `self.PowerIsOn` (not (`self.PowerIsOn`))))

(fn `GetInteractionName`
  (returns (InteractionName :type Text))
  (if (`self.PowerIsOn`)
    (return "Power off")
    (else
      (return "Power on"))))

(fn `GetIsInteractKeyWidgetVisible`
  (returns (IsInteractKeyWidgetVisible :type Boolean))
  (return true))

(fn `UserConstructionScript`)
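; Broken one-arm factory press hazard that jams shut until shot with a reverse bullet, killing players caught in its two press colliders while lethal.
; Power-on starts timelines that lower the upper arm and its linked actors together.
; A BP_ReverseBullet hit on a linked actor reopens it, then it holds and slams shut again.
; Visor slow scales timeline play rates; power-off freezes them.
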(event `self.PressUp.OnComponentBeginOverlap`
  (params (OverlappedComponent :type "PrimitiveComponent Object Reference") (OtherActor :type "Actor Object Reference") (OtherComp :type "PrimitiveComponent Object Reference") (OtherBodyIndex :type Integer) (bFromSweep :type Boolean) (SweepResult :type "HitResult Structure (by ref)"))
  ;[1 1 1] Kill Mechanic
  (bind _asbp_vpplayer_character (cast `/Game/_VisionProtocol/Core/BP_VPPlayerCharacter` OtherActor))
  (`/Engine/EditorBlueprintResources/StandardMacros.IsValid` _asbp_vpplayer_character
    (:`Is Valid`
      (if (`self.KillTrigger`)
        (if (`self.CanKill`)
          (`/Game/_VisionProtocol/Core/DMG-HP/C_DMG-HP.TakeDamage` (`/Game/_VisionProtocol/Core/BP_VPPlayerCharacter.C_DMG-HP` _asbp_vpplayer_character) 1000000.0))
        (else
          (set `self.KillTrigger` true))))))

(event `self.PressDown.OnComponentBeginOverlap`
  (params (OverlappedComponent :type "PrimitiveComponent Object Reference") (OtherActor :type "Actor Object Reference") (OtherComp :type "PrimitiveComponent Object Reference") (OtherBodyIndex :type Integer) (bFromSweep :type Boolean) (SweepResult :type "HitResult Structure (by ref)"))
  ;[1 1 1] Kill Mechanic
  (bind _asbp_vpplayer_character (cast `/Game/_VisionProtocol/Core/BP_VPPlayerCharacter` OtherActor))
  (`/Engine/EditorBlueprintResources/StandardMacros.IsValid` _asbp_vpplayer_character
    (:`Is Valid`
      (if (`self.KillTrigger`)
        (if (`self.CanKill`)
          (`/Game/_VisionProtocol/Core/DMG-HP/C_DMG-HP.TakeDamage` (`/Game/_VisionProtocol/Core/BP_VPPlayerCharacter.C_DMG-HP` _asbp_vpplayer_character) 1000000.0))
        (else
          (set `self.KillTrigger` true))))))

(event `self.PressUp.OnComponentEndOverlap`
  (params (OverlappedComponent :type "PrimitiveComponent Object Reference") (OtherActor :type "Actor Object Reference") (OtherComp :type "PrimitiveComponent Object Reference") (OtherBodyIndex :type Integer))
  ;[1 1 1] Kill Mechanic
  (bind _asbp_vpplayer_character (cast `/Game/_VisionProtocol/Core/BP_VPPlayerCharacter` OtherActor))
  (`/Engine/EditorBlueprintResources/StandardMacros.IsValid` _asbp_vpplayer_character
    (:`Is Valid`
      (if (`self.KillTrigger`) :!label _label
        (set `self.KillTrigger` false)
        (else
          (`KismetSystemLibrary.PrintString` "ERROR  - Press collision"))))))

(event `self.PressDown.OnComponentEndOverlap`
  (params (OverlappedComponent :type "PrimitiveComponent Object Reference") (OtherActor :type "Actor Object Reference") (OtherComp :type "PrimitiveComponent Object Reference") (OtherBodyIndex :type Integer))
  ;[1 1 1] Kill Mechanic
  (bind _asbp_vpplayer_character (cast `/Game/_VisionProtocol/Core/BP_VPPlayerCharacter` OtherActor))
  (`/Engine/EditorBlueprintResources/StandardMacros.IsValid` _asbp_vpplayer_character
    (:`Is Valid`
      (goto _label))))

(event `/Game/_VisionProtocol/Objects/Factory/BPI_Powerable.Power On`
  (bind _relativelocation (`SceneComponent.RelativeLocation` (`self.PressUp`)))
  (set `self.IsPowered` true)
  (`self.NormalSpeed`)
  (`/Engine/EditorBlueprintResources/StandardMacros.DoOnce` false
    (:`Completed`
      (`GameplayStatics.PlaySoundAtLocation` "/Game/_VisionProtocol/Audio/SFX/NewSFX/shotgun.shotgun" (`self.K2_GetActorLocation`) (struct) 0.3 0.6 0.0 "/Game/_VisionProtocol/Audio/BasicSoundAttenuation.BasicSoundAttenuation" null null null)
      (`KismetSystemLibrary.Delay` (`self.SpawnDelay`))
      ;[1 1 1] Save start position
      (set `self.StartLocationUp` _relativelocation)
      (set `self.DistanceFromCenter` (.z (- _relativelocation (`SceneComponent.RelativeLocation` (`self.PressDown`)))))
      (for _array_element (`self.PressUpObjectList`)
        (add `self.OnActorHit` _array_element (delegate `ControlledObjectHit`))
        (`KismetArrayLibrary.Array_Add` (`self.PressUpLocations`) (`self.K2_GetActorLocation` _array_element)))
      (add `self.OnLoopEnd` (delegate `ActivatePress`))
      (`self.ActivatePress`))))

(event `ActivatePress`
  (bind _waitinnit (`self.WaitInnit`))
  (bind _close (`self.Close`))
  (bind _startlocationup (`self.StartLocationUp`))
  (bind _returnvalue (`KismetMathLibrary.MultiplyMultiply_FloatFloat` (`self.CloseDuration`) -1.0))
  (bind _returnvalue_2 (`KismetMathLibrary.MultiplyMultiply_FloatFloat` (`self.InitialDelay`) -1.0))
  (if (not (`self.ActivelySlowed`))
    (`TimelineComponent.SetPlayRate` _waitinnit _returnvalue_2)
    (`Timeline|WaitInnit` :!via `PlayFromStart` :!label _label_2
      (:`Finished`
        (if (not (`self.ActivelySlowed`)) :!label _label_3
          (`TimelineComponent.SetPlayRate` _close _returnvalue)
          (bind (_direction _open_animation) (`Timeline|Close` :!via `PlayFromStart` :!label _label_4)
            (:`Update`
              (`SceneComponent.K2_SetRelativeLocation` (`self.PressUp`) (`KismetMathLibrary.VLerp` _startlocationup (- _startlocationup (`KismetMathLibrary.MakeVector` 0.0 0.0 (`self.DistanceFromCenter`))) _open_animation) false false)
              (for (_array_element _array_index) (`self.PressUpObjectList`)
                (`/Engine/EditorBlueprintResources/StandardMacros.IsValid` _array_element
                  (:`Is Valid`
                    (bind _output (`|GetArrayItem` (`self.PressUpLocations`) _array_index))
                    (`self.K2_SetActorLocation` _array_element (`KismetMathLibrary.VLerp` _output (- _output (`KismetMathLibrary.GreaterGreater_VectorRotator` (`KismetMathLibrary.MakeVector` 0.0 0.0 (`self.DistanceFromCenter`)) (`self.K2_GetActorRotation`))) _open_animation) false false)))))
            (:`Finished`
              (`GameplayStatics.PlaySoundAtLocation` "/Game/_VisionProtocol/Audio/SFX/explosion.explosion" (`self.K2_GetActorLocation`) (struct) 1.0 0.5 0.0 "/Game/_VisionProtocol/Audio/BasicSoundAttenuation.BasicSoundAttenuation" null null null)
              (set `self.ReadyToReverse` true)))
          (else
            (`TimelineComponent.SetPlayRate` _close (/ _returnvalue (`self.SlowStrength`)))
            (goto _label_4 :!via `PlayFromStart`)))))
    (else
      (`TimelineComponent.SetPlayRate` _waitinnit (/ _returnvalue_2 (`self.SlowStrength`)))
      (goto _label_2 :!via `PlayFromStart`))))

(event `ControlledObjectHit` :!signature `self.OnActorHit`
  (params (SelfActor :type "Actor Object Reference") (OtherActor :type "Actor Object Reference") (NormalImpulse :type "Vector Structure") (Hit :type "HitResult Structure (by ref)"))
  ;[1 1 1] Save start position
  (cast `/Game/_VisionProtocol/Core/Weapons/Projectiles/Chronovisor/BP_ReverseBullet` OtherActor)
  (`/Game/_VisionProtocol/Core/Visors/Chronovisor/BPI_Reversable.Reverse`))

(event `SlowDown`
  (`TimelineComponent.SetPlayRate` (`self.WaitInnit`) (/ (`KismetMathLibrary.MultiplyMultiply_FloatFloat` (`self.InitialDelay`) -1.0) (`self.SlowStrength`)))
  (`TimelineComponent.SetPlayRate` (`self.Close`) (/ (`KismetMathLibrary.MultiplyMultiply_FloatFloat` (`self.CloseDuration`) -1.0) (`self.SlowStrength`)))
  (`TimelineComponent.SetPlayRate` (`self.WaitHold`) (/ (`KismetMathLibrary.MultiplyMultiply_FloatFloat` (`self.HoldDuration`) -1.0) (`self.SlowStrength`)))
  (`TimelineComponent.SetPlayRate` (`self.Open`) (/ (`KismetMathLibrary.MultiplyMultiply_FloatFloat` (`self.OpenDuration`) -1.0) (`self.SlowStrength`))))

(event `VisorSlowActivated`
  (params (SlowDown :type Boolean))
  (if SlowDown
    (if (not (`self.ActivelySlowed`))
      (set `self.ActivelySlowed` true)
      (`self.SlowDown`))
    (elif (`self.ActivelySlowed`)
      (set `self.ActivelySlowed` false)
      (`self.NormalSpeed`))))

(event `NormalSpeed`
  (`TimelineComponent.SetPlayRate` (`self.WaitInnit`) (`KismetMathLibrary.MultiplyMultiply_FloatFloat` (`self.InitialDelay`) -1.0))
  (`TimelineComponent.SetPlayRate` (`self.Close`) (`KismetMathLibrary.MultiplyMultiply_FloatFloat` (`self.CloseDuration`) -1.0))
  (`TimelineComponent.SetPlayRate` (`self.WaitHold`) (`KismetMathLibrary.MultiplyMultiply_FloatFloat` (`self.HoldDuration`) -1.0))
  (`TimelineComponent.SetPlayRate` (`self.Open`) (`KismetMathLibrary.MultiplyMultiply_FloatFloat` (`self.OpenDuration`) -1.0)))

(event `/Game/_VisionProtocol/Core/Visors/Chronovisor/BPI_Reversable.Reverse`
  (bind _waithold (`self.WaitHold`))
  (bind _open (`self.Open`))
  (bind _startlocationup (`self.StartLocationUp`))
  (bind _returnvalue (`KismetMathLibrary.MultiplyMultiply_FloatFloat` (`self.HoldDuration`) -1.0))
  (bind _returnvalue_2 (`KismetMathLibrary.MultiplyMultiply_FloatFloat` (`self.OpenDuration`) -1.0))
  (if (and (`self.ReadyToReverse`) (`self.IsPowered`))
    (set `self.ReadyToReverse` false)
    (if (not (`self.ActivelySlowed`))
      (`TimelineComponent.SetPlayRate` _open _returnvalue_2)
      (else
        (`TimelineComponent.SetPlayRate` _open (/ _returnvalue_2 (`self.SlowStrength`)))))
    (`GameplayStatics.PlaySoundAtLocation` null (`self.K2_GetActorLocation`) (struct) 1.0 1.0 0.0 null null null null)
    (bind (_direction _close_animation) (`Timeline|Open` :!via `PlayFromStart`)
      (:`Update`
        (`SceneComponent.K2_SetRelativeLocation` (`self.PressUp`) (`KismetMathLibrary.VLerp` (- _startlocationup (`KismetMathLibrary.MakeVector` 0.0 0.0 (`self.DistanceFromCenter`))) _startlocationup _close_animation) false false)
        (for (_array_element _array_index) (`self.PressUpObjectList`)
          (`/Engine/EditorBlueprintResources/StandardMacros.IsValid` _array_element
            (:`Is Valid`
              (bind _output (`|GetArrayItem` (`self.PressUpLocations`) _array_index))
              (`self.K2_SetActorLocation` _array_element (`KismetMathLibrary.VLerp` (- _output (`KismetMathLibrary.GreaterGreater_VectorRotator` (`KismetMathLibrary.MakeVector` 0.0 0.0 (`self.DistanceFromCenter`)) (`self.K2_GetActorRotation`))) _output _close_animation) false false)))))
      (:`Finished`
        (if (not (`self.ActivelySlowed`))
          (`TimelineComponent.SetPlayRate` _waithold _returnvalue)
          (bind (_direction_2 _wait_timer) (`Timeline|WaitHold` :!via `PlayFromStart` :!label _label_5)
            (:`Update`
              (`KismetSystemLibrary.PrintString` (`KismetStringLibrary.Conv_DoubleToString` _wait_timer))
              (if (or (== _wait_timer 0.75) (== _wait_timer 0.8) (== _wait_timer 0.85) (== _wait_timer 0.9))
                (`GameplayStatics.PlaySoundAtLocation` "/Game/_VisionProtocol/Audio/SFX/line_shoot.line_shoot" (`self.K2_GetActorLocation`) (struct) 1.0 0.5 0.0 "/Game/_VisionProtocol/Audio/BasicSoundAttenuation.BasicSoundAttenuation" null null null)))
            (:`Finished`
              (goto _label_3)))
          (else
            (`TimelineComponent.SetPlayRate` _waithold (/ _returnvalue (`self.SlowStrength`)))
            (goto _label_5 :!via `PlayFromStart`)))))))

(event `/Game/_VisionProtocol/Objects/Factory/BPI_Powerable.Power Off`
  (`TimelineComponent.SetPlayRate` (`self.WaitInnit`) 0.0)
  (`TimelineComponent.SetPlayRate` (`self.Close`) 0.0)
  (`TimelineComponent.SetPlayRate` (`self.WaitHold`) 0.0)
  (`TimelineComponent.SetPlayRate` (`self.Open`) 0.0)
  (set `self.IsPowered` false))

(fn `UserConstructionScript`)
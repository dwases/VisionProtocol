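; Interactable computer terminal that powers factory machines and opens dialogue, also configurable as a book, page or drone.
; The first interaction calls PowerOn through BPI_Powerable on its ControlledMashines and fires the PoweredOn dispatcher for each.
; Every interaction starts the chosen dialogue on the interactor's BPC_DialogSystem, if present, with a 2D sound picked by ObjectType.
; It supplies its interaction name and always shows the interact key widget.
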(event `self.Interact`
  (params (Interactor :type "Actor Object Reference") (InteracteeComponent :type "PrimitiveComponent Object Reference"))
  (bind _returnvalue (`self.GetComponentByClass` Interactor "/Game/_VisionProtocol/Core/DialogSystem/BPC_DialogSystem.BPC_DialogSystem_C"))
  (`|ExecutionSequence`
    (:`then_0`
      (`/Engine/EditorBlueprintResources/StandardMacros.DoOnce` false
        (:`Completed`
          (for _array_element (`self.ControlledMashines`)
            (bind _asbpi_powerable (cast `/Game/_VisionProtocol/Objects/Factory/BPI_Powerable` _array_element))
            (`/Game/_VisionProtocol/Objects/Factory/BPI_Powerable.Power On` _asbpi_powerable)
            (`self.PoweredOn`)))))
    (:`then_1`
      (`/Engine/EditorBlueprintResources/StandardMacros.IsValid` _returnvalue
        (:`Is Valid`
          (`/Game/_VisionProtocol/Core/DialogSystem/BPC_DialogSystem.BeginDialog` _returnvalue (`self.ChooseDialogue`))
          (switch `/Game/_VisionProtocol/Objects/EObjectType` (`self.ObjectType`)
            (:`NewEnumerator0`
              (`GameplayStatics.PlaySound2D` "/Game/_VisionProtocol/Audio/SFX/book.book" 1.0 1.0 0.0 null null))
            (:`NewEnumerator1`
              (`GameplayStatics.PlaySound2D` "/Game/_VisionProtocol/Audio/SFX/dron_lub_komp.dron_lub_komp" 1.0 1.0 0.0 null null))
            (:`NewEnumerator2`
              (`GameplayStatics.PlaySound2D` "/Game/_VisionProtocol/Audio/SFX/dron_lub_komp.dron_lub_komp" 1.0 1.0 0.0 null null))
            (:`NewEnumerator3`
              (`GameplayStatics.PlaySound2D` "/Game/_VisionProtocol/Audio/SFX/page.page" 1.0 1.0 0.0 null null))))))))

(fn `GetInteractionName`
  (returns (InteractionName :type Text))
  (return (`self.InteractionName`)))

(fn `GetIsInteractKeyWidgetVisible`
  (returns (IsInteractKeyWidgetVisible :type Boolean))
  (return true))

(fn `UserConstructionScript`)
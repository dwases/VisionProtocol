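; BP_IceBlock is a thermovisor-specific ice block that melts away when heated.
; HeatUp caches the current scale, then plays a falloff timeline that scales the block from it, ignoring calls while the timeline runs.
; When the timeline finishes, the actor waits briefly and destroys itself.
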(event `/Game/_VisionProtocol/Core/Visors/Termovisor/BPI_Heatable.HeatUp`
  (if (not (`TimelineComponent.IsPlaying` (`self.TL_IceSizeFalloff`)))
    (set `self.FormerScale` (`self.GetActorScale3D`))
    (bind (_direction _falloff) (`Timeline|TL_IceSizeFalloff` :!via `PlayFromStart`)
      (:`Update`
        (`self.SetActorScale3D` self (* (`self.FormerScale`) _falloff)))
      (:`Finished`
        (`KismetSystemLibrary.Delay` 0.4)
        (`self.K2_DestroyActor`)))))

(fn `UserConstructionScript`)
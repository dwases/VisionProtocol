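; BP_HotPlatform is a Termovisor platform that can be cooled, then melted away by heat.
; CoolDown swaps the cube from the laser pointer material to the hover material and sets its custom depth stencil to 1.
; HeatUp works only on a cooled cube, scaling the actor through an ice falloff timeline and destroying it after a short delay.
; The current material doubles as the hot/cold state.
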(event `/Game/_VisionProtocol/Core/Visors/Termovisor/BPI_Coolable.CoolDown`
  (bind _cube (`self.Cube`))
  (if (== (`PrimitiveComponent.GetMaterial` (`self.Cube`) 0) "/Engine/VREditor/LaserPointer/LaserPointerMaterialInst.LaserPointerMaterialInst")
    (`PrimitiveComponent.SetMaterial` _cube 0 "/Engine/VREditor/LaserPointer/HoverMaterial.HoverMaterial")
    (`PrimitiveComponent.SetCustomDepthStencilValue` _cube 1)))

(event `/Game/_VisionProtocol/Core/Visors/Termovisor/BPI_Heatable.HeatUp`
  (if (and (== (`PrimitiveComponent.GetMaterial` (`self.Cube`) 0) "/Engine/VREditor/LaserPointer/HoverMaterial.HoverMaterial") (not (`TimelineComponent.IsPlaying` (`self.TL_IceSizeFalloff`))))
    (set `self.FormerScale` (`self.GetActorScale3D`))
    (bind (_direction _falloff) (`Timeline|TL_IceSizeFalloff` :!via `PlayFromStart`)
      (:`Update`
        (`self.SetActorScale3D` self (* (`self.FormerScale`) _falloff)))
      (:`Finished`
        (`KismetSystemLibrary.Delay` 0.4)
        (`self.K2_DestroyActor`)))))

(fn `UserConstructionScript`)
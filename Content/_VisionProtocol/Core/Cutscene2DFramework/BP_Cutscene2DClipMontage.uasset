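; Blueprint that plays a 2D cutscene montage as timed image slides with voicelines, subtitles and a soundtrack.
; On BeginPlay it adds the WBP_Cutscene2DMaster widget to the viewport and loads clip rows from the ClipsDT DataTable.
; Each clip updates the widget's image and subtitle, plays its voiceline and optionally starts a zoom lasting its duration.
; A delay then advances the index and re-triggers playback through a near-instant timer until clips run out.
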(event `self.ReceiveBeginPlay`
  (`GameplayStatics.SpawnSound2D` (`self.Soundtrack`) 1.0 1.0 0.0 null)
  (bind _returnvalue (`|CreateWidget` "/Game/_VisionProtocol/Core/Cutscene2DFramework/UI/WBP_Cutscene2DMaster.WBP_Cutscene2DMaster_C"))
  (bind _output_get (set `self.MasterWidgetRef` _returnvalue))
  (`UserWidget.AddToViewport` _output_get 0)
  (bind _outrownames (`DataTableFunctionLibrary.GetDataTableRowNames` (`self.ClipsDT`)))
  (for _array_element _outrownames
    (bind _returnvalue_2 (`|GetDataTableRow` (`self.ClipsDT`) _array_element)
      (:`then`
        (`KismetArrayLibrary.Array_Add` (`self.Clips`) _returnvalue_2)
        (`self.PlayClips`)))))

(event `PlayClips`
  (`KismetSystemLibrary.PrintString` (`KismetStringLibrary.Conv_DoubleToString` (`self.CurrentClipTime`)))
  (bind _returnvalue (`KismetSystemLibrary.K2_SetTimerDelegate` (delegate `PlayClipOfCurrentClipIndex`) 1e-06))
  (set `self.TimerHandle` _returnvalue))

(event `PlayClipOfCurrentClipIndex`
  (bind (_image _zoom _subtitles _voiceline _duration) (break `/Game/_VisionProtocol/Core/Cutscene2DFramework/SClipData` (`|GetArrayItem` (`self.Clips`) (`self.CurrentClipIndex`))))
  (set `self.CurrentClipTime` _duration)
  (`GameplayStatics.SpawnSound2D` _voiceline 1.0 1.0 0.0 null)
  (set `TextBlock.Text` _subtitles (`/Game/_VisionProtocol/Core/Cutscene2DFramework/UI/WBP_Cutscene2DMaster.SubtitleBoxText` (`self.MasterWidgetRef`)))
  (`Image.SetBrushFromTexture` (`/Game/_VisionProtocol/Core/Cutscene2DFramework/UI/WBP_Cutscene2DMaster.BackgroundImage` (`self.MasterWidgetRef`)) _image false)
  (setmembers `SlateBrush` :`StructRef` (`Image.Brush` (`/Game/_VisionProtocol/Core/Cutscene2DFramework/UI/WBP_Cutscene2DMaster.BackgroundImage` (`self.MasterWidgetRef`))) :`ImageSize` (`SlateBlueprintLibrary.GetLocalSize` (`Widget.GetCachedGeometry` (`self.MasterWidgetRef`))))
  (if (!= _zoom 0.0)
    (`/Game/_VisionProtocol/Core/Cutscene2DFramework/UI/WBP_Cutscene2DMaster.InitiateZoom` (`self.MasterWidgetRef`) _zoom _duration))
  (set `self.CurrentClipIndex` (+ (`self.CurrentClipIndex`) 1))
  (`KismetSystemLibrary.Delay` (`self.CurrentClipTime`))
  (if (< (`self.CurrentClipIndex`) (`KismetArrayLibrary.Array_Length` (`self.Clips`)))
    (`/Game/_VisionProtocol/Core/Cutscene2DFramework/UI/WBP_Cutscene2DMaster.AbortZoom` (`self.MasterWidgetRef`))
    (`self.PlayClips`)))

(fn `UserConstructionScript`)
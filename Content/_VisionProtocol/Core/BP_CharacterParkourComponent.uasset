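; Parkour component for the VP player character that handles jumping, with coyote time and a tag-gated double jump.
; Tick accumulates airtime while falling, letting a jump launch normally from the ground or within the brief coyote window.
; Later presses need the DoubleJump skill tag and pass through a DoN gate fed by the midair jump counter, which only coyote jumps increment.
; Landing clears airtime and resets the gate, which a separate air-jump reset event also does.
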(event `self.ReceiveTick`
  (params (DeltaSeconds :type "Float (single-precision)"))
  (bind _playerparkourdata (`self.PlayerParkourData`))
  ;[1 1 1] midair time counter
  (if (`NavMovementComponent.IsFalling` (`Character.CharacterMovement` (`self.OwnerRef`)))
    (setmembers `/Game/_VisionProtocol/Core/Structures/SPlayerParkourData` :`StructRef` _playerparkourdata :`CurrMidairTime` (+ (* DeltaSeconds 1.0) (`.CurrMidairTime_5_C2ABA58F47D15CF15970F6BAF75CD5D1` (break `/Game/_VisionProtocol/Core/Structures/SPlayerParkourData` _playerparkourdata))))))

(event `self.ReceiveBeginPlay`
  (bind _asbp_vpplayer_character (cast `/Game/_VisionProtocol/Core/BP_VPPlayerCharacter` (`self.GetOwner` self)))
  (set `self.OwnerRef` _asbp_vpplayer_character)
  (setmembers `/Game/_VisionProtocol/Core/Structures/SPlayerParkourData` :`StructRef` (`self.PlayerParkourData`) :`MaxCoyoteTime` 0.15 :`CurrMidairTime` 0.0 :`MidairJumpCounter` 0))

(event `ParkourJump`
  (bind _playerparkourdata (`self.PlayerParkourData`))
  (bind (_maxcoyotetime _currmidairtime) (break `/Game/_VisionProtocol/Core/Structures/SPlayerParkourData` (`self.PlayerParkourData`)))
  (switch `EMovementMode` (`CharacterMovementComponent.MovementMode` (`Actor.GetComponentByClass` (`self.OwnerRef`) "/Script/Engine.CharacterMovementComponent"))
    (:`MOVE_Walking`
      (`Character.LaunchCharacter` (`self.OwnerRef`) (0.0 0.0 1000.0) false true))
    (:`MOVE_Falling`
      ;[1 1 1] coyote time logic trigger
      (if (< _currmidairtime _maxcoyotetime)
        (`Character.LaunchCharacter` (`self.OwnerRef`) (0.0 0.0 1000.0) false true)
        (setmembers `/Game/_VisionProtocol/Core/Structures/SPlayerParkourData` :`StructRef` _playerparkourdata :`MidairJumpCounter` (+ (`.MidairJumpCounter_8_896DCA6E4A3EDD33C4CA0E9C602787AA` (break `/Game/_VisionProtocol/Core/Structures/SPlayerParkourData` _playerparkourdata)) 1))
        (else
          ;[1 1 1] double jump logic
          (if (`BlueprintGameplayTagLibrary.HasTag` (`self.ParkourTags`) (struct :`TagName` "Player.AvailableSkill.DoubleJump") true)
            (bind _counter (`/Engine/EditorBlueprintResources/StandardMacros.Do N` (`.MidairJumpCounter_8_896DCA6E4A3EDD33C4CA0E9C602787AA` (break `/Game/_VisionProtocol/Core/Structures/SPlayerParkourData` (`self.PlayerParkourData`))) :!label _label)
              (:`Exit`
                (switch `int` _counter
                  (:`1`
                    (`Character.LaunchCharacter` (`self.OwnerRef`) (0.0 0.0 1000.0) false true)))))))))))

(event `ParkourLand`
  ;[1 1 1] double jump logic
  (setmembers `/Game/_VisionProtocol/Core/Structures/SPlayerParkourData` :`StructRef` (`self.PlayerParkourData`) :`CurrMidairTime` 0.0)
  (goto _label :!via `Reset`))

(event `ParkourResetAirJump`
  ;[1 1 1] double jump logic
  (goto _label :!via `Reset`))
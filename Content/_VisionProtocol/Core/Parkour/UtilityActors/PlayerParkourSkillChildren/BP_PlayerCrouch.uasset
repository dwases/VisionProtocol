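; Player parkour skill that handles crouching, sliding and standing up.
; When the tag allows and the player is neither dashing nor falling, it crouches if stationary or slides if moving, otherwise standing up.
; Timelines resize the capsule and drive slide velocity along last input; slides switch the controller's sliding context and end crouched.
; Gameplay tags track state, and a timer cooldown is mirrored into the component's parkour data on Tick.
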(event `self.ReceiveTick`
  (params (DeltaSeconds :type "Float (single-precision)"))
  (if (`KismetSystemLibrary.K2_IsValidTimerHandle` (`self.CooldownHandle`))
    (setmembers `/Game/_VisionProtocol/Core/Structures/SPlayerParkourData` :`StructRef` (`/Game/_VisionProtocol/Core/Parkour/BP_CharacterParkourComponent.PlayerParkourData` (`/Game/_VisionProtocol/Core/BP_VPPlayerCharacter.BP_CharacterParkourComponent` (`self.VPPlayerRef`))) :`CrouchCurrCooldown` (`KismetSystemLibrary.K2_GetTimerRemainingTimeHandle` (`self.CooldownHandle`)))))

(event `self.ReceiveBeginPlay`
  (`parent.ReceiveBeginPlay`))

(event `/Game/_VisionProtocol/Core/Parkour/Interfaces/BPI_PlayerParkourSkill.PerformIfPossible`
  (params (ParkourData :type "/Game/_VisionProtocol/Core/Structures/SPlayerParkourData Structure") (ParkourTags :type "GameplayTagContainer Structure"))
  (bind _returnvalue (`Pawn.GetLastMovementInputVector` (`self.VPPlayerRef`)))
  (bind _charactermovement (`Character.CharacterMovement` (`self.VPPlayerRef`)))
  (bind (_velocity_x _velocity_y) (`KismetMathLibrary.BreakVector` (`MovementComponent.Velocity` (`Character.CharacterMovement` (`self.VPPlayerRef`)))))
  (bind (_velocity_x_2 _velocity_y_2) (`KismetMathLibrary.BreakVector` (`MovementComponent.Velocity` (`Character.CharacterMovement` (`self.VPPlayerRef`)))))
  (bind (_velocity_x_3 _velocity_y_3 _velocity_z) (`KismetMathLibrary.BreakVector` (`MovementComponent.Velocity` _charactermovement)))
  ;[1 1 1] cases: ignore, crouch, slide
  ;[1 1 1] Pass if crouching or sliding is unavailable
  (if (`BlueprintGameplayTagLibrary.HasAllTags` ParkourTags (`BlueprintGameplayTagLibrary.MakeLiteralGameplayTagContainer` (struct :`GameplayTags` (struct :`(TagName` "Player.AvailableSkill.Crouch") :`(TagName` "Player.AvailableSkill.Slide")))) true)
    ;[1 1 1] Pass if player is dashing or falling
    (if (not (or (`BlueprintGameplayTagLibrary.HasAnyTags` ParkourTags (`BlueprintGameplayTagLibrary.MakeLiteralGameplayTagContainer` (struct :`GameplayTags` (struct :`(TagName` "Player.Dash")))) true) (`|EnumEquality` (`CharacterMovementComponent.MovementMode` (`Character.CharacterMovement` (`self.VPPlayerRef`))) "MOVE_Falling")))
      ;[1 1 1] Crouch if not moving and not crouching or sliding and crouch not on cooldown
      (if (and (<= (`KismetMathLibrary.VSize` (`KismetMathLibrary.MakeVector` _velocity_x_2 _velocity_y_2)) 0.0) (not (`BlueprintGameplayTagLibrary.HasAnyTags` (`/Game/_VisionProtocol/Core/Parkour/BP_CharacterParkourComponent.ParkourTags` (`/Game/_VisionProtocol/Core/BP_VPPlayerCharacter.BP_CharacterParkourComponent` (`self.VPPlayerRef`))) (`BlueprintGameplayTagLibrary.MakeLiteralGameplayTagContainer` (struct :`GameplayTags` (struct :`(TagName` "Player.Crouch") :`(TagName` "Player.Slide")))) true)) (<= (`.CrouchCurrCooldown_39_CA044C494C39E554951201B164CC40D4` (break `/Game/_VisionProtocol/Core/Structures/SPlayerParkourData` (`/Game/_VisionProtocol/Core/Parkour/BP_CharacterParkourComponent.PlayerParkourData` (`/Game/_VisionProtocol/Core/BP_VPPlayerCharacter.BP_CharacterParkourComponent` (`self.VPPlayerRef`))))) 0.0))
        ;[1 1 1] crouching behaviour
        (`self.CrouchBeginCooldown`)
        (`BlueprintGameplayTagLibrary.AddGameplayTag` (`/Game/_VisionProtocol/Core/Parkour/BP_CharacterParkourComponent.ParkourTags` (`/Game/_VisionProtocol/Core/BP_VPPlayerCharacter.BP_CharacterParkourComponent` (`self.VPPlayerRef`))) (struct :`TagName` "Player.Crouch"))
        (bind (_direction _crouchvelocity) (`Timeline|CrouchingTL` :!via `PlayFromStart`)
          (:`Update`
            (`CapsuleComponent.SetCapsuleHalfHeight` (`Character.CapsuleComponent` (`self.VPPlayerRef`)) (- (`CapsuleComponent.CapsuleHalfHeight` (`Character.CapsuleComponent` (`self.VPPlayerRef`))) (* _crouchvelocity (`.CrouchSpeedMultiplier_25_CD967649426C90C34C1D0F864FD5C42F` (break `/Game/_VisionProtocol/Core/Structures/SPlayerParkourData` (`/Game/_VisionProtocol/Core/Parkour/BP_CharacterParkourComponent.PlayerParkourData` (`/Game/_VisionProtocol/Core/BP_VPPlayerCharacter.BP_CharacterParkourComponent` (`self.VPPlayerRef`))))))) true)))
        (else
          ;[1 1 1] Slide if moving and not crouching or sliding and crouch not on cooldown
          (if (and (> (`KismetMathLibrary.VSize` (`KismetMathLibrary.MakeVector` _velocity_x _velocity_y)) 0.0) (not (`BlueprintGameplayTagLibrary.HasAnyTags` (`/Game/_VisionProtocol/Core/Parkour/BP_CharacterParkourComponent.ParkourTags` (`/Game/_VisionProtocol/Core/BP_VPPlayerCharacter.BP_CharacterParkourComponent` (`self.VPPlayerRef`))) (`BlueprintGameplayTagLibrary.MakeLiteralGameplayTagContainer` (struct :`GameplayTags` (struct :`(TagName` "Player.Crouch") :`(TagName` "Player.Slide")))) true)) (<= (`.CrouchCurrCooldown_39_CA044C494C39E554951201B164CC40D4` (break `/Game/_VisionProtocol/Core/Structures/SPlayerParkourData` (`/Game/_VisionProtocol/Core/Parkour/BP_CharacterParkourComponent.PlayerParkourData` (`/Game/_VisionProtocol/Core/BP_VPPlayerCharacter.BP_CharacterParkourComponent` (`self.VPPlayerRef`))))) 0.0))
            ;[1 1 1] sliding behaviour
            (`self.CrouchBeginCooldown`)
            (bind _asbp_vpplayer_controller (cast `/Game/_VisionProtocol/Core/BP_VPPlayerController` (`Pawn.GetController` (`self.VPPlayerRef`))))
            (`/Game/_VisionProtocol/Core/BP_VPPlayerController.InitiateSlidingContext` _asbp_vpplayer_controller)
            (set `self.SlideDirection` (/ _returnvalue (`KismetMathLibrary.VSize` _returnvalue)))
            (`BlueprintGameplayTagLibrary.AddGameplayTag` (`/Game/_VisionProtocol/Core/Parkour/BP_CharacterParkourComponent.ParkourTags` (`/Game/_VisionProtocol/Core/BP_VPPlayerCharacter.BP_CharacterParkourComponent` (`self.VPPlayerRef`))) (struct :`TagName` "Player.Slide"))
            (bind (_direction_2 _slideverticalvelocity _slidehorizontalvelocity) (`Timeline|SlidingTL` :!via `PlayFromStart`)
              (:`Update`
                (`CapsuleComponent.SetCapsuleHalfHeight` (`Character.CapsuleComponent` (`self.VPPlayerRef`)) (- (`CapsuleComponent.CapsuleHalfHeight` (`Character.CapsuleComponent` (`self.VPPlayerRef`))) (* _slideverticalvelocity (`.CrouchSpeedMultiplier_25_CD967649426C90C34C1D0F864FD5C42F` (break `/Game/_VisionProtocol/Core/Structures/SPlayerParkourData` (`/Game/_VisionProtocol/Core/Parkour/BP_CharacterParkourComponent.PlayerParkourData` (`/Game/_VisionProtocol/Core/BP_VPPlayerCharacter.BP_CharacterParkourComponent` (`self.VPPlayerRef`))))))) true)
                (bind (_returnvalue_x _returnvalue_y) (`KismetMathLibrary.BreakVector` (* (* (`self.SlideDirection`) _slidehorizontalvelocity) (`.SlideSpeedMultiplier_28_C45AA09645FB02B21E5E50A91B1A34D0` (break `/Game/_VisionProtocol/Core/Structures/SPlayerParkourData` (`/Game/_VisionProtocol/Core/Parkour/BP_CharacterParkourComponent.PlayerParkourData` (`/Game/_VisionProtocol/Core/BP_VPPlayerCharacter.BP_CharacterParkourComponent` (`self.VPPlayerRef`))))))))
                (set `MovementComponent.Velocity` (`KismetMathLibrary.MakeVector` _returnvalue_x _returnvalue_y _velocity_z) _charactermovement))
              (:`Finished`
                (`BlueprintGameplayTagLibrary.RemoveGameplayTag` (`/Game/_VisionProtocol/Core/Parkour/BP_CharacterParkourComponent.ParkourTags` (`/Game/_VisionProtocol/Core/BP_VPPlayerCharacter.BP_CharacterParkourComponent` (`self.VPPlayerRef`))) (struct :`TagName` "Player.Slide"))
                (`BlueprintGameplayTagLibrary.AddGameplayTag` (`/Game/_VisionProtocol/Core/Parkour/BP_CharacterParkourComponent.ParkourTags` (`/Game/_VisionProtocol/Core/BP_VPPlayerCharacter.BP_CharacterParkourComponent` (`self.VPPlayerRef`))) (struct :`TagName` "Player.Crouch"))
                (bind _asbp_vpplayer_controller_2 (cast `/Game/_VisionProtocol/Core/BP_VPPlayerController` (`Pawn.GetController` (`self.VPPlayerRef`))))
                (`/Game/_VisionProtocol/Core/BP_VPPlayerController.ExitSlidingContext` _asbp_vpplayer_controller_2)))
            (else
              ;[1 1 1] initiating stand up behaviour
              (`self.ExitCrouch`))))))))

(event `ExitCrouch`
  (bind _crouchingtl (`self.CrouchingTL`))
  (bind _slidingtl (`self.SlidingTL`))
  (bind _parkourtags (`/Game/_VisionProtocol/Core/Parkour/BP_CharacterParkourComponent.ParkourTags` (`/Game/_VisionProtocol/Core/BP_VPPlayerCharacter.BP_CharacterParkourComponent` (`self.VPPlayerRef`))))
  ;[1 1 1] Stand up behaviour
  (bind _asbp_vpplayer_controller (cast `/Game/_VisionProtocol/Core/BP_VPPlayerController` (`Pawn.GetController` (`self.VPPlayerRef`))))
  (`/Game/_VisionProtocol/Core/BP_VPPlayerController.ExitSlidingContext` _asbp_vpplayer_controller)
  (`BlueprintGameplayTagLibrary.RemoveGameplayTag` _parkourtags (struct :`TagName` "Player.Crouch"))
  (`BlueprintGameplayTagLibrary.RemoveGameplayTag` _parkourtags (struct :`TagName` "Player.Slide"))
  (`/Engine/EditorBlueprintResources/StandardMacros.IsValid` _crouchingtl
    (:`Is Valid`
      (`TimelineComponent.Stop` _crouchingtl)
      (`/Engine/EditorBlueprintResources/StandardMacros.IsValid` _slidingtl
        (:`Is Valid`
          (`TimelineComponent.Stop` _slidingtl)
          (bind (_direction _standupspeed) (`Timeline|StandUpTL` :!via `PlayFromStart`)
            (:`Update`
              (`CapsuleComponent.SetCapsuleHalfHeight` (`Character.CapsuleComponent` (`self.VPPlayerRef`)) (`KismetMathLibrary.FClamp` (+ (`CapsuleComponent.CapsuleHalfHeight` (`Character.CapsuleComponent` (`self.VPPlayerRef`))) (* _standupspeed (`.CrouchStandUpSpeedMultiplier_33_A34A81C74A2C88F88E33988DCB3BC2B7` (break `/Game/_VisionProtocol/Core/Structures/SPlayerParkourData` (`/Game/_VisionProtocol/Core/Parkour/BP_CharacterParkourComponent.PlayerParkourData` (`/Game/_VisionProtocol/Core/BP_VPPlayerCharacter.BP_CharacterParkourComponent` (`self.VPPlayerRef`))))))) 0.0 (`.OriginCapsuleHalfHeight_30_76D8FA044C1837A24C4099883559D62A` (break `/Game/_VisionProtocol/Core/Structures/SPlayerParkourData` (`/Game/_VisionProtocol/Core/Parkour/BP_CharacterParkourComponent.PlayerParkourData` (`/Game/_VisionProtocol/Core/BP_VPPlayerCharacter.BP_CharacterParkourComponent` (`self.VPPlayerRef`)))))) true))))))))

(event `CrouchBeginCooldown`
  ;[1 1 1] cooldown management
  (bind _returnvalue (`KismetSystemLibrary.K2_SetTimerDelegate` (delegate `CrouchActivateCooldown`) (`.CrouchMaxCooldown_38_58ADAD60410A7211289CCCB687307C63` (break `/Game/_VisionProtocol/Core/Structures/SPlayerParkourData` (`/Game/_VisionProtocol/Core/Parkour/BP_CharacterParkourComponent.PlayerParkourData` (`/Game/_VisionProtocol/Core/BP_VPPlayerCharacter.BP_CharacterParkourComponent` (`self.VPPlayerRef`)))))))
  (set `self.CooldownHandle` _returnvalue))

(event `CrouchActivateCooldown`
  ;[1 1 1] cooldown management
  (setmembers `/Game/_VisionProtocol/Core/Structures/SPlayerParkourData` :`StructRef` (`/Game/_VisionProtocol/Core/Parkour/BP_CharacterParkourComponent.PlayerParkourData` (`/Game/_VisionProtocol/Core/BP_VPPlayerCharacter.BP_CharacterParkourComponent` (`self.VPPlayerRef`))) :`CrouchCurrCooldown` 0.0))

(fn `UserConstructionScript`)
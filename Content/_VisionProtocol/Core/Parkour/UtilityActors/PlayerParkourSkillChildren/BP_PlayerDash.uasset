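; Parkour utility actor that performs the player's dash skill when it is off cooldown, unlocked by gameplay tag and movement input exists.
; A dash exits any slide, tags the player as dashing, switches the controller to a dashing context and drives velocity along the input direction through a timeline curve.
; A timer runs the cooldown, with Tick copying its remaining time into the parkour data.
; ExitDash cancels the dash early.
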(event `self.ReceiveTick`
  (params (DeltaSeconds :type "Float (single-precision)"))
  (if (`KismetSystemLibrary.K2_IsValidTimerHandle` (`self.CooldownHandle`))
    (setmembers `/Game/_VisionProtocol/Core/Structures/SPlayerParkourData` :`StructRef` (`/Game/_VisionProtocol/Core/Parkour/BP_CharacterParkourComponent.PlayerParkourData` (`/Game/_VisionProtocol/Core/BP_VPPlayerCharacter.BP_CharacterParkourComponent` (`self.VPPlayerRef`))) :`DashCurrCooldown` (`KismetSystemLibrary.K2_GetTimerRemainingTimeHandle` (`self.CooldownHandle`)))))

(event `DashActivateCooldown`
  (setmembers `/Game/_VisionProtocol/Core/Structures/SPlayerParkourData` :`StructRef` (`/Game/_VisionProtocol/Core/Parkour/BP_CharacterParkourComponent.PlayerParkourData` (`/Game/_VisionProtocol/Core/BP_VPPlayerCharacter.BP_CharacterParkourComponent` (`self.VPPlayerRef`))) :`DashCurrCooldown` 0.0))

(event `self.ReceiveBeginPlay`
  (`parent.ReceiveBeginPlay`))

(event `/Game/_VisionProtocol/Core/Parkour/Interfaces/BPI_PlayerParkourSkill.PerformIfPossible`
  (params (ParkourData :type "/Game/_VisionProtocol/Core/Structures/SPlayerParkourData Structure") (ParkourTags :type "GameplayTagContainer Structure"))
  (bind _returnvalue (`Pawn.GetLastMovementInputVector` (`self.VPPlayerRef`)))
  (bind _bp_characterparkourcomponent (`/Game/_VisionProtocol/Core/BP_VPPlayerCharacter.BP_CharacterParkourComponent` (`self.VPPlayerRef`)))
  ;[1 1 1] check dashing conditions
  (if (and (<= (`.DashCurrCooldown_13_211CAE20488CA8E070EFE1AE655A2565` (break `/Game/_VisionProtocol/Core/Structures/SPlayerParkourData` ParkourData)) 0.0) (`BlueprintGameplayTagLibrary.HasTag` ParkourTags (struct :`TagName` "Player.AvailableSkill.Dash") true) (> (`KismetMathLibrary.VSize` (`Pawn.GetLastMovementInputVector` (`self.VPPlayerRef`))) 0.0))
    (`|ExecutionSequence`
      (:`then_0`
        (if (`BlueprintGameplayTagLibrary.HasAnyTags` (`/Game/_VisionProtocol/Core/Parkour/BP_CharacterParkourComponent.ParkourTags` _bp_characterparkourcomponent) (`BlueprintGameplayTagLibrary.MakeLiteralGameplayTagContainer` (struct :`GameplayTags` (struct :`(TagName` "Player.Slide") :`(TagName` "Player.Crouch")))) true)
          (`/Game/_VisionProtocol/Core/Parkour/UtilityActors/PlayerParkourSkillChildren/BP_PlayerCrouch.ExitCrouch` (`/Game/_VisionProtocol/Core/Parkour/BP_CharacterParkourComponent.CrouchUtilityActor` _bp_characterparkourcomponent))))
      (:`then_1`
        (set `self.DashDirection` (/ _returnvalue (`KismetMathLibrary.VSize` _returnvalue)))
        (`|ExecutionSequence`
          (:`then_0`
            (`BlueprintGameplayTagLibrary.AddGameplayTag` (`/Game/_VisionProtocol/Core/Parkour/BP_CharacterParkourComponent.ParkourTags` (`/Game/_VisionProtocol/Core/BP_VPPlayerCharacter.BP_CharacterParkourComponent` (`self.VPPlayerRef`))) (struct :`TagName` "Player.Dash"))
            (bind _returnvalue_2 (`KismetSystemLibrary.K2_SetTimerDelegate` (delegate `DashActivateCooldown`) (`.DashMaxCooldown_11_7925F6AE4B3EDB6A7BF4FFAF694A6688` (break `/Game/_VisionProtocol/Core/Structures/SPlayerParkourData` (`/Game/_VisionProtocol/Core/Parkour/BP_CharacterParkourComponent.PlayerParkourData` (`/Game/_VisionProtocol/Core/BP_VPPlayerCharacter.BP_CharacterParkourComponent` (`self.VPPlayerRef`)))))))
            (set `self.CooldownHandle` _returnvalue_2)
            (bind _asbp_vpplayer_controller (cast `/Game/_VisionProtocol/Core/BP_VPPlayerController` (`Pawn.GetController` (`self.VPPlayerRef`))))
            (`/Game/_VisionProtocol/Core/BP_VPPlayerController.InitiateDashingContext` _asbp_vpplayer_controller))
          (:`then_1`
            (bind (_direction _dashvelocity) (`Timeline|DashTL` :!via `PlayFromStart` :!label _label)
              (:`Update`
                (set `MovementComponent.Velocity` (* (`self.DashDirection`) (* _dashvelocity (`.DashSpeedMultiplier_20_C8C78EE749CC892ABC71EB8F2887A1EE` (break `/Game/_VisionProtocol/Core/Structures/SPlayerParkourData` (`/Game/_VisionProtocol/Core/Parkour/BP_CharacterParkourComponent.PlayerParkourData` (`/Game/_VisionProtocol/Core/BP_VPPlayerCharacter.BP_CharacterParkourComponent` (`self.VPPlayerRef`))))))) (`Character.CharacterMovement` (`self.VPPlayerRef`))))
              (:`Finished`
                (`BlueprintGameplayTagLibrary.RemoveGameplayTag` (`/Game/_VisionProtocol/Core/Parkour/BP_CharacterParkourComponent.ParkourTags` (`/Game/_VisionProtocol/Core/BP_VPPlayerCharacter.BP_CharacterParkourComponent` (`self.VPPlayerRef`))) (struct :`TagName` "Player.Dash"))
                (bind _asbp_vpplayer_controller_2 (cast `/Game/_VisionProtocol/Core/BP_VPPlayerController` (`Pawn.GetController` (`self.VPPlayerRef`))))
                (`/Game/_VisionProtocol/Core/BP_VPPlayerController.ExitDashingContext` _asbp_vpplayer_controller_2)))))))))

(event `ExitDash`
  (set `MovementComponent.Velocity` (0.0 0.0 0.0) (`Character.CharacterMovement` (`self.VPPlayerRef`)))
  (`BlueprintGameplayTagLibrary.RemoveGameplayTag` (`/Game/_VisionProtocol/Core/Parkour/BP_CharacterParkourComponent.ParkourTags` (`/Game/_VisionProtocol/Core/BP_VPPlayerCharacter.BP_CharacterParkourComponent` (`self.VPPlayerRef`))) (struct :`TagName` "Player.Dash"))
  (bind _asbp_vpplayer_controller (cast `/Game/_VisionProtocol/Core/BP_VPPlayerController` (`Pawn.GetController` (`self.VPPlayerRef`))))
  (`/Game/_VisionProtocol/Core/BP_VPPlayerController.ExitDashingContext` _asbp_vpplayer_controller)
  (goto _label :!via `Stop`))

(fn `UserConstructionScript`)
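; Player parkour skill actor that lets a falling player wall-run horizontally along surfaces tagged HorizontalWallRun when off cooldown.
; Right and left camera-height line traces feed HorizontalWallRun, which launches the character along the rotated wall normal, switches controller input context, adds a gameplay tag and resets air jump.
; Aborting restores the context, removes the tag and starts a cooldown timer, mirrored on Tick into the parkour component's data.
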(event `self.ReceiveTick`
  (params (DeltaSeconds :type "Float (single-precision)"))
  (if (`KismetSystemLibrary.K2_IsValidTimerHandle` (`self.CooldownHandle`))
    (`/Engine/EditorBlueprintResources/StandardMacros.IsValid` (`self.VPPlayerRef`)
      (:`Is Valid`
        (setmembers `/Game/_VisionProtocol/Core/Structures/SPlayerParkourData` :`StructRef` (`/Game/_VisionProtocol/Core/Parkour/BP_CharacterParkourComponent.PlayerParkourData` (`/Game/_VisionProtocol/Core/BP_VPPlayerCharacter.BP_CharacterParkourComponent` (`self.VPPlayerRef`))) :`HorizontalWallRunCurrCooldown` (`KismetSystemLibrary.K2_GetTimerRemainingTimeHandle` (`self.CooldownHandle`)))))))

(event `/Game/_VisionProtocol/Core/Parkour/Interfaces/BPI_PlayerParkourSkill.PerformIfPossible`
  (params (ParkourData :type "/Game/_VisionProtocol/Core/Structures/SPlayerParkourData Structure") (ParkourTags :type "GameplayTagContainer Structure"))
  (if (<= (`.HorizontalWallRunCurrCooldown_71_FA696EF744073204BDCA04B37E0915FF` (break `/Game/_VisionProtocol/Core/Structures/SPlayerParkourData` (`/Game/_VisionProtocol/Core/Parkour/BP_CharacterParkourComponent.PlayerParkourData` (`/Game/_VisionProtocol/Core/BP_VPPlayerCharacter.BP_CharacterParkourComponent` (`self.VPPlayerRef`))))) 0.0)
    (switch `EMovementMode` (`CharacterMovementComponent.MovementMode` (`Character.CharacterMovement` (`self.VPPlayerRef`)))
      (:`MOVE_Falling`
        (`self.WallRunningCheckerAndInitializer`)))))

(event `HorizontalWallRunActivateCooldown`
  (setmembers `/Game/_VisionProtocol/Core/Structures/SPlayerParkourData` :`StructRef` (`/Game/_VisionProtocol/Core/Parkour/BP_CharacterParkourComponent.PlayerParkourData` (`/Game/_VisionProtocol/Core/BP_VPPlayerCharacter.BP_CharacterParkourComponent` (`self.VPPlayerRef`))) :`HorizontalWallRunCurrCooldown` 0.0))

(fn `AbortHorizontalWallRun`
  (bind _bp_characterparkourcomponent (`/Game/_VisionProtocol/Core/BP_VPPlayerCharacter.BP_CharacterParkourComponent` (`self.VPPlayerRef`)))
  (bind _asbp_vpplayer_controller (cast `/Game/_VisionProtocol/Core/BP_VPPlayerController` (`Pawn.GetController` (`self.VPPlayerRef`))))
  (`/Game/_VisionProtocol/Core/BP_VPPlayerController.ExitHorizontalWallRunningContext` _asbp_vpplayer_controller)
  (if (`BlueprintGameplayTagLibrary.HasTag` (`/Game/_VisionProtocol/Core/Parkour/BP_CharacterParkourComponent.ParkourTags` _bp_characterparkourcomponent) (struct :`TagName` "Player.HorizontalWallRun") true)
    (bind _returnvalue (`KismetSystemLibrary.K2_SetTimerDelegate` (`|CreateDelegate` :!event `HorizontalWallRunActivateCooldown`) (`.HorizontalWallRunMaxCooldown_70_4A473A0A4CD95BB25E1CA58A0839C30D` (break `/Game/_VisionProtocol/Core/Structures/SPlayerParkourData` (`/Game/_VisionProtocol/Core/Parkour/BP_CharacterParkourComponent.PlayerParkourData` _bp_characterparkourcomponent)))))
    (set `self.CooldownHandle` _returnvalue))
  (`BlueprintGameplayTagLibrary.RemoveGameplayTag` (`/Game/_VisionProtocol/Core/Parkour/BP_CharacterParkourComponent.ParkourTags` (`/Game/_VisionProtocol/Core/BP_VPPlayerCharacter.BP_CharacterParkourComponent` (`self.VPPlayerRef`))) (struct :`TagName` "Player.HorizontalWallRun")))

(fn `HorizontalWallRun`
  (params (WallNormal :type "Vector Structure") (WallSide :type "/Game/_VisionProtocol/Core/Enums/EWallRunDirections Enum" :default "NewEnumerator0"))
  (bind _vpplayerref (`self.VPPlayerRef`))
  (bind _vpplayerref_2 (`self.VPPlayerRef`))
  (bind _bp_characterparkourcomponent (`/Game/_VisionProtocol/Core/BP_VPPlayerCharacter.BP_CharacterParkourComponent` (`self.VPPlayerRef`)))
  (bind _bp_characterparkourcomponent_2 (`/Game/_VisionProtocol/Core/BP_VPPlayerCharacter.BP_CharacterParkourComponent` (`self.VPPlayerRef`)))
  (bind ((`HorizontalWallRunImpulseMultiplier_47_B756AE1D4295A51297E9F5A52CD77E4C` _horizontalwallrunimpulsemultiplier) (`HorizontalWallRunElevation_49_2F879AE24F7251D879999A938C5CEE54` _horizontalwallrunelevation)) (break `/Game/_VisionProtocol/Core/Structures/SPlayerParkourData` (`/Game/_VisionProtocol/Core/Parkour/BP_CharacterParkourComponent.PlayerParkourData` (`/Game/_VisionProtocol/Core/BP_VPPlayerCharacter.BP_CharacterParkourComponent` (`self.VPPlayerRef`)))))
  (switch `/Game/_VisionProtocol/Core/Enums/EWallRunDirections` WallSide
    (:`NewEnumerator0`
      (`Character.LaunchCharacter` _vpplayerref_2 (+ (* (`KismetMathLibrary.GreaterGreater_VectorRotator` WallNormal (struct :`Yaw` -90.0)) _horizontalwallrunimpulsemultiplier) (`KismetMathLibrary.MakeVector` 0.0 0.0 _horizontalwallrunelevation)) true true)
      (bind _asbp_vpplayer_controller (cast `/Game/_VisionProtocol/Core/BP_VPPlayerController` (`Pawn.GetController` _vpplayerref_2)))
      (`/Game/_VisionProtocol/Core/BP_VPPlayerController.InitiateHorizontalWallRunningContext` _asbp_vpplayer_controller)
      (`BlueprintGameplayTagLibrary.AddGameplayTag` (`/Game/_VisionProtocol/Core/Parkour/BP_CharacterParkourComponent.ParkourTags` _bp_characterparkourcomponent_2) (struct :`TagName` "Player.HorizontalWallRun"))
      (`/Game/_VisionProtocol/Core/Parkour/BP_CharacterParkourComponent.ParkourResetAirJump` _bp_characterparkourcomponent_2))
    (:`NewEnumerator1`
      (`Character.LaunchCharacter` _vpplayerref (+ (* (`KismetMathLibrary.GreaterGreater_VectorRotator` WallNormal (struct :`Yaw` 90.0)) _horizontalwallrunimpulsemultiplier) (`KismetMathLibrary.MakeVector` 0.0 0.0 _horizontalwallrunelevation)) true true)
      (bind _asbp_vpplayer_controller_2 (cast `/Game/_VisionProtocol/Core/BP_VPPlayerController` (`Pawn.GetController` _vpplayerref)))
      (`/Game/_VisionProtocol/Core/BP_VPPlayerController.InitiateHorizontalWallRunningContext` _asbp_vpplayer_controller_2)
      (`BlueprintGameplayTagLibrary.AddGameplayTag` (`/Game/_VisionProtocol/Core/Parkour/BP_CharacterParkourComponent.ParkourTags` _bp_characterparkourcomponent) (struct :`TagName` "Player.HorizontalWallRun"))
      (`/Game/_VisionProtocol/Core/Parkour/BP_CharacterParkourComponent.ParkourResetAirJump` _bp_characterparkourcomponent))))

(fn `HorizontalWallRunJump`
  (params (WallNormal :type "Vector Structure"))
  (bind _vpplayerref (`self.VPPlayerRef`))
  (`/Game/_VisionProtocol/Core/Parkour/BP_CharacterParkourComponent.HelJump` (`/Game/_VisionProtocol/Core/BP_VPPlayerCharacter.BP_CharacterParkourComponent` _vpplayerref))
  (bind _asbp_vpplayer_controller (cast `/Game/_VisionProtocol/Core/BP_VPPlayerController` (`Pawn.GetController` _vpplayerref)))
  (`/Game/_VisionProtocol/Core/BP_VPPlayerController.ExitHorizontalWallRunningContext` _asbp_vpplayer_controller))

(fn `UserConstructionScript`
  (`parent.UserConstructionScript`))

(fn `WallRunningCheckerAndInitializer`
  (returns (ReturnValue :type Boolean))
  (locals (RightWallChecker :type "Vector Structure") (LeftWallChecker :type "Vector Structure") (IsDecidedToWallRun :type Boolean))
  (bind _vpplayerref (`self.VPPlayerRef`))
  (bind _vpplayerref_2 (`self.VPPlayerRef`))
  (bind _returnvalue (`SceneComponent.K2_GetComponentLocation` (`/Game/FirstPerson/Blueprints/BP_FirstPersonCharacter.FirstPersonCamera` _vpplayerref)))
  (bind _returnvalue_2 (`SceneComponent.K2_GetComponentLocation` (`/Game/FirstPerson/Blueprints/BP_FirstPersonCharacter.FirstPersonCamera` _vpplayerref_2)))
  (bind _returnvalue_3 (+ _returnvalue (* (`KismetMathLibrary.GetRightVector` (`Controller.GetControlRotation` (`Pawn.GetController` _vpplayerref))) (`.HorizontalWallRunMaxWallDistance_42_BAEA9C5F4C17357984FEE78334FAA6C5` (break `/Game/_VisionProtocol/Core/Structures/SPlayerParkourData` (`/Game/_VisionProtocol/Core/Parkour/BP_CharacterParkourComponent.PlayerParkourData` (`/Game/_VisionProtocol/Core/BP_VPPlayerCharacter.BP_CharacterParkourComponent` (`self.VPPlayerRef`))))))))
  (bind _returnvalue_4 (+ _returnvalue_2 (* (* (`KismetMathLibrary.GetRightVector` (`Controller.GetControlRotation` (`Pawn.GetController` _vpplayerref_2))) -1.0) (`.HorizontalWallRunMaxWallDistance_42_BAEA9C5F4C17357984FEE78334FAA6C5` (break `/Game/_VisionProtocol/Core/Structures/SPlayerParkourData` (`/Game/_VisionProtocol/Core/Parkour/BP_CharacterParkourComponent.PlayerParkourData` (`/Game/_VisionProtocol/Core/BP_VPPlayerCharacter.BP_CharacterParkourComponent` (`self.VPPlayerRef`))))))))
  ;[1 1 1] wykrywanie prawej sciany
  (set `local.RightWallChecker` _returnvalue_3)
  (bind _outhit (`KismetSystemLibrary.LineTraceSingleForObjects` _returnvalue _returnvalue_3 (`|MakeArray` "ObjectTypeQuery1" :!type "EObjectTypeQuery Enum") false (`|MakeArray` (`self.VPPlayerRef`) :!type "Actor Object Reference") "ForDuration"))
  (if (`GameplayStatics.BreakHitResult` _outhit)
    (if (`self.ActorHasTag` (`.HitActor` (`GameplayStatics.BreakHitResult` _outhit)) "HorizontalWallRun")
      (`KismetSystemLibrary.PrintString` "wykryto prawa sciane")
      (`self.HorizontalWallRun` (`.Normal` (`GameplayStatics.BreakHitResult` _outhit)) "NewEnumerator1")
      (set `local.IsDecidedToWallRun` true)
      ;[1 1 1] wykrywanie lewej sciany
      (set `local.LeftWallChecker` _returnvalue_4 :!label _label)
      (bind _outhit_2 (`KismetSystemLibrary.LineTraceSingleForObjects` _returnvalue_2 _returnvalue_4 (`|MakeArray` "ObjectTypeQuery1" :!type "EObjectTypeQuery Enum") false (`|MakeArray` (`self.VPPlayerRef`) :!type "Actor Object Reference") "ForDuration"))
      (if (`GameplayStatics.BreakHitResult` _outhit_2)
        (if (`self.ActorHasTag` (`.HitActor` (`GameplayStatics.BreakHitResult` _outhit_2)) "HorizontalWallRun")
          (`KismetSystemLibrary.PrintString` "wykryto lewa sciane")
          (`self.HorizontalWallRun` (`.Normal` (`GameplayStatics.BreakHitResult` _outhit_2)))
          (set `local.IsDecidedToWallRun` true)
          (if (`local.IsDecidedToWallRun`) :!label _label_2
            (`/Game/_VisionProtocol/Core/Parkour/BP_CharacterParkourComponent.ParkourLand` (`/Game/_VisionProtocol/Core/BP_VPPlayerCharacter.BP_CharacterParkourComponent` (`self.VPPlayerRef`)))
            (else
              (`self.AbortHorizontalWallRun`)))
          (return false))
        (else
          (goto _label_2))))
    (else
      (goto _label))))
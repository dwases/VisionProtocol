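; Player grappling hook parkour skill that pulls the character toward a surface hit by a camera line trace.
; Grapple checks cooldown, resets air jump, hops if walking, shows the rope, switches input context and starts the cooldown timer.
; A gameplay tag on the parkour component holds the state, while Tick drives velocity and rope end and publishes remaining cooldown.
; ExitGrappling clears tag, velocity, rope and input context, then triggers landing.
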(event `self.ReceiveTick`
  (params (DeltaSeconds :type "Float (single-precision)"))
  (bind _vpplayerref (`self.VPPlayerRef`))
  (if (`BlueprintGameplayTagLibrary.HasTag` (`/Game/_VisionProtocol/Core/Parkour/BP_CharacterParkourComponent.ParkourTags` (`/Game/_VisionProtocol/Core/BP_VPPlayerCharacter.BP_CharacterParkourComponent` (`self.VPPlayerRef`))) (struct :`TagName` "Player.GrapplingHook") true)
    (`self.ContinueGrappling`))
  (if (`KismetSystemLibrary.K2_IsValidTimerHandle` (`self.CooldownHandle`))
    (`/Engine/EditorBlueprintResources/StandardMacros.IsValid` _vpplayerref
      (:`Is Valid`
        (setmembers `/Game/_VisionProtocol/Core/Structures/SPlayerParkourData` :`StructRef` (`/Game/_VisionProtocol/Core/Parkour/BP_CharacterParkourComponent.PlayerParkourData` (`/Game/_VisionProtocol/Core/BP_VPPlayerCharacter.BP_CharacterParkourComponent` _vpplayerref)) :`GrapplingHookRemainingCooldown` (`KismetSystemLibrary.K2_GetTimerRemainingTimeHandle` (`self.CooldownHandle`)))))))

(event `/Game/_VisionProtocol/Core/Parkour/Interfaces/BPI_PlayerParkourSkill.PerformIfPossible`
  (params (ParkourData :type "/Game/_VisionProtocol/Core/Structures/SPlayerParkourData Structure") (ParkourTags :type "GameplayTagContainer Structure"))
  (if (`BlueprintGameplayTagLibrary.HasTag` (`/Game/_VisionProtocol/Core/Parkour/BP_CharacterParkourComponent.ParkourTags` (`/Game/_VisionProtocol/Core/BP_VPPlayerCharacter.BP_CharacterParkourComponent` (`self.VPPlayerRef`))) (struct :`TagName` "Player.AvailableSkill.GrapplingHook") true)
    (if (`BlueprintGameplayTagLibrary.HasTag` (`/Game/_VisionProtocol/Core/Parkour/BP_CharacterParkourComponent.ParkourTags` (`/Game/_VisionProtocol/Core/BP_VPPlayerCharacter.BP_CharacterParkourComponent` (`self.VPPlayerRef`))) (struct :`TagName` "Player.GrapplingHook") true)
      (`self.ContinueGrappling`)
      (else
        (`self.Grapple`)))))

(event `Grapple`
  (bind _returnvalue (`SceneComponent.K2_GetComponentLocation` (`/Game/FirstPerson/Blueprints/BP_FirstPersonCharacter.FirstPersonCamera` (`self.VPPlayerRef`))))
  (if (<= (`.GrapplingHookRemainingCooldown_64_A670C6A04A345F73F4A725A360194BDB` (break `/Game/_VisionProtocol/Core/Structures/SPlayerParkourData` (`/Game/_VisionProtocol/Core/Parkour/BP_CharacterParkourComponent.PlayerParkourData` (`/Game/_VisionProtocol/Core/BP_VPPlayerCharacter.BP_CharacterParkourComponent` (`self.VPPlayerRef`))))) 0.0)
    (if (not (`BlueprintGameplayTagLibrary.HasTag` (`/Game/_VisionProtocol/Core/Parkour/BP_CharacterParkourComponent.ParkourTags` (`/Game/_VisionProtocol/Core/BP_VPPlayerCharacter.BP_CharacterParkourComponent` (`self.VPPlayerRef`))) (struct :`TagName` "Player.GrapplingHook") true))
      (if (`|EnumEquality` (`CharacterMovementComponent.MovementMode` (`Character.CharacterMovement` (`self.VPPlayerRef`))) "MOVE_Walking")
        (set `self.IsShouldJump` true))
      (bind _outhit (`KismetSystemLibrary.LineTraceSingle` _returnvalue (+ _returnvalue (* (`KismetMathLibrary.GetForwardVector` (`SceneComponent.K2_GetComponentRotation` (`/Game/FirstPerson/Blueprints/BP_FirstPersonCharacter.FirstPersonCamera` (`self.VPPlayerRef`)))) (`.GrapplingHookRange_59_36A243B849844445487679B0A3331754` (break `/Game/_VisionProtocol/Core/Structures/SPlayerParkourData` (`/Game/_VisionProtocol/Core/Parkour/BP_CharacterParkourComponent.PlayerParkourData` (`/Game/_VisionProtocol/Core/BP_VPPlayerCharacter.BP_CharacterParkourComponent` (`self.VPPlayerRef`))))))) "TraceTypeQuery1" false (`|MakeArray` (`self.VPPlayerRef`) :!type "Actor Object Reference")))
      (if (`GameplayStatics.BreakHitResult` _outhit)
        (set `self.GrapplingDirection` (`.ImpactPoint` (`GameplayStatics.BreakHitResult` _outhit)))
        (`/Game/_VisionProtocol/Core/Parkour/BP_CharacterParkourComponent.ParkourResetAirJump` (`/Game/_VisionProtocol/Core/BP_VPPlayerCharacter.BP_CharacterParkourComponent` (`self.VPPlayerRef`)))
        (`BlueprintGameplayTagLibrary.AddGameplayTag` (`/Game/_VisionProtocol/Core/Parkour/BP_CharacterParkourComponent.ParkourTags` (`/Game/_VisionProtocol/Core/BP_VPPlayerCharacter.BP_CharacterParkourComponent` (`self.VPPlayerRef`))) (struct :`TagName` "Player.GrapplingHook"))
        (`SceneComponent.SetVisibility` (`/Game/_VisionProtocol/Core/BP_VPPlayerCharacter.GrapplingHookRope` (`self.VPPlayerRef`)) true false)
        (if (`self.IsShouldJump`)
          (`/Game/_VisionProtocol/Core/Parkour/BP_CharacterParkourComponent.HelJump` (`/Game/_VisionProtocol/Core/BP_VPPlayerCharacter.BP_CharacterParkourComponent` (`self.VPPlayerRef`))))
        (bind _asbp_vpplayer_controller (cast `/Game/_VisionProtocol/Core/BP_VPPlayerController` (`Pawn.GetController` (`self.VPPlayerRef`))))
        (`/Game/_VisionProtocol/Core/BP_VPPlayerController.InitiateGrapplingHookContext` _asbp_vpplayer_controller)
        (bind _returnvalue_2 (`KismetSystemLibrary.K2_SetTimerDelegate` (delegate `GrapplingHookActivateCooldown`) (`.GrapplingHookCooldown_62_FCF41DF9475FB63A5D68688C06132142` (break `/Game/_VisionProtocol/Core/Structures/SPlayerParkourData` (`/Game/_VisionProtocol/Core/Parkour/BP_CharacterParkourComponent.PlayerParkourData` (`/Game/_VisionProtocol/Core/BP_VPPlayerCharacter.BP_CharacterParkourComponent` (`self.VPPlayerRef`)))))))
        (set `self.CooldownHandle` _returnvalue_2)))))

(event `GrapplingHookActivateCooldown`
  (setmembers `/Game/_VisionProtocol/Core/Structures/SPlayerParkourData` :`StructRef` (`/Game/_VisionProtocol/Core/Parkour/BP_CharacterParkourComponent.PlayerParkourData` (`/Game/_VisionProtocol/Core/BP_VPPlayerCharacter.BP_CharacterParkourComponent` (`self.VPPlayerRef`))) :`GrapplingHookRemainingCooldown` 0.0))

(event `ContinueGrappling`
  (bind _returnvalue (- (`self.GrapplingDirection`) (`SceneComponent.K2_GetComponentLocation` (`Character.CapsuleComponent` (`self.VPPlayerRef`)))))
  (if (`BlueprintGameplayTagLibrary.HasTag` (`/Game/_VisionProtocol/Core/Parkour/BP_CharacterParkourComponent.ParkourTags` (`/Game/_VisionProtocol/Core/BP_VPPlayerCharacter.BP_CharacterParkourComponent` (`self.VPPlayerRef`))) (struct :`TagName` "Player.GrapplingHook") true)
    (set `CableComponent.EndLocation` (`KismetMathLibrary.InverseTransformLocation` (`self.GetTransform` (`self.VPPlayerRef`)) (`self.GrapplingDirection`)) (`/Game/_VisionProtocol/Core/BP_VPPlayerCharacter.GrapplingHookRope` (`self.VPPlayerRef`)))
    (set `MovementComponent.Velocity` (* (/ _returnvalue (`KismetMathLibrary.VSize` _returnvalue)) (`.GrapplingHookGrapplingSpeed_56_B828C7E242FE5740D0B55AB519EDCA4B` (break `/Game/_VisionProtocol/Core/Structures/SPlayerParkourData` (`/Game/_VisionProtocol/Core/Parkour/BP_CharacterParkourComponent.PlayerParkourData` (`/Game/_VisionProtocol/Core/BP_VPPlayerCharacter.BP_CharacterParkourComponent` (`self.VPPlayerRef`)))))) (`Character.CharacterMovement` (`self.VPPlayerRef`)))
    (bind _asbp_vpplayer_controller (cast `/Game/_VisionProtocol/Core/BP_VPPlayerController` (`Pawn.GetController` (`self.VPPlayerRef`))))
    (`/Game/_VisionProtocol/Core/BP_VPPlayerController.InitiateGrapplingHookContext` _asbp_vpplayer_controller)))

(event `ExitGrappling`
  (if (`BlueprintGameplayTagLibrary.HasTag` (`/Game/_VisionProtocol/Core/Parkour/BP_CharacterParkourComponent.ParkourTags` (`/Game/_VisionProtocol/Core/BP_VPPlayerCharacter.BP_CharacterParkourComponent` (`self.VPPlayerRef`))) (struct :`TagName` "Player.GrapplingHook") true)
    (`BlueprintGameplayTagLibrary.RemoveGameplayTag` (`/Game/_VisionProtocol/Core/Parkour/BP_CharacterParkourComponent.ParkourTags` (`/Game/_VisionProtocol/Core/BP_VPPlayerCharacter.BP_CharacterParkourComponent` (`self.VPPlayerRef`))) (struct :`TagName` "Player.GrapplingHook"))
    (set `MovementComponent.Velocity` (0.0 0.0 0.0) (`Character.CharacterMovement` (`self.VPPlayerRef`)))
    (`SceneComponent.SetVisibility` (`/Game/_VisionProtocol/Core/BP_VPPlayerCharacter.GrapplingHookRope` (`self.VPPlayerRef`)) false false)
    (bind _asbp_vpplayer_controller (cast `/Game/_VisionProtocol/Core/BP_VPPlayerController` (`Pawn.GetController` (`self.VPPlayerRef`))))
    (`/Game/_VisionProtocol/Core/BP_VPPlayerController.ExitGrapplingHookContext` _asbp_vpplayer_controller)
    (`/Game/_VisionProtocol/Core/Parkour/BP_CharacterParkourComponent.ParkourLand` (`/Game/_VisionProtocol/Core/BP_VPPlayerCharacter.BP_CharacterParkourComponent` (`self.VPPlayerRef`)))))

(fn `UserConstructionScript`
  (`parent.UserConstructionScript`))
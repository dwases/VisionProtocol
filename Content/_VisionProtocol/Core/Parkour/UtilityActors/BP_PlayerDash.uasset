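; BP_PlayerDash is a parkour utility actor that performs the player's dash.
; PerformifPossible checks cooldown and the dash skill tag, then tags the player as dashing and starts a cooldown timer.
; A timeline drives CharacterMovement velocity along the normalized last input direction, scaled by a speed multiplier, and removes the tag when finished.
; Tick mirrors the timer's remaining time into the parkour component's data, and timer expiry zeroes it.
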(event `self.ReceiveTick`
  (params (DeltaSeconds :type "Float (single-precision)"))
  (if (`KismetSystemLibrary.K2_IsValidTimerHandle` (`self.CooldownHandle`))
    (setmembers `/Game/_VisionProtocol/Core/Structures/SPlayerParkourData` :`StructRef` (`/Game/_VisionProtocol/Core/Parkour/BP_CharacterParkourComponent.PlayerParkourData` (`/Game/_VisionProtocol/Core/BP_VPPlayerCharacter.BP_CharacterParkourComponent` (`self.VPPlayerRef`))) :`DashCurrCooldown` (`KismetSystemLibrary.K2_GetTimerRemainingTimeHandle` (`self.CooldownHandle`)))))

(event `self.ReceiveBeginPlay`
  (bind _asbp_vpplayer_character (cast `/Game/_VisionProtocol/Core/BP_VPPlayerCharacter` (`GameplayStatics.GetPlayerCharacter` 0)))
  (set `self.VPPlayerRef` _asbp_vpplayer_character))

(event `DashActivateCooldown`
  (setmembers `/Game/_VisionProtocol/Core/Structures/SPlayerParkourData` :`StructRef` (`/Game/_VisionProtocol/Core/Parkour/BP_CharacterParkourComponent.PlayerParkourData` (`/Game/_VisionProtocol/Core/BP_VPPlayerCharacter.BP_CharacterParkourComponent` (`self.VPPlayerRef`))) :`DashCurrCooldown` 0.0))

(event `/Game/_VisionProtocol/Core/Parkour/Interfaces/BPI_PlayerParkourSkill.PerformIfPossible`
  (params (ParkourData :type "/Game/_VisionProtocol/Core/Structures/SPlayerParkourData Structure") (ParkourTags :type "GameplayTagContainer Structure"))
  (bind _returnvalue (`Pawn.GetLastMovementInputVector` (`self.VPPlayerRef`)))
  ;[1 1 1] check dashing conditions
  (if (and (<= (`.DashCurrCooldown_13_211CAE20488CA8E070EFE1AE655A2565` (break `/Game/_VisionProtocol/Core/Structures/SPlayerParkourData` ParkourData)) 0.0) (`BlueprintGameplayTagLibrary.HasTag` ParkourTags (struct :`TagName` "Player.AvailableSkill.Dash") true))
    (set `self.DashDirection` (/ _returnvalue (`KismetMathLibrary.VSize` _returnvalue)))
    (`|ExecutionSequence`
      (:`then_0`
        (`BlueprintGameplayTagLibrary.AddGameplayTag` (`/Game/_VisionProtocol/Core/Parkour/BP_CharacterParkourComponent.ParkourTags` (`/Game/_VisionProtocol/Core/BP_VPPlayerCharacter.BP_CharacterParkourComponent` (`self.VPPlayerRef`))) (struct :`TagName` "Player.Dash"))
        (bind _returnvalue_2 (`KismetSystemLibrary.K2_SetTimerDelegate` (delegate `DashActivateCooldown`) (`.DashMaxCooldown_11_7925F6AE4B3EDB6A7BF4FFAF694A6688` (break `/Game/_VisionProtocol/Core/Structures/SPlayerParkourData` (`/Game/_VisionProtocol/Core/Parkour/BP_CharacterParkourComponent.PlayerParkourData` (`/Game/_VisionProtocol/Core/BP_VPPlayerCharacter.BP_CharacterParkourComponent` (`self.VPPlayerRef`)))))))
        (set `self.CooldownHandle` _returnvalue_2))
      (:`then_1`
        (bind (_direction _dashvelocity) (`Timeline|DashTL` :!via `PlayFromStart`)
          (:`Update`
            (set `MovementComponent.Velocity` (* (`self.DashDirection`) (* _dashvelocity (`.DashSpeedMultiplier_20_C8C78EE749CC892ABC71EB8F2887A1EE` (break `/Game/_VisionProtocol/Core/Structures/SPlayerParkourData` (`/Game/_VisionProtocol/Core/Parkour/BP_CharacterParkourComponent.PlayerParkourData` (`/Game/_VisionProtocol/Core/BP_VPPlayerCharacter.BP_CharacterParkourComponent` (`self.VPPlayerRef`))))))) (`Character.CharacterMovement` (`self.VPPlayerRef`))))
          (:`Finished`
            (`BlueprintGameplayTagLibrary.RemoveGameplayTag` (`/Game/_VisionProtocol/Core/Parkour/BP_CharacterParkourComponent.ParkourTags` (`/Game/_VisionProtocol/Core/BP_VPPlayerCharacter.BP_CharacterParkourComponent` (`self.VPPlayerRef`))) (struct :`TagName` "Player.Dash"))))))))

(fn `UserConstructionScript`)
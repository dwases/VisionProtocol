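; Player interaction component that detects interactable objects in view and lets the player use them.
; Each tick it line-traces from the first-person camera out to the interaction range, caching any hit actor implementing BPI_Interactable and its component.
; An on-screen prompt widget created at BeginPlay shows that target's action name and hides otherwise.
; AttemptInteract calls Interact on the cached target, passing the owner and hit component.
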(event `self.ReceiveBeginPlay`
  (bind _returnvalue (`|CreateWidget` "/Game/_VisionProtocol/Core/InteractionFramework/WBP_InteractPrompt.WBP_InteractPrompt_C"))
  (bind _output_get (set `self.InteractionWidgetRef` _returnvalue))
  (`UserWidget.AddToViewport` _output_get 0))

(event `self.ReceiveTick`
  (params (DeltaSeconds :type "Float (single-precision)"))
  (bind _interactionwidgetref (`self.InteractionWidgetRef`))
  (bind _asbp_first_person_character (cast `/Game/FirstPerson/Blueprints/BP_FirstPersonCharacter` (`self.GetOwner`)))
  (bind _firstpersoncamera (`/Game/FirstPerson/Blueprints/BP_FirstPersonCharacter.FirstPersonCamera` _asbp_first_person_character))
  (bind (_outhit _returnvalue) (`KismetSystemLibrary.LineTraceSingle` (`SceneComponent.K2_GetComponentLocation` (`/Game/FirstPerson/Blueprints/BP_FirstPersonCharacter.FirstPersonCamera` _asbp_first_person_character)) (+ (* (`SceneComponent.GetForwardVector` _firstpersoncamera) (`.InteractionRange_2_9E87CBB6468D34BE9FF8FF915E787939` (break `/Game/_VisionProtocol/Core/InteractionFramework/SInteractionFrameworkData` (`self.InteractionData`)))) (`SceneComponent.K2_GetComponentLocation` _firstpersoncamera)) "TraceTypeQuery1" false (`|MakeArray` _asbp_first_person_character :!type "Actor Object Reference")))
  (if _returnvalue
    (bind _asbpi_interactable (cast `/Game/_VisionProtocol/Core/InteractionFramework/BPI_Interactable` (`.HitActor` (`GameplayStatics.BreakHitResult` _outhit)))
      (:`then`
        (set `self.HitActor` (`.HitActor` (`GameplayStatics.BreakHitResult` _outhit)))
        (set `self.HitComponent` (`.HitComponent` (`GameplayStatics.BreakHitResult` _outhit)))
        (set `self.IsCanInteract` true)
        (`Widget.SetVisibility` _interactionwidgetref "Visible")
        (bind _interactionname (`/Game/_VisionProtocol/Core/InteractionFramework/BPI_Interactable.GetInteractionName` _asbpi_interactable))
        (set `/Game/_VisionProtocol/Core/InteractionFramework/WBP_InteractPrompt.CurrentActionName` _interactionname _interactionwidgetref))
      (:`CastFailed`
        (set `self.IsCanInteract` false :!label _label)
        (`Widget.SetVisibility` (`self.InteractionWidgetRef`) "Hidden")))
    (else
      (goto _label))))

(event `AttemptInteract`
  (bind _hitactor (`self.HitActor`))
  (if (`self.IsCanInteract`)
    (`/Engine/EditorBlueprintResources/StandardMacros.IsValid` _hitactor
      (:`Is Valid`
        (bind _asbpi_interactable (cast `/Game/_VisionProtocol/Core/InteractionFramework/BPI_Interactable` _hitactor))
        (`/Game/_VisionProtocol/Core/InteractionFramework/BPI_Interactable.Interact` _asbpi_interactable (`self.GetOwner`) (`self.HitComponent`))))))
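; Player character variant, apparently for the ending sequence: input is disabled on BeginPlay, while step noise, level loading and visor status are stubbed out.
; The CDMGHP component holds health; damage and healing update screen feedback and a looping-state low-health sound below 30%.
; Death shows a temporary WBP_Death widget, and the OnDeath dispatcher triggers a delayed Timeline moving the first-person camera to a fixed world pose.
; Quest, sandbox and visor startup logic is disconnected.
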(event `Steps Noise`
  ;[1 1 1] Backendowy hałas z kroków do AI oraz chwilowe wyswietlanie HP
)

(event `self.ReceiveBeginPlay`
  (`self.DisableInput` (`GameplayStatics.GetPlayerController` 0))
  (add `self.OnDeath` (delegate `DoOnDeath`)))

(event `DoOnDeath`
  (`KismetSystemLibrary.Delay` 2.0)
  (bind (_direction _newtrack_0) (`Timeline|Timeline`)
    (:`Update`
      (`SceneComponent.K2_SetWorldLocationAndRotation` (`self.FirstPersonCamera`) (`KismetMathLibrary.VLerp` (`KismetMathLibrary.MakeVector` 14430.0 9580.0 102000.0) (`KismetMathLibrary.MakeVector` 11654.81 7286.45 104136.0) _newtrack_0) (struct :`Pitch` -32.6 :`Yaw` 33.6) false false))))

(event `EventOnDeath`
  (bind _returnvalue (`|CreateWidget` "/Game/_VisionProtocol/Widgets/WBP_Death.WBP_Death_C"))
  (`UserWidget.AddToViewport` _returnvalue 0)
  (`self.OnDeath`)
  (`KismetSystemLibrary.Delay` 3.0)
  (`Widget.RemoveFromParent` _returnvalue))

(event `LoadLevel`
  (params (MapName :type Name) (Options :type String)))

(fn `Get Q Visor Status`
  (returns (Activated :type Boolean)))

(fn `GetCurrentHealth`
  (returns (Health :type "Float (double-precision)"))
  (return (`/Game/_VisionProtocol/Core/DMG-HP/C_DMG-HP.CurrentHealth` (`self.C_DMG-HP`))))

(fn `GetMaxHealth`
  (returns (MaxHealth :type "Float (double-precision)"))
  (return (`/Game/_VisionProtocol/Core/DMG-HP/C_DMG-HP.MaximumHealth` (`self.C_DMG-HP`))))

(fn `GetParkourComponent`
  (returns (Component :type "/Game/_VisionProtocol/Core/Parkour/BP_CharacterParkourComponent Object Reference"))
  (return null))

(fn `Heal`
  (params (HP_Amount :type "Float (double-precision)"))
  (returns (`New Health` :type "Float (double-precision)"))
  (bind _lowhpsound (`self.LowHPSound`))
  (bind _new_health (`/Game/_VisionProtocol/Core/DMG-HP/C_DMG-HP.Heal` (`self.C_DMG-HP`) HP_Amount))
  (`/Game/_VisionProtocol/Core/DMG-HP/C_DMG-HP.PlayerUpdateDamagedScreen` (`self.C_DMG-HP`))
  (bind _hp_ (`/Game/_VisionProtocol/Core/DMG-HP/C_DMG-HP.ReturnPercent` (`self.C_DMG-HP`)))
  (if (or (>= _hp_ 0.3) (<= _hp_ 0.0))
    (`/Engine/EditorBlueprintResources/StandardMacros.IsValid` _lowhpsound
      (:`Is Valid`
        (`AudioComponent.FadeOut` _lowhpsound 1.0 0.0 "Logarithmic")
        (`ActorComponent.K2_DestroyComponent` _lowhpsound)
        (set `self.LowHPSound` null))
      (:`Is Not Valid`
        _)))
  (return _new_health))

(fn `IsDead`
  (returns (Dead :type Boolean))
  (return (`/Game/_VisionProtocol/Core/DMG-HP/C_DMG-HP.isDead` (`self.C_DMG-HP`))))

(fn `TakeDamage`
  (params (Amount :type "Float (double-precision)"))
  (returns (`Was Damaged` :type Boolean))
  (bind _lowhpsound (`self.LowHPSound`))
  (bind _was_damaged (`/Game/_VisionProtocol/Core/DMG-HP/C_DMG-HP.TakeDamage` (`self.C_DMG-HP`) Amount))
  (`/Game/_VisionProtocol/Core/DMG-HP/C_DMG-HP.PlayerDamageResponse` (`self.C_DMG-HP`))
  (`/Game/_VisionProtocol/Core/DMG-HP/C_DMG-HP.PlayerUpdateDamagedScreen` (`self.C_DMG-HP`))
  (bind _dead (`self.IsDead`))
  (if (not _dead)
    (`GameplayStatics.PlaySound2D` "/Game/_VisionProtocol/Audio/SFX/getHit.getHit" 1.0 1.0 0.0 null null false)
    (bind _hp_ (`/Game/_VisionProtocol/Core/DMG-HP/C_DMG-HP.ReturnPercent` (`self.C_DMG-HP`)))
    (if (and (< _hp_ 0.3) (> _hp_ 0.0))
      (`/Engine/EditorBlueprintResources/StandardMacros.IsValid` (`self.LowHPSound`)
        (:`Is Not Valid`
          (bind _returnvalue (`GameplayStatics.SpawnSound2D` "/Game/_VisionProtocol/Audio/SFX/lowHP.lowHP" 1.0 1.0 0.0 null))
          (set `self.LowHPSound` _returnvalue)))
      (else
        (`/Engine/EditorBlueprintResources/StandardMacros.IsValid` _lowhpsound
          (:`Is Valid`
            (`ActorComponent.K2_DestroyComponent` _lowhpsound))))))
  (return _was_damaged))

(fn `UserConstructionScript`
  (bind _c_dmg_hp (`self.C_DMG-HP`))
  (`parent.UserConstructionScript`)
  (`SceneComponent.K2_SetWorldRotation` (`self.FirstPersonCamera`) (struct :`Pitch` -90.0) false false)
  (add `/Game/_VisionProtocol/Core/DMG-HP/C_DMG-HP.OnDeath` _c_dmg_hp (`|CreateDelegate` :!event `EventOnDeath`))
  (bind _output_get (set `/Game/_VisionProtocol/Core/DMG-HP/C_DMG-HP.MaximumHealth` 100.0 _c_dmg_hp))
  (set `/Game/_VisionProtocol/Core/DMG-HP/C_DMG-HP.CurrentHealth` _output_get _c_dmg_hp))
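; Game mode that handles persistent music and the world-side Spectovisor visor effects and quest marker.
; Music events crossfade, pause and resume a 2D sound that survives level transitions.
; Visor activation applies overlay materials to interactable and damageable actors' meshes; deactivation clears only those materials.
; Activation also shows a marker spawned at BeginPlay, then moves it to the active quest location, hiding it if the quest's map differs.
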(event `self.PlayMusic`
  (params (Music :type "SoundBase Object Reference") (OldFadeOutTime :type "Float (double-precision)") (NewFadeInTime :type "Float (double-precision)"))
  (set `self.Music` Music)
  (set `self.Old Fade Out Time` OldFadeOutTime)
  (set `self.New Fade in Time` NewFadeInTime)
  (`/Engine/EditorBlueprintResources/StandardMacros.IsValid` (`self.ActiveMusicPlayer`)
    (:`Is Valid`
      (`self.StopMusic` (`self.Old Fade Out Time`)))
    (:`Is Not Valid`
      _))
  (bind _returnvalue (`GameplayStatics.CreateSound2D` (`self.Music`) 1.0 1.0 0.0 null true))
  (bind _output_get (set `self.ActiveMusicPlayer` _returnvalue))
  (`AudioComponent.FadeIn` _output_get (`self.New Fade in Time`) 1.0 0.0 "Linear"))

(event `self.StopMusic`
  (params (FadeOutTime :type "Float (double-precision)"))
  (bind _output_get (set `self.FadeOutMusicPlayer` (`self.ActiveMusicPlayer`)))
  (`AudioComponent.FadeOut` _output_get FadeOutTime 0.0 "Linear"))

(event `self.PauseMusic`
  (`AudioComponent.SetPaused` (`self.ActiveMusicPlayer`) true))

(event `self.ResumeMusic`
  (`AudioComponent.SetPaused` (`self.ActiveMusicPlayer`) false))

(event `self.ReceiveBeginPlay`
  (bind _asbp_vpplayer_character (cast `/Game/_VisionProtocol/Core/BP_VPPlayerCharacter` (`GameplayStatics.GetPlayerPawn` 0)))
  (bind _c_visors (`/Game/_VisionProtocol/Core/BP_VPPlayerCharacter.C_Visors` _asbp_vpplayer_character))
  (add `/Game/_VisionProtocol/Core/Visors/C_Visors.ONSActivation` _c_visors (`|CreateDelegate` :!event `SActivationResponse`))
  (add `/Game/_VisionProtocol/Core/Visors/C_Visors.ONSDeactivation` _c_visors (`|CreateDelegate` :!event `SDeactivationResponse`))
  (bind _asbp_vpplayer_character_2 (cast `/Game/_VisionProtocol/Core/BP_VPPlayerCharacter` (`GameplayStatics.GetPlayerPawn` 0)))
  ;[1 1 1] lokacja nie ma znaczenia; jest aktualizowana przy wlaczeniu spectovisora i tak
  (bind _returnvalue (`|SpawnActorFromClass` "/Game/_VisionProtocol/Core/QuestManagementFramework/BP_QuestMarker.BP_QuestMarker_C" (`KismetMathLibrary.Conv_VectorToTransform` (`KismetMathLibrary.MakeVector` 500.0 500.0 500.0)) "Undefined" "MultiplyWithRoot" null null))
  (bind _output_get (set `self.WorldQuestMarker` _returnvalue))
  (`Widget.SetVisibility` (`WidgetComponent.GetWidget` (`/Game/_VisionProtocol/Core/QuestManagementFramework/BP_QuestMarker.Widget` _output_get)) "Hidden"))

(event `SActivationResponse`
  (bind _outactors (`GameplayStatics.GetAllActorsWithInterface` "/Game/_VisionProtocol/Core/InteractionFramework/BPI_Interactable.BPI_Interactable_C"))
  (`self.Update Actor Overlay Materials` _outactors (`self.SpectovisorInteractableMI`))
  (bind _outactors_2 (`GameplayStatics.GetAllActorsWithInterface` "/Game/_VisionProtocol/Core/DMG-HP/BPI_Damageable.BPI_Damageable_C"))
  (`self.Update Actor Overlay Materials` _outactors_2 (`self.SpectovisorDamageableMI`))
  (`Widget.SetVisibility` (`WidgetComponent.GetWidget` (`/Game/_VisionProtocol/Core/QuestManagementFramework/BP_QuestMarker.Widget` (`self.WorldQuestMarker`))) "Visible")
  (`self.UpdateQuestMarkerData`))

(event `SDeactivationResponse`
  (bind _outactors (`GameplayStatics.GetAllActorsWithInterface` "/Game/_VisionProtocol/Core/InteractionFramework/BPI_Interactable.BPI_Interactable_C"))
  (`self.Clear Specific Actor Overlay MaterialInstance` (`self.SpectovisorInteractableMI`) _outactors)
  (bind _outactors_2 (`GameplayStatics.GetAllActorsWithInterface` "/Game/_VisionProtocol/Core/DMG-HP/BPI_Damageable.BPI_Damageable_C"))
  (`self.Clear Specific Actor Overlay MaterialInstance` (`self.SpectovisorDamageableMI`) _outactors_2))

(event `UpdateQuestMarkerData`
  (`KismetSystemLibrary.Delay` 0.08)
  (bind _asbp_vpplayer_character (cast `/Game/_VisionProtocol/Core/BP_VPPlayerCharacter` (`GameplayStatics.GetPlayerPawn` 0)))
  (bind _returnvalue (`GameplayStatics.GetCurrentLevelName` true))
  (bind ((`Description_4_B1DE3FA7440CFCAACFA1FE88A3ABB276` _description) (`QuestMarkerLocation_27_E0F34FDE4732F3FD2B7565BC3BA48D7F` _questmarkerlocation) (`QuestMap_30_D3C85AC04DD9252B953782A41E602F07` _questmap) (`MapName_33_D8A3F5DA4FD8A21D38207A8A7E68F5BC` _mapname)) (break `/Game/_VisionProtocol/Core/QuestManagementFramework/SQuest` (`/Game/_VisionProtocol/Core/QuestManagementFramework/BP_PlayerQuestTrackerComponent.ActiveQuest` (`self.GetComponentByClass` _asbp_vpplayer_character "/Game/_VisionProtocol/Core/QuestManagementFramework/BP_PlayerQuestTrackerComponent.BP_PlayerQuestTrackerComponent_C"))))
  (if (not (`KismetStringLibrary.EqualEqual_StrStr` _returnvalue (`KismetTextLibrary.Conv_TextToString` _mapname)))
    (`Widget.SetVisibility` (`WidgetComponent.GetWidget` (`/Game/_VisionProtocol/Core/QuestManagementFramework/BP_QuestMarker.Widget` (`self.WorldQuestMarker`))) "Hidden"))
  ;[1 1 1] Update waypoint world location
  (`self.K2_SetActorLocation` (`self.WorldQuestMarker`) _questmarkerlocation false false)
  ;[1 1 1] Update waypoint description
  (bind _aswbp_waypoint (cast `/Game/_VisionProtocol/Core/QuestManagementFramework/WBP_Waypoint` (`WidgetComponent.GetWidget` (`/Game/_VisionProtocol/Core/QuestManagementFramework/BP_QuestMarker.Widget` (`self.WorldQuestMarker`)))))
  (`/Game/_VisionProtocol/Core/QuestManagementFramework/WBP_Waypoint.UpdateQuestDescriptionText` _aswbp_waypoint))

(fn `Clear Specific Actor Overlay MaterialInstance`
  (params (`MaterialInstanceTo Clear` :type "MaterialInstance Object Reference") (Actors :type "Array of Actor Object Reference"))
  (for _array_element Actors
    (for _array_element_2 (`self.K2_GetComponentsByClass` _array_element "/Script/Engine.StaticMeshComponent")
      (if (== (`MeshComponent.GetOverlayMaterial` _array_element_2) `MaterialInstanceTo Clear`)
        (`MeshComponent.SetOverlayMaterial` _array_element_2 null)))
    (for _array_element_3 (`self.K2_GetComponentsByClass` _array_element "/Script/Engine.SkeletalMeshComponent")
      (if (== (`MeshComponent.GetOverlayMaterial` _array_element_3) `MaterialInstanceTo Clear`)
        (`MeshComponent.SetOverlayMaterial` _array_element_3 null)))))

(fn `Update Actor Overlay Materials`
  (params (Actors :type "Array of Actor Object Reference") (TargetOverlayMaterial :type "MaterialInstance Object Reference"))
  (for _array_element Actors
    (for _array_element_2 (`self.K2_GetComponentsByClass` _array_element "/Script/Engine.StaticMeshComponent")
      (`MeshComponent.SetOverlayMaterial` _array_element_2 TargetOverlayMaterial))
    (for _array_element_3 (`self.K2_GetComponentsByClass` _array_element "/Script/Engine.SkeletalMeshComponent")
      (`MeshComponent.SetOverlayMaterial` _array_element_3 TargetOverlayMaterial))))

(fn `UserConstructionScript`
  (`parent.UserConstructionScript`))
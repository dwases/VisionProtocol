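; BP_TestQuestObject is a test interactable actor that feeds an objective tag into the quest system.
; On Interact, it finds BP_PlayerQuestManager on the player pawn, adds its ObjectiveTag, then destroys itself after a short delay.
; It also supplies its interaction name and always shows the interact key widget.
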(event `/Game/_VisionProtocol/Core/InteractionFramework/BPI_Interactable.Interact`
  (params (Interactor :type "Actor Object Reference") (InteracteeComponent :type "PrimitiveComponent Object Reference"))
  (`/Game/_VisionProtocol/Core/QuestManagementFramework/BP_PlayerQuestManager.AddTag` (`self.GetComponentByClass` (`GameplayStatics.GetPlayerPawn` 0) "/Game/_VisionProtocol/Core/QuestManagementFramework/BP_PlayerQuestManager.BP_PlayerQuestManager_C") (`self.ObjectiveTag`))
  (`KismetSystemLibrary.Delay` 0.2)
  (`self.K2_DestroyActor`))

(fn `GetInteractionName`
  (returns (InteractionName :type Text))
  (return (`self.InteractionName`)))

(fn `GetIsInteractKeyWidgetVisible`
  (returns (IsInteractKeyWidgetVisible :type Boolean))
  (return true))

(fn `UserConstructionScript`)
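; BP_QuestMarker is a quest waypoint actor that shows its distance from the player through a WBP_Waypoint widget component.
; On BeginPlay it caches the widget's distance text and binds to the S activation and deactivation events on the player's CVisors component.
; Those events show and hide the widget.
; Every Tick rewrites the text with the player distance, converted to whole meters.
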(event `self.ReceiveBeginPlay`
  (bind _aswbp_waypoint (cast `/Game/_VisionProtocol/Core/QuestManagementFramework/WBP_Waypoint` (`WidgetComponent.GetWidget` (`self.Widget`))))
  (set `self.Distance Text` (`/Game/_VisionProtocol/Core/QuestManagementFramework/WBP_Waypoint.DistanceText` _aswbp_waypoint))
  (bind _asbp_vpplayer_character (cast `/Game/_VisionProtocol/Core/BP_VPPlayerCharacter` (`GameplayStatics.GetPlayerPawn` 0)))
  (bind _c_visors (`/Game/_VisionProtocol/Core/BP_VPPlayerCharacter.C_Visors` _asbp_vpplayer_character))
  (add `/Game/_VisionProtocol/Core/Visors/C_Visors.ONSActivation` _c_visors (delegate `SActivationResponse`))
  (add `/Game/_VisionProtocol/Core/Visors/C_Visors.ONSDeactivation` _c_visors (delegate `SDeactivationResponse`)))

(event `SActivationResponse`
  (`SceneComponent.SetVisibility` (`self.Widget`) true true))

(event `SDeactivationResponse`
  (`SceneComponent.SetVisibility` (`self.Widget`) false true))

(event `self.ReceiveTick`
  (params (DeltaSeconds :type "Float (single-precision)"))
  (`TextBlock.SetText` (`self.Distance Text`) (`self.GetDistanceText`)))

(fn `GetDistanceText`
  (returns (ReturnValue :type Text))
  (return (`KismetTextLibrary.Conv_StringToText` (`KismetStringLibrary.Concat_StrStr` (`KismetStringLibrary.Conv_IntToString` (`KismetMathLibrary.FTrunc` (/ (`KismetMathLibrary.Vector_Distance` (`self.K2_GetActorLocation`) (`self.K2_GetActorLocation` (`GameplayStatics.GetPlayerCharacter` 0))) 100.0))) " m"))))

(fn `UserConstructionScript`)
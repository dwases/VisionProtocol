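; Player quest manager that stores quest gameplay tags in a container and notifies listeners when they change.
; AddTag and RemoveTag update CurrentTags, then NotifyTagChange broadcasts the changed tag and container through that tag's own event dispatcher.
; AddListener and RemoveListener bind or unbind events by tag, using hard-coded tag switches, so only the listed objective and test quest tags have notifications.
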(event `Signature` :!signature `self.TagListener`
  (params (TagChanged :type "GameplayTag Structure") (CurrentTags :type "GameplayTagContainer Structure")))

(fn `AddListener`
  (params (Event :type "Delegate (by ref)") (GameplayTagToListenTo :type "GameplayTag Structure"))
  (`|SwitchGameplayTag` GameplayTagToListenTo
    (:`Quest.Objectives.InteractWithObject`
      (add `self.InteractWithObject` Event))
    (:`Quest.Testing.Quest1Testowy`
      (add `self.Quest1Testowy` Event))
    (:`Quest.Testing.Quest2Testowy`
      (add `self.Quest2Testowy` Event))))

(fn `AddTag`
  (params (Tag :type "GameplayTag Structure"))
  (`BlueprintGameplayTagLibrary.AddGameplayTag` (`self.CurrentTags`) Tag)
  (`self.NotifyTagChange` Tag))

(fn `NotifyTagChange`
  (params (GameplayTag :type "GameplayTag Structure"))
  (bind _currenttags (`self.CurrentTags`))
  (`|SwitchGameplayTag` GameplayTag
    (:`Quest.Objectives.InteractWithObject`
      (`self.InteractWithObject` GameplayTag _currenttags))
    (:`Quest.Testing.Quest1Testowy`
      (`self.Quest1Testowy` GameplayTag _currenttags))
    (:`Quest.Testing.Quest2Testowy`
      (`self.Quest2Testowy` GameplayTag _currenttags))))

(fn `RemoveListener`
  (params (Event :type "Delegate (by ref)") (GameplayTagToRemove :type "GameplayTag Structure"))
  (`|SwitchGameplayTag` GameplayTagToRemove
    (:`Quest.Objectives.InteractWithObject`
      (remove `self.InteractWithObject` Event))
    (:`Quest.Testing.Quest1Testowy`
      (remove `self.Quest1Testowy` Event))
    (:`Quest.Testing.Quest2Testowy`
      (remove `self.Quest2Testowy` Event))))

(fn `RemoveTag`
  (params (Tag :type "GameplayTag Structure"))
  (`BlueprintGameplayTagLibrary.RemoveGameplayTag` (`self.CurrentTags`) Tag)
  (`self.NotifyTagChange` Tag))
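; Logo component in the quest management framework that displays a marker on its owning actor and can be shown or hidden through events.
; On BeginPlay it spawns its own BP_VPLogoOnActorService actor at the component's transform and starts logo rotation.
; Rotation is delegated to that service, which receives the component itself, while a custom event can trigger the same call again.
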(event `ShowLogo`
  (`self.SetVisibility` true))

(event `HideLogo`
  (`self.SetVisibility` false))

(event `CustomEvent`
  (`self.RotateLogo`))

(event `RotateLogo`
  (`/Game/_VisionProtocol/Core/QuestManagementFramework/BP_VPLogoOnActorService.RotateLogoService` (`self.LogoOnActorService`) self))

(event `self.ReceiveBeginPlay`
  (bind _returnvalue (`|SpawnActorFromClass` "/Game/_VisionProtocol/Core/QuestManagementFramework/BP_VPLogoOnActorService.BP_VPLogoOnActorService_C" (`self.K2_GetComponentToWorld`) "Undefined" "MultiplyWithRoot" null null))
  (set `self.LogoOnActorService` _returnvalue)
  (`self.RotateLogo`))
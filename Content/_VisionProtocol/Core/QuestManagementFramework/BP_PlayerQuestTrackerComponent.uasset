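; Player quest tracker component that holds available, active and completed quests, seeded with starting quests from the GameInstance.
; Only one quest is active: its objective gameplay tags become listeners on the pawn's BP_PlayerQuestManager, skipping already completed unique objectives.
; Tag callbacks record progress and finish the quest when completed-tag counts match its objective total.
; Completion adds linked quests, activating one if none is active, and refreshes BP_VPGameMode's quest markers.
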(event `StartQuests`
  (bind _startingquests (message `/Game/_VisionProtocol/Core/QuestManagementFramework/BPI_GameInstanceQuestingInterface.GetStartingQuests` (`GameplayStatics.GetGameInstance`)))
  (bind _output_get (set `self.StartingQuests` _startingquests))
  (for _array_element _output_get
    (`self.AddQuest` _array_element)))

(event `ObjectiveComplete`
  (params (TagChanged :type "GameplayTag Structure") (CurrentTags :type "GameplayTagContainer Structure"))
  (`BlueprintGameplayTagLibrary.AddGameplayTag` (`self.CompletedObjectives`) TagChanged)
  (`/Game/_VisionProtocol/Core/QuestManagementFramework/BP_PlayerQuestManager.RemoveListener` (`Actor.GetComponentByClass` (`GameplayStatics.GetPlayerPawn` 0) "/Game/_VisionProtocol/Core/QuestManagementFramework/BP_PlayerQuestManager.BP_PlayerQuestManager_C") (delegate `ObjectiveComplete`) TagChanged)
  (bind (_objectivesremaining _objectivestotal _objectivescomplete) (`self.Check Objectives Completed`))
  (if _objectivescomplete
    (`self.QuestCompleted`)
    (set `self.CompletedObjectives` (struct))))

(event `UniqueObjectiveCompleted`
  (params (TagChanged :type "GameplayTag Structure") (CurrentTags :type "GameplayTagContainer Structure"))
  (`BlueprintGameplayTagLibrary.AddGameplayTag` (`self.CompletedObjectives`) TagChanged)
  (`BlueprintGameplayTagLibrary.AddGameplayTag` (`self.CompletedUniqueObjectives`) TagChanged)
  (`/Game/_VisionProtocol/Core/QuestManagementFramework/BP_PlayerQuestManager.RemoveListener` (`Actor.GetComponentByClass` (`GameplayStatics.GetPlayerPawn` 0) "/Game/_VisionProtocol/Core/QuestManagementFramework/BP_PlayerQuestManager.BP_PlayerQuestManager_C") (delegate `UniqueObjectiveCompleted`) TagChanged)
  (bind (_objectivesremaining _objectivestotal _objectivescomplete) (`self.Check Objectives Completed`))
  (if _objectivescomplete
    (`self.QuestCompleted`)))

(fn `Activate Quest`
  (params (QuestToActivate :type "/Game/_VisionProtocol/Core/QuestManagementFramework/SQuest Structure"))
  (bind _returnvalue (`Actor.GetComponentByClass` (`GameplayStatics.GetPlayerPawn` 0) "/Game/_VisionProtocol/Core/QuestManagementFramework/BP_PlayerQuestManager.BP_PlayerQuestManager_C"))
  (bind _output_get (set `self.ActiveQuest` QuestToActivate))
  (bind (_name _description _status _uuidtag _tags _requiredquests _linkedquests _objectives _uniqueobjectives) (break `/Game/_VisionProtocol/Core/QuestManagementFramework/SQuest` _output_get))
  (for _array_element (`BlueprintGameplayTagLibrary.BreakGameplayTagContainer` _objectives)
    (`/Game/_VisionProtocol/Core/QuestManagementFramework/BP_PlayerQuestManager.AddListener` _returnvalue (`|CreateDelegate` :!event `ObjectiveComplete`) _array_element))
  (for _array_element_2 (`BlueprintGameplayTagLibrary.BreakGameplayTagContainer` _uniqueobjectives)
    (if (`BlueprintGameplayTagLibrary.HasTag` (`self.CompletedObjectives`) _array_element_2 true)
      (`BlueprintGameplayTagLibrary.AddGameplayTag` (`self.CompletedObjectives`) _array_element_2)
      (else
        (`/Game/_VisionProtocol/Core/QuestManagementFramework/BP_PlayerQuestManager.AddListener` _returnvalue (`|CreateDelegate` :!event `UniqueObjectiveCompleted`) _array_element_2)))
    ;[1 1 1] Update World Quest Widget Location
    (bind _asbp_vpgame_mode (cast `/Game/_VisionProtocol/Core/BP_VPGameMode` (`GameplayStatics.GetGameMode`)))
    (`/Game/_VisionProtocol/Core/BP_VPGameMode.UpdateQuestMarkerData` _asbp_vpgame_mode)))

(fn `AddQuest`
  (params (QuestToAdd :type "/Game/_VisionProtocol/Core/QuestManagementFramework/SQuest Structure"))
  ;[1 1 1] Add All Available Quests To Array
  (`KismetArrayLibrary.Array_AddUnique` (`self.AvailableQuests`) QuestToAdd)
  (`self.QuestAdded` QuestToAdd)
  ;[1 1 1] Proceed only if there is no active quest
  (if (== (`.UUIDTag_10_7803F5D3413822A32F2FDCABE73364FB` (break `/Game/_VisionProtocol/Core/QuestManagementFramework/SQuest` (`self.ActiveQuest`))) (struct))
    (`self.Activate Quest` QuestToAdd)))

(fn `Check Objectives Completed`
  (returns (ObjectivesRemaining :type Integer) (ObjectivesTotal :type Integer) (ObjectivesComplete :type Boolean))
  (bind (_name _description _status _uuidtag _tags _requiredquests _linkedquests _objectives _uniqueobjectives) (break `/Game/_VisionProtocol/Core/QuestManagementFramework/SQuest` (`self.ActiveQuest`)))
  (bind _returnvalue (+ (`BlueprintGameplayTagLibrary.GetNumGameplayTagsInContainer` _objectives) (`BlueprintGameplayTagLibrary.GetNumGameplayTagsInContainer` _uniqueobjectives)))
  (bind _returnvalue_2 (- _returnvalue (`self.GetCompletedObjectiveCount`)))
  (return _returnvalue_2 _returnvalue (== _returnvalue_2 0)))

(fn `GetCompletedObjectiveCount`
  (returns (ReturnValue :type Integer))
  (return (+ (`BlueprintGameplayTagLibrary.GetNumGameplayTagsInContainer` (`self.CompletedObjectives`)) (`BlueprintGameplayTagLibrary.GetNumGameplayTagsInContainer` (`self.CompletedUniqueObjectives`)))))

(fn `QuestCompleted`
  (locals (RecentlyCompletedQuest :type "/Game/_VisionProtocol/Core/QuestManagementFramework/SQuest Structure"))
  (bind _availablequests (`self.AvailableQuests`))
  (bind _activequest (`self.ActiveQuest`))
  ;[1 1 1] Add Completed Quest
  (`KismetArrayLibrary.Array_AddUnique` (`self.CompletedQuests`) _activequest)
  (set `local.RecentlyCompletedQuest` _activequest)
  ;[1 1 1] RemoveActiveQuest
  (`KismetArrayLibrary.Array_Remove` _availablequests (`KismetArrayLibrary.Array_Find` _availablequests (`self.ActiveQuest`)))
  (set `self.ActiveQuest` (struct))
  ;[1 1 1] Update World Quest Widget Location
  (bind _asbp_vpgame_mode (cast `/Game/_VisionProtocol/Core/BP_VPGameMode` (`GameplayStatics.GetGameMode`)))
  (`/Game/_VisionProtocol/Core/BP_VPGameMode.UpdateQuestMarkerData` _asbp_vpgame_mode)
  ;[1 1 1] Linked Quests Handling
  (for _array_element (`BlueprintGameplayTagLibrary.BreakGameplayTagContainer` (`.LinkedQuests_20_E4DF9BE24A2BB530DC05408FC1A799F4` (break `/Game/_VisionProtocol/Core/QuestManagementFramework/SQuest` (`local.RecentlyCompletedQuest`))))
    (bind (_isquestfound _returnedquest) (message `/Game/_VisionProtocol/Core/QuestManagementFramework/BPI_GameInstanceQuestingInterface.GetQuestByTag` (`GameplayStatics.GetGameInstance`) _array_element))
    (if _isquestfound
      (`self.AddQuest` _returnedquest)
      ;[1 1 1] Update World Quest Widget Location
      (bind _asbp_vpgame_mode_2 (cast `/Game/_VisionProtocol/Core/BP_VPGameMode` (`GameplayStatics.GetGameMode`)))
      (`/Game/_VisionProtocol/Core/BP_VPGameMode.UpdateQuestMarkerData` _asbp_vpgame_mode_2))))
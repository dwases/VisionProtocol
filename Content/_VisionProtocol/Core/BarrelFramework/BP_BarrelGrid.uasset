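; BP_BarrelGrid is a construction-time placement actor that builds a three-dimensional grid of barrel instances.
; Its construction script runs nested loops over the X, Y and Z barrel counts, adding each instance to the ISMBarrels instanced static mesh component at its index times the per-axis gap.
; The event graph holds only disabled default events, so it has no runtime logic.
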(fn `UserConstructionScript`
  (for _index (range (`self.XNumberOfBarrels`))
    (for _index_2 (range (`self.YNumberOfBarrels`))
      (for _index_3 (range (`self.ZNumberOfBarrels`))
        (`InstancedStaticMeshComponent.AddInstance` (`self.ISM_Barrels`) (`KismetMathLibrary.MakeTransform` (`KismetMathLibrary.MakeVector` (`KismetMathLibrary.Conv_IntToDouble` (* _index (`self.XGap`))) (`KismetMathLibrary.Conv_IntToDouble` (* _index_2 (`self.YGap`))) (`KismetMathLibrary.Conv_IntToDouble` (* _index_3 (`self.ZGap`))))) false)))))
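; First-person player character for Vision Protocol that routes Enhanced Input to gameplay components and owns the pause toggle.
; Parkour (jump, dash, crouch, wall run, grappling hook), interaction, weapons and dialog each delegate to their own component.
; The CDMGHP component holds health, initialized in the construction script and exposed through wrapper functions.
; Death only prints a message, the looping step-noise timer event is empty, and katana spawn test code is disconnected.
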(event Custom|Event%20On%20Death
  ;[1 1 1] Nie ma jeszcze ustalone, jak wygląda smierc
  (Development|PrintString "DEAD" true true "(R=0.000000,G=0.660000,B=1.000000,A=1.000000)" 1e+01))

(event Custom|Steps%20Noise
  ;[1 1 1] Backendowy hałas z kroków do AI oraz chwilowe wyswietlanie HP
)

(event Input|EnhancedActionEvents|EnhancedInputActionIA_Jump
  (params (ActionValue :type Boolean) (ElapsedSeconds :type Float%20%28double-precision%29) (TriggeredSeconds :type Float%20%28double-precision%29) (InputAction :type Input%20Action%20Object%20Reference :default "/Game/FirstPerson/Input/Actions/IA_Jump.IA_Jump"))
  ;[1 1 1] actions and events connected to parkour
  (:Triggered
    (Default|ParkourJump (Variables|Default|GetBP_CharacterParkourComponent)))
  (:Completed
    (Character|StopJumping)))

(event Input|EnhancedActionEvents|EnhancedInputActionIA_Dash
  (params (ActionValue :type Boolean) (ElapsedSeconds :type Float%20%28double-precision%29) (TriggeredSeconds :type Float%20%28double-precision%29) (InputAction :type Input%20Action%20Object%20Reference :default "/Game/_VisionProtocol/Core/Input/Actions/IA_Dash.IA_Dash"))
  ;[1 1 1] actions and events connected to parkour
  (:Started
    (Default|ParkourDash (Variables|Default|GetBP_CharacterParkourComponent))))

(event Input|EnhancedActionEvents|EnhancedInputActionIA_Dialog2
  (params (ActionValue :type Boolean) (ElapsedSeconds :type Float%20%28double-precision%29) (TriggeredSeconds :type Float%20%28double-precision%29) (InputAction :type Input%20Action%20Object%20Reference :default "/Game/_VisionProtocol/Core/Input/Actions/IA_Dialog2.IA_Dialog2"))
  (Default|NextDialog (Variables|Default|GetBPC_DialogSystem)))

(event Input|EnhancedActionEvents|EnhancedInputActionIA_Dialog3
  (params (ActionValue :type Boolean) (ElapsedSeconds :type Float%20%28double-precision%29) (TriggeredSeconds :type Float%20%28double-precision%29) (InputAction :type Input%20Action%20Object%20Reference :default "/Game/_VisionProtocol/Core/Input/Actions/IA_Dialog3.IA_Dialog3"))
  (Default|NextDialog (Variables|Default|GetBPC_DialogSystem)))

(event Input|EnhancedActionEvents|EnhancedInputActionIA_Pause
  (params (ActionValue :type Boolean) (ElapsedSeconds :type Float%20%28double-precision%29) (TriggeredSeconds :type Float%20%28double-precision%29) (InputAction :type Input%20Action%20Object%20Reference :default "/Game/_VisionProtocol/Core/Input/Actions/IA_Pause.IA_Pause"))
  (:Started
    (if (Game|IsGamePaused)
      (Utilities|IsValid (Variables|Default|GetPauseWidget)
        (:Is%20Valid
          (Default|ResumeGame (Variables|Default|GetPauseWidget))))
      (else
        (bind _returnvalue (UserInterface|CreateWidget "/Game/_VisionProtocol/Widgets/Menu/WBP_PauseMenu.WBP_PauseMenu_C"))
        (bind _output_get (Variables|Default|SetPauseWidget _returnvalue))
        (UserInterface|Viewport|AddtoViewport _output_get 0)
        (Game|SetGamePaused true)
        (Variables|/Script/Engine.PlayerController|SetbShowMouseCursor (Game|GetPlayerController 0) true)))))

(event Input|EnhancedActionEvents|EnhancedInputActionIA_Crouch
  (params (ActionValue :type Boolean) (ElapsedSeconds :type Float%20%28double-precision%29) (TriggeredSeconds :type Float%20%28double-precision%29) (InputAction :type Input%20Action%20Object%20Reference :default "/Game/_VisionProtocol/Core/Input/Actions/IA_Crouch.IA_Crouch"))
  ;[1 1 1] actions and events connected to parkour
  (:Started
    (Default|ParkourCrouch (Variables|Default|GetBP_CharacterParkourComponent))))

(event Input|EnhancedActionEvents|EnhancedInputActionIA_HorizontalWallRun
  (params (ActionValue :type Boolean) (ElapsedSeconds :type Float%20%28double-precision%29) (TriggeredSeconds :type Float%20%28double-precision%29) (InputAction :type Input%20Action%20Object%20Reference :default "/Game/_VisionProtocol/Core/Input/Actions/IA_HorizontalWallRun.IA_HorizontalWallRun"))
  ;[1 1 1] actions and events connected to parkour
  (:Triggered
    (Default|ParkourHorizontalWallRun (Variables|Default|GetBP_CharacterParkourComponent)))
  (:Canceled
    (Default|AttemptAbortHorizontalWallRun (Variables|Default|GetBP_CharacterParkourComponent) :!label _label))
  (:Completed
    (goto _label)))

(event Input|EnhancedActionEvents|EnhancedInputActionIA_GrapplingHook
  (params (ActionValue :type Boolean) (ElapsedSeconds :type Float%20%28double-precision%29) (TriggeredSeconds :type Float%20%28double-precision%29) (InputAction :type Input%20Action%20Object%20Reference :default "/Game/_VisionProtocol/Core/Input/Actions/IA_GrapplingHook.IA_GrapplingHook"))
  ;[1 1 1] actions and events connected to parkour
  (:Triggered
    (Default|AttemptGrapplingHookShot (Variables|Default|GetBP_CharacterParkourComponent)))
  (:Canceled
    (Default|AttemptAbortGrappling (Variables|Default|GetBP_CharacterParkourComponent) :!label _label))
  (:Completed
    (goto _label)))

(event Input|EnhancedActionEvents|EnhancedInputActionIA_Interact
  (params (ActionValue :type Boolean) (ElapsedSeconds :type Float%20%28double-precision%29) (TriggeredSeconds :type Float%20%28double-precision%29) (InputAction :type Input%20Action%20Object%20Reference :default "/Game/_VisionProtocol/Core/InteractionFramework/Input/Actions/IA_Interact.IA_Interact"))
  (Default|AttemptInteract (Variables|Default|GetBP_PlayerInteractionComponent)))

(event Input|EnhancedActionEvents|EnhancedInputActionIA_WeaponPrimaryFire
  (params (ActionValue :type Boolean) (ElapsedSeconds :type Float%20%28double-precision%29) (TriggeredSeconds :type Float%20%28double-precision%29) (InputAction :type Input%20Action%20Object%20Reference :default "/Game/_VisionProtocol/Core/Input/Actions/IA_WeaponPrimaryFire.IA_WeaponPrimaryFire"))
  (Default|TriggerPrimaryFire (Variables|Default|GetBPC_Weapons) (Transformation|GetWorldTransform (Variables|Default|GetFirstPersonCamera))))

(event Input|EnhancedActionEvents|EnhancedInputActionIA_WeaponUp
  (params (ActionValue :type Boolean) (ElapsedSeconds :type Float%20%28double-precision%29) (TriggeredSeconds :type Float%20%28double-precision%29) (InputAction :type Input%20Action%20Object%20Reference :default "/Game/_VisionProtocol/Core/Input/Actions/IA_WeaponUp.IA_WeaponUp"))
  (Default|ChangeWeapon (Variables|Default|GetBPC_Weapons) true))

(event Input|EnhancedActionEvents|EnhancedInputActionIA_WeaponDown
  (params (ActionValue :type Boolean) (ElapsedSeconds :type Float%20%28double-precision%29) (TriggeredSeconds :type Float%20%28double-precision%29) (InputAction :type Input%20Action%20Object%20Reference :default "/Game/_VisionProtocol/Core/Input/Actions/IA_WeaponDown.IA_WeaponDown"))
  (Default|ChangeWeapon (Variables|Default|GetBPC_Weapons) false))

(event Input|EnhancedActionEvents|EnhancedInputActionIA_Dialog1
  (params (ActionValue :type Boolean) (ElapsedSeconds :type Float%20%28double-precision%29) (TriggeredSeconds :type Float%20%28double-precision%29) (InputAction :type Input%20Action%20Object%20Reference :default "/Game/_VisionProtocol/Core/Input/Actions/IA_Dialog1.IA_Dialog1"))
  (Default|NextDialog (Variables|Default|GetBPC_DialogSystem)))

(event EventOnLanded
  (params (Hit :type Hit%20Result%20Structure%20%28by%20ref%29))
  ;[1 1 1] actions and events connected to parkour
  (Default|ParkourLand (Variables|Default|GetBP_CharacterParkourComponent)))

(event EventBeginPlay
  ;[1 1 1] Backendowy hałas z kroków do AI oraz chwilowe wyswietlanie HP
  (Utilities|Time|SetTimerbyEvent (delegate Custom|Steps%20Noise) 0.5 true))

(event Input|KeyboardEvents|DebugKeyI
  (params (Key :type Key%20Structure :default "None") (ActionValue :type Input%20Action%20Value%20Structure))
  (:Pressed
    (Animation|Montage|PlayMontage (Variables|Default|GetFirstPersonMesh) "/Game/_VisionProtocol/Animations/KatanaStrike/AM_ArmsKatanaStrike.AM_ArmsKatanaStrike")))

(fn ConstructionScript
  (bind _c_dmg_hp (Variables|Default|GetC_DMG-HP))
  (|CallParentFunction)
  (EventDispatchers|BindEventtoOnDeath _c_dmg_hp (EventDispatchers|CreateEvent :!event Custom|Event%20On%20Death))
  (bind _output_get (Variables|/Game/_VisionProtocol/Core/DMG-HP/C_DMG-HP.C_DMG-HP_C|SetMaximumHealth _c_dmg_hp 1e+02))
  (Variables|/Game/_VisionProtocol/Core/DMG-HP/C_DMG-HP.C_DMG-HP_C|SetCurrentHealth _c_dmg_hp _output_get))

(fn GetCurrentHealth
  (return (Variables|/Game/_VisionProtocol/Core/DMG-HP/C_DMG-HP.C_DMG-HP_C|GetCurrentHealth (Variables|Default|GetC_DMG-HP))))

(fn GetMaxHealth
  (return (Variables|/Game/_VisionProtocol/Core/DMG-HP/C_DMG-HP.C_DMG-HP_C|GetMaximumHealth (Variables|Default|GetC_DMG-HP))))

(fn Heal
  (params (HP_Amount :type Float%20%28double-precision%29))
  (bind _new_health (Default|Heal (Variables|Default|GetC_DMG-HP) HP_Amount))
  (return _new_health))

(fn IsDead
  (return (Variables|/Game/_VisionProtocol/Core/DMG-HP/C_DMG-HP.C_DMG-HP_C|GetisDead (Variables|Default|GetC_DMG-HP))))

(fn TakeDamage
  (params (Amount :type Float%20%28double-precision%29))
  (bind _was_damaged (Default|TakeDamage (Variables|Default|GetC_DMG-HP) Amount))
  (return _was_damaged))
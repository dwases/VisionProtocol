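; Quantovisor bullet that draws a Niagara beam back to the player and triggers quantum interactions with objects it touches.
; A looping timer updates the beam endpoints and line traces from bullet to player on the Projectile profile, so the beam itself detects hits.
; A trace or box hit calls Interact on QFMoveable SC_Quantum components, passing its SCQuantum reference.
; Any hit destroys the bullet, which otherwise expires after a short lifetime.
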(event `BeamUpdate`
  (bind _niagara (`self.Niagara`))
  (bind _returnvalue (`self.K2_GetActorLocation` (`GameplayStatics.GetPlayerCharacter` 0)))
  (`NiagaraComponent.SetVariablePosition` _niagara "BeamEnd" (`self.K2_GetActorLocation`))
  (`NiagaraComponent.SetVariablePosition` _niagara "BeamStart" _returnvalue)
  (bind (_outhit _returnvalue_2) (`KismetSystemLibrary.LineTraceSingleByProfile` (`self.K2_GetActorLocation`) _returnvalue "Projectile"))
  (if _returnvalue_2
    (bind _returnvalue_3 (`self.GetComponentByClass` (`.HitActor` (`GameplayStatics.BreakHitResult` _outhit)) "/Game/_VisionProtocol/Core/Visors/Quantovisor/SC_Quantum.SC_Quantum_C"))
    (`/Engine/EditorBlueprintResources/StandardMacros.IsValid` _returnvalue_3
      (:`Is Valid`
        (if (`/Game/_VisionProtocol/Core/Visors/Quantovisor/SC_Quantum.QF_Moveable` _returnvalue_3)
          (`/Game/_VisionProtocol/Core/Visors/Quantovisor/SC_Quantum.Interact` _returnvalue_3 (`self.SC_Quantum`))
          (`self.K2_DestroyActor`)
          (else
            (`self.K2_DestroyActor` :!label _label))))
      (:`Is Not Valid`
        (goto _label)))))

(event `self.ReceiveBeginPlay`
  (`KismetSystemLibrary.K2_SetTimerDelegate` (delegate `BeamUpdate`) 0.01 true)
  (`KismetSystemLibrary.Delay` 1.5)
  (`self.K2_DestroyActor`))

(event `self.Box.OnComponentHit`
  (params (HitComponent :type "PrimitiveComponent Object Reference") (OtherActor :type "Actor Object Reference") (OtherComp :type "PrimitiveComponent Object Reference") (NormalImpulse :type "Vector Structure") (Hit :type "HitResult Structure (by ref)"))
  (bind _returnvalue (`self.GetComponentByClass` OtherActor "/Game/_VisionProtocol/Core/Visors/Quantovisor/SC_Quantum.SC_Quantum_C"))
  (`/Engine/EditorBlueprintResources/StandardMacros.IsValid` _returnvalue
    (:`Is Valid`
      (if (`/Game/_VisionProtocol/Core/Visors/Quantovisor/SC_Quantum.QF_Moveable` _returnvalue)
        (`/Game/_VisionProtocol/Core/Visors/Quantovisor/SC_Quantum.Interact` _returnvalue (`self.SC_Quantum`))
        (`self.K2_DestroyActor`)
        (else
          (`self.K2_DestroyActor` :!label _label_2))))
    (:`Is Not Valid`
      (goto _label_2))))

(fn `UserConstructionScript`
  (bind _returnvalue (`self.K2_GetActorLocation`))
  (bind _niagara (`self.Niagara`))
  (`NiagaraComponent.SetVariablePosition` _niagara "BeamEnd" _returnvalue)
  (`NiagaraComponent.SetVariablePosition` _niagara "BeamStart" _returnvalue))
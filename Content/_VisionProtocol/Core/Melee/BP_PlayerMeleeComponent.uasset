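; Player melee component that performs katana strikes for BP_VPPlayerCharacter.
; MeleeAttack picks Dragonblood or Rotten katana by gameplay tag, preferring Dragonblood, and briefly spawns it on the first-person hand socket.
; While IsMeleeAttack is set, Tick sphere-traces along the blade's up vector with debug drawing, damaging BPI_Damageable hits.
; SlashedActors blocks repeat hits and is never cleared here, so each target takes damage only once.
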(event `self.ReceiveTick`
  (params (DeltaSeconds :type "Float (single-precision)"))
  (bind _weaponactor (`self.WeaponActor`))
  (bind _slashedactors (`self.SlashedActors`))
  (bind _returnvalue (`Actor.K2_GetActorLocation` _weaponactor))
  (if (`/Game/_VisionProtocol/Core/BP_VPPlayerCharacter.IsMeleeAttack` (`self.OwnerRef`))
    (bind _outhits (`KismetSystemLibrary.SphereTraceMulti` _returnvalue (+ _returnvalue (* (`Actor.GetActorUpVector` _weaponactor) 600.0)) 70.0 "TraceTypeQuery1" false (`|MakeArray` (`self.OwnerRef`) (`self.WeaponActor`) :!type "Actor Object Reference") "ForDuration" true (struct :`R` 1.0 :`A` 1.0) (struct :`G` 1.0 :`A` 1.0) 15.0))
    (for _array_element _outhits
      (bind _asbpi_damageable (cast `/Game/_VisionProtocol/Core/DMG-HP/BPI_Damageable` (`.HitActor` (`GameplayStatics.BreakHitResult` _array_element))))
      (if (not (`KismetArrayLibrary.Array_Contains` (`self.SlashedActors`) _asbpi_damageable))
        (bind _returnvalue_2 (`KismetArrayLibrary.Array_AddUnique` _slashedactors _asbpi_damageable))
        (bind _was_damaged (`/Game/_VisionProtocol/Core/DMG-HP/BPI_Damageable.TakeDamage` (`|GetArrayItem` _slashedactors _returnvalue_2) 30.0))
        (`KismetSystemLibrary.PrintString` "damaged" _was_damaged)))))

(event `KatanaStrike`
  (params (WeaponClass :type "Actor Class Reference"))
  (bind _returnvalue (`|SpawnActorFromClass` WeaponClass (`KismetMathLibrary.MakeTransform` (0.0 0.0 0.0)) "Undefined" "MultiplyWithRoot" (`self.OwnerRef`) null))
  (set `self.WeaponActor` _returnvalue)
  (bind _returnvalue_2 (`Actor.K2_AttachToComponent` _returnvalue (`/Game/FirstPerson/Blueprints/BP_FirstPersonCharacter.FirstPersonMesh` (`self.OwnerRef`)) "hand_r_Weapon_socket" "KeepRelative" "KeepRelative" "KeepRelative" true))
  (`KismetSystemLibrary.PrintString` (`KismetStringLibrary.Conv_BoolToString` _returnvalue_2))
  (`KismetSystemLibrary.Delay` 0.5)
  (set `/Game/_VisionProtocol/Core/BP_VPPlayerCharacter.IsMeleeAttack` false (`self.OwnerRef`))
  (`Actor.K2_DestroyActor` _returnvalue))

(event `self.ReceiveBeginPlay`
  (bind _asbp_vpplayer_character (cast `/Game/_VisionProtocol/Core/BP_VPPlayerCharacter` (`self.GetOwner`)))
  (set `self.OwnerRef` _asbp_vpplayer_character))

(event `MeleeAttack`
  (set `/Game/_VisionProtocol/Core/BP_VPPlayerCharacter.IsMeleeAttack` true (`self.OwnerRef`))
  (if (`BlueprintGameplayTagLibrary.HasTag` (`self.MeleeWeaponTags`) (struct :`TagName` "Player.AvailableWeapon.Melee.DragonbloodKatana") true)
    (`self.KatanaStrike` "/Game/_VisionProtocol/Core/Melee/Weapons/BP_DragonbloodKatana.BP_DragonbloodKatana_C")
    (set `self.CurrentWeaponClass` "/Game/_VisionProtocol/Core/Melee/Weapons/BP_DragonbloodKatana.BP_DragonbloodKatana_C")
    (elif (`BlueprintGameplayTagLibrary.HasTag` (`self.MeleeWeaponTags`) (struct :`TagName` "Player.AvailableWeapon.Melee.RottenKatana") true)
      (`self.KatanaStrike` "/Game/_VisionProtocol/Core/Melee/Weapons/BP_RottenKatana.BP_RottenKatana_C")
      (set `self.CurrentWeaponClass` "/Game/_VisionProtocol/Core/Melee/Weapons/BP_RottenKatana.BP_RottenKatana_C"))))
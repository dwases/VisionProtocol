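; Player save/load component that captures and restores the player character's state for continuing a game.
; GetPlayerSave gathers transform, control rotation, map name and references to the parkour, damage/health and weapons components.
; On continue game, UsePlayerSave applies the save from the game instance's data message, skipping default transforms and reassigning component references rather than copying values.
; Weapons and map name are captured but not restored here.
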(event `OnContinueGame`
  ;[1 1 1] Nalezy zaimplementowac continue game w main menu
  (bind _savegamedata (message `/Game/_VisionProtocol/Core/SaveLoadSystem/BPI_SaveGame.GetGameData` (`GameplayStatics.GetGameInstance`)))
  (`/Engine/EditorBlueprintResources/StandardMacros.IsValid` _savegamedata
    (:`Is Valid`
      (`self.UsePlayerSave` (`/Game/_VisionProtocol/Core/SaveLoadSystem/BP_SaveGame.PlayerSave` _savegamedata)))))

(fn `GetPlayerSave`
  (returns (PlayerSave :type "/Game/_VisionProtocol/Core/SaveLoadSystem/SPlayerSave Structure"))
  (bind _asbp_vpplayer_character (cast `/Game/_VisionProtocol/Core/BP_VPPlayerCharacter` (`GameplayStatics.GetPlayerPawn` 0)))
  (bind _returnvalue (`GameplayStatics.GetCurrentLevelName` true))
  (return (make `/Game/_VisionProtocol/Core/SaveLoadSystem/SPlayerSave` (`Actor.GetTransform` _asbp_vpplayer_character) (`Actor.GetComponentByClass` _asbp_vpplayer_character "/Game/_VisionProtocol/Core/Parkour/BP_CharacterParkourComponent.BP_CharacterParkourComponent_C") (`Actor.GetComponentByClass` _asbp_vpplayer_character "/Game/_VisionProtocol/Core/DMG-HP/C_DMG-HP.C_DMG-HP_C") (`Pawn.GetControlRotation` _asbp_vpplayer_character) (`Actor.GetComponentByClass` _asbp_vpplayer_character "/Game/_VisionProtocol/Core/Weapons/BPC_Weapons.BPC_Weapons_C") (`KismetStringLibrary.Conv_StringToName` _returnvalue))))

(fn `UsePlayerSave`
  (params (PlayerSave :type "/Game/_VisionProtocol/Core/SaveLoadSystem/SPlayerSave Structure"))
  (`|ExecutionSequence`
    (:`then_0`
      (if (not (== PlayerSave_Transform_2_92D92C984574B20C235302B2EE1DC01F (`KismetMathLibrary.MakeTransform` (0.0 0.0 0.0))))
        (`Actor.K2_SetActorTransform` (`GameplayStatics.GetPlayerPawn` 0) PlayerSave_Transform_2_92D92C984574B20C235302B2EE1DC01F false false)))
    (:`then_1`
      (bind _asbp_vpplayer_character (cast `/Game/_VisionProtocol/Core/BP_VPPlayerCharacter` (`GameplayStatics.GetPlayerPawn` 0)))
      (set `/Game/_VisionProtocol/Core/BP_VPPlayerCharacter.BP_CharacterParkourComponent` PlayerSave_Parkour_5_9E8599814A5AECF330AA4EB6F3E4241D _asbp_vpplayer_character))
    (:`then_2`
      (bind _asbp_vpplayer_character_2 (cast `/Game/_VisionProtocol/Core/BP_VPPlayerCharacter` (`GameplayStatics.GetPlayerPawn` 0)))
      (set `/Game/_VisionProtocol/Core/BP_VPPlayerCharacter.C_DMG-HP` PlayerSave_DMG_HP_8_F5B109C14EEB489ECF1F48A5EDB486DD _asbp_vpplayer_character_2))
    (:`then_3`
      (`Controller.SetControlRotation` (`Pawn.GetController` (`GameplayStatics.GetPlayerPawn` 0)) PlayerSave_ControlRotation_11_3C107CF940BA5E57FBCC9383F1C63859))))
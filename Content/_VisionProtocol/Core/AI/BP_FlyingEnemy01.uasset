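; BP_FlyingEnemy01 is a flying AI enemy character that starts play with 50 health.
; A CDMGHP component holds health, and the damage, heal, death and health query functions forward to it.
; Other functions expose the patrol route and ideal attack and defense ranges, and map named speed tiers to the CharacterMovement max walk speed.
; It holds no flight or attack logic of its own.
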(event `self.ReceiveBeginPlay`
  (bind _c_dmg_hp (`self.C_DMG-HP`))
  (`parent.ReceiveBeginPlay`)
  (bind _output_get (set `/Game/_VisionProtocol/Core/DMG-HP/C_DMG-HP.MaximumHealth` 50.0 _c_dmg_hp))
  (set `/Game/_VisionProtocol/Core/DMG-HP/C_DMG-HP.CurrentHealth` _output_get _c_dmg_hp))

(fn `GetCurrentHealth`
  (returns (Health :type "Float (double-precision)"))
  (return (`/Game/_VisionProtocol/Core/DMG-HP/C_DMG-HP.CurrentHealth` (`self.C_DMG-HP`))))

(fn `GetIdealRange`
  (returns (AttackRadius :type "Float (double-precision)") (DefenseRadius :type "Float (double-precision)"))
  (return 100.0 500.0))

(fn `GetMaxHealth`
  (returns (MaxHealth :type "Float (double-precision)"))
  (return (`/Game/_VisionProtocol/Core/DMG-HP/C_DMG-HP.MaximumHealth` (`self.C_DMG-HP`))))

(fn `GetPatrolRoute`
  (returns (PatrolRoute :type "/Game/_VisionProtocol/Core/AI/BP_PatrolPath1 Object Reference"))
  (return (`self.Patrol Route`)))

(fn `Heal`
  (params (HP_Amount :type "Float (double-precision)"))
  (returns (`New Health` :type "Float (double-precision)"))
  (bind _new_health (`/Game/_VisionProtocol/Core/DMG-HP/C_DMG-HP.Heal` (`self.C_DMG-HP`) HP_Amount))
  (return _new_health))

(fn `IsDead`
  (returns (Dead :type Boolean))
  (return (`/Game/_VisionProtocol/Core/DMG-HP/C_DMG-HP.isDead` (`self.C_DMG-HP`))))

(fn `SetMovementSpeed`
  (params (Speed :type "/Game/_VisionProtocol/Core/AI/Enums/E_MovementSpeed Enum" :default "NewEnumerator0"))
  (returns (SpeedValue :type "Float (double-precision)"))
  (bind _output_get (set `CharacterMovementComponent.MaxWalkSpeed` (select `/Game/_VisionProtocol/Core/AI/Enums/E_MovementSpeed` Speed :`NewEnumerator1` 50.0 :`NewEnumerator2` 125.0 :`NewEnumerator3` 350.0 :`NewEnumerator4` 500.0 :`NewEnumerator5` 700.0 :!type "Float (single-precision)") (`self.CharacterMovement`)))
  (return _output_get))

(fn `TakeDamage`
  (params (Amount :type "Float (double-precision)"))
  (returns (`Was Damaged` :type Boolean))
  (bind _was_damaged (message `/Game/_VisionProtocol/Core/DMG-HP/BPI_Damageable.TakeDamage` (`self.C_DMG-HP`) Amount))
  (return _was_damaged))

(fn `UserConstructionScript`
  (`parent.UserConstructionScript`))
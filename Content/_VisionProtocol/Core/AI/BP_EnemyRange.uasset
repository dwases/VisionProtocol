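; BP_EnemyRange is a ranged enemy whose Attack1 event fires a BP_DefaultProjectile from its BulletSpawn point, with itself as owner.
; It sets its starting health on BeginPlay and delegates damage, healing and death queries to the CDMGHP component.
; It also exposes its patrol route and attack and defense radii.
; SetMovementSpeed only maps a speed tier to a value and returns it, without applying it.
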(event `self.ReceiveBeginPlay`
  (bind _c_dmg_hp (`self.C_DMG-HP`))
  (`parent.ReceiveBeginPlay`)
  (bind _output_get (set `/Game/_VisionProtocol/Core/DMG-HP/C_DMG-HP.MaximumHealth` 150.0 _c_dmg_hp))
  (set `/Game/_VisionProtocol/Core/DMG-HP/C_DMG-HP.CurrentHealth` _output_get _c_dmg_hp))

(event `/Game/_VisionProtocol/Core/AI/BPI_Enemy.Attack1`
  (bind (_returnvalue_location _returnvalue_rotation) (`KismetMathLibrary.BreakTransform` (`SceneComponent.K2_GetComponentToWorld` (`self.BulletSpawn`))))
  (`|SpawnActorFromClass` "/Game/_VisionProtocol/Core/Weapons/Projectiles/BP_DefaultProjectile.BP_DefaultProjectile_C" (`KismetMathLibrary.MakeTransform` _returnvalue_location _returnvalue_rotation) "AdjustIfPossibleButDontSpawnIfColliding" "MultiplyWithRoot" self 1000.0 null))

(fn `GetCurrentHealth`
  (returns (Health :type "Float (double-precision)"))
  (return (`/Game/_VisionProtocol/Core/DMG-HP/C_DMG-HP.CurrentHealth` (`self.C_DMG-HP`))))

(fn `GetIdealRange`
  (returns (AttackRadius :type "Float (double-precision)") (DefenseRadius :type "Float (double-precision)"))
  (return 400.0 1000.0))

(fn `GetMaxHealth`
  (returns (MaxHealth :type "Float (double-precision)"))
  (return (`/Game/_VisionProtocol/Core/DMG-HP/C_DMG-HP.MaximumHealth` (`self.C_DMG-HP`))))

(fn `GetPatrolRoute`
  (returns (PatrolRoute :type "/Game/_VisionProtocol/Core/AI/BP_PatrolPath1 Object Reference"))
  (return (`self.Patrol Route`)))

(fn `Heal`
  (params (HP_Amount :type "Float (double-precision)"))
  (returns (`New Health` :type "Float (double-precision)"))
  (bind _new_health (`/Game/_VisionProtocol/Core/DMG-HP/C_DMG-HP.Heal` (`self.C_DMG-HP`) HP_Amount))
  (return _new_health))

(fn `IsDead`
  (returns (Dead :type Boolean))
  (return (`/Game/_VisionProtocol/Core/DMG-HP/C_DMG-HP.isDead` (`self.C_DMG-HP`))))

(fn `SetMovementSpeed`
  (params (Speed :type "/Game/_VisionProtocol/Core/AI/Enums/E_MovementSpeed Enum" :default "NewEnumerator0"))
  (returns (SpeedValue :type "Float (double-precision)"))
  (return (select `/Game/_VisionProtocol/Core/AI/Enums/E_MovementSpeed` Speed :`NewEnumerator1` 50.0 :`NewEnumerator2` 110.0 :`NewEnumerator3` 300.0 :`NewEnumerator4` 450.0 :`NewEnumerator5` 600.0)))

(fn `TakeDamage`
  (params (Amount :type "Float (double-precision)"))
  (returns (`Was Damaged` :type Boolean))
  (bind _was_damaged (`/Game/_VisionProtocol/Core/DMG-HP/C_DMG-HP.TakeDamage` (`self.C_DMG-HP`) Amount))
  (return _was_damaged))

(fn `UserConstructionScript`
  (`parent.UserConstructionScript`))
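; Weapon component that handles primary fire and weapon switching, driven by a WeaponsData array indexed by WeaponID.
; TriggerPrimaryFire spawns the current weapon's projectile just ahead of the supplied spawn transform when FireDelay is zero, then resets the delay from that weapon's fire rate.
; Tick counts FireDelay down to zero.
; ChangeWeapon cycles through three weapon slots with wraparound, prints the new ID and restarts the fire delay.
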(event `self.ReceiveTick`
  (params (DeltaSeconds :type "Float (single-precision)"))
  (set `self.FireDelay` (`KismetMathLibrary.FClamp` (- (`self.FireDelay`) DeltaSeconds) 0.0 999.0)))

(fn `ChangeWeapon`
  (params (ScrollUp :type Boolean))
  (bind _weaponid (`self.WeaponID`))
  (bind _weaponid_2 (`self.WeaponID`))
  (bind _weaponid_3 (`self.WeaponID`))
  (if ScrollUp
    (set `self.WeaponID` (select `bool` (== _weaponid_2 0) :`false` (- _weaponid_2 1) :`true` 2))
    (else
      (set `self.WeaponID` (select `bool` (== _weaponid 2) :`false` (+ _weaponid 1)))))
  (`KismetSystemLibrary.PrintString` (`KismetStringLibrary.Conv_IntToString` _weaponid_3))
  (set `self.FireDelay` (/ 1.0 (`.Firerate_7_E089AE31413FBF7105D9DE812A3438C7` (break `/Game/_VisionProtocol/Core/Weapons/ST_WeaponData` (`|GetArrayItem` (`self.WeaponsData`) _weaponid_3))))))

(fn `TriggerPrimaryFire`
  (params (ProjectileSpawnPoint :type "Transform Structure"))
  (bind (_name _firerate _projectile) (break `/Game/_VisionProtocol/Core/Weapons/ST_WeaponData` (`|GetArrayItem` (`self.WeaponsData`) (`self.WeaponID`))))
  (if (== (`self.FireDelay`) 0.0)
    (`|SpawnActorFromClass` _projectile (`KismetMathLibrary.MakeTransform` (+ (* (`KismetMathLibrary.GetForwardVector` ProjectileSpawnPoint_Rotation) 150.0) ProjectileSpawnPoint_Location) ProjectileSpawnPoint_Rotation ProjectileSpawnPoint_Scale) "Undefined" "MultiplyWithRoot" null null)
    (set `self.FireDelay` (/ 1.0 _firerate))))
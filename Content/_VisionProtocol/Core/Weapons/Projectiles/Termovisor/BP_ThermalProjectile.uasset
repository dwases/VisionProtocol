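; Thermal projectile actor for the Termovisor weapon that carries an attached fire particle effect.
; When its Box component hits something, it sends damage and heat-up messages to the other actor, spawns a BP_FireSurface at its own transform, then destroys itself.
; If nothing is hit, it destroys itself after a fixed delay.
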(event `self.ReceiveBeginPlay`
  (`GameplayStatics.SpawnEmitterAttached` "/Game/StarterContent/Particles/P_Fire.P_Fire" (`self.Sphere`))
  (`KismetSystemLibrary.Delay` 6.0)
  (`self.K2_DestroyActor`))

(event `self.Box.OnComponentHit`
  (params (HitComponent :type "PrimitiveComponent Object Reference") (OtherActor :type "Actor Object Reference") (OtherComp :type "PrimitiveComponent Object Reference") (NormalImpulse :type "Vector Structure") (Hit :type "HitResult Structure (by ref)"))
  (message `/Game/_VisionProtocol/Core/DMG-HP/BPI_Damageable.TakeDamage` OtherActor 30.0)
  (message `/Game/_VisionProtocol/Core/Visors/Termovisor/BPI_Heatable.HeatUp` OtherActor)
  (`|SpawnActorFromClass` "/Game/_VisionProtocol/Core/Weapons/Projectiles/Termovisor/BP_FireSurface.BP_FireSurface_C" (`self.GetTransform` self) "Undefined" "MultiplyWithRoot" null null)
  (`self.K2_DestroyActor`))

(fn `UserConstructionScript`)
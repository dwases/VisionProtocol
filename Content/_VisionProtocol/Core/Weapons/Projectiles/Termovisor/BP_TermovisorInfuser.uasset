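; Thermal visor infuser projectile that damages what it hits and charges the player's Termovisor with cold or warmth from that target.
; On box hit it reads the custom depth stencil of the target's static mesh, or skeletal mesh if none, as a cold or warm tag.
; The matching infuse call goes to the player character's CVisors component.
; It destroys itself after any hit or a short lifetime.
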(event `self.ReceiveBeginPlay`
  (`KismetSystemLibrary.Delay` 10.0)
  (`self.K2_DestroyActor`))

(event `self.Box.OnComponentHit`
  (params (HitComponent :type "PrimitiveComponent Object Reference") (OtherActor :type "Actor Object Reference") (OtherComp :type "PrimitiveComponent Object Reference") (NormalImpulse :type "Vector Structure") (Hit :type "HitResult Structure (by ref)"))
  (bind _returnvalue (`self.GetComponentByClass` OtherActor "/Script/Engine.SkeletalMeshComponent"))
  (bind _returnvalue_2 (`self.GetComponentByClass` OtherActor "/Script/Engine.StaticMeshComponent"))
  (bind _customdepthstencilvalue (`PrimitiveComponent.CustomDepthStencilValue` _returnvalue_2))
  (bind _customdepthstencilvalue_2 (`PrimitiveComponent.CustomDepthStencilValue` _returnvalue))
  (message `/Game/_VisionProtocol/Core/DMG-HP/BPI_Damageable.TakeDamage` OtherActor 10.0)
  (bind _asbp_vpplayer_character (cast `/Game/_VisionProtocol/Core/BP_VPPlayerCharacter` (`GameplayStatics.GetPlayerPawn` 0))
    (:`then`
      (`/Engine/EditorBlueprintResources/StandardMacros.IsValid` _returnvalue_2
        (:`Is Valid`
          (if (== _customdepthstencilvalue 1)
            (bind _c_visors (`/Game/_VisionProtocol/Core/BP_VPPlayerCharacter.C_Visors` _asbp_vpplayer_character))
            (`/Game/_VisionProtocol/Core/Visors/C_Visors.InfuseTermovisorWithCold` _c_visors)
            (`self.K2_DestroyActor`)
            (else
              (if (== _customdepthstencilvalue 2)
                (`/Game/_VisionProtocol/Core/Visors/C_Visors.InfuseTermovisorWithWarm` _c_visors))
              (`self.K2_DestroyActor`))))
        (:`Is Not Valid`
          (`/Engine/EditorBlueprintResources/StandardMacros.IsValid` _returnvalue
            (:`Is Valid`
              (if (== _customdepthstencilvalue_2 1)
                (`/Game/_VisionProtocol/Core/Visors/C_Visors.InfuseTermovisorWithCold` _c_visors)
                (`self.K2_DestroyActor`)
                (else
                  (if (== _customdepthstencilvalue_2 2)
                    (`/Game/_VisionProtocol/Core/Visors/C_Visors.InfuseTermovisorWithWarm` _c_visors))
                  (`self.K2_DestroyActor`))))
            (:`Is Not Valid`
              (`self.K2_DestroyActor`))))))
    (:`CastFailed`
      (`self.K2_DestroyActor`))))

(fn `UserConstructionScript`)
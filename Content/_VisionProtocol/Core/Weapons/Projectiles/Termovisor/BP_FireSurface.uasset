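; BP_FireSurface is an actor that leaves a temporary fire effect at its location, apparently for the Termovisor weapon's projectiles.
; On BeginPlay it spawns an enlarged fire particle emitter and stores its world scale.
; A timeline falloff curve rescales the emitter over time, then after a short delay the emitter and actor are destroyed.
; It is purely visual, with no damage or collision logic in its graphs.
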(event `self.ReceiveBeginPlay`
  (bind _returnvalue (`GameplayStatics.SpawnEmitterAtLocation` "/Game/StarterContent/Particles/P_Fire.P_Fire" (`self.K2_GetActorLocation` self) (struct) (4.0 4.0 4.0)))
  (bind _output_get (set `self.FireEmitter` _returnvalue))
  (set `self.FormerWorldScale` (`SceneComponent.K2_GetComponentScale` _output_get))
  (bind (_direction _falloff) (`Timeline|TL_FireDecay` :!via `PlayFromStart`)
    (:`Update`
      (`SceneComponent.SetWorldScale3D` (`self.FireEmitter`) (* (`self.FormerWorldScale`) _falloff)))
    (:`Finished`
      (`KismetSystemLibrary.Delay` 2.0)
      (`ActorComponent.K2_DestroyComponent` (`self.FireEmitter`))
      (`self.K2_DestroyActor`))))

(fn `UserConstructionScript`)
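; BP_FreezingProjectile is a Termovisor weapon projectile that cools down whatever it hits.
; It trails a FreezingWater effect attached to its sphere and destroys itself after a fixed lifetime if nothing is hit.
; On a box hit it sends the other actor a zero-damage message and a cool-down message, prints leftover debug text, spawns a scaled FreezingAura effect, then destroys itself.
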(event `self.ReceiveBeginPlay`
  (`NiagaraFunctionLibrary.SpawnSystemAttached` "/Game/_VisionProtocol/TechArt/VFX/Visors/Termovisor/FreezingWater.FreezingWater" (`self.Sphere`) "None" (0.0 0.0 0.0) (struct) "KeepRelativeOffset")
  (`KismetSystemLibrary.Delay` 6.0)
  (`self.K2_DestroyActor`))

(event `self.Box.OnComponentHit`
  (params (HitComponent :type "PrimitiveComponent Object Reference") (OtherActor :type "Actor Object Reference") (OtherComp :type "PrimitiveComponent Object Reference") (NormalImpulse :type "Vector Structure") (Hit :type "HitResult Structure (by ref)"))
  (message `/Game/_VisionProtocol/Core/DMG-HP/BPI_Damageable.TakeDamage` OtherActor 0.0)
  (message `/Game/_VisionProtocol/Core/Visors/Termovisor/BPI_Coolable.CoolDown` OtherActor)
  (`KismetSystemLibrary.PrintString` "eawfaewf")
  (`NiagaraFunctionLibrary.SpawnSystemAtLocation` "/Game/_VisionProtocol/TechArt/VFX/Visors/Termovisor/FreezingAura.FreezingAura" (`self.K2_GetActorLocation` self) (struct) (6.0 6.0 10.0))
  (`self.K2_DestroyActor`))

(fn `UserConstructionScript`
  (`parent.UserConstructionScript`))
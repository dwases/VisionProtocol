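; BP_WindSlice is a weapon projectile with slight gravity and configurable speed that destroys itself after its lifetime expires.
; Overlap and mesh hit events share a DoOnce, so only the first contact reaches DamageOtherActor.
; That function ignores the owner, reports an AI damage event at the owner's location, sends TakeDamageMessage to the target, and optionally destroys the projectile.
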(event `self.ReceiveBeginPlay`
  (`|ExecutionSequence`
    (:`then_0`
      (`KismetSystemLibrary.Delay` (`self.Lifetime`))
      (`self.K2_DestroyActor`))))

(event `self.ReceiveActorBeginOverlap`
  (params (OtherActor :type "Actor Object Reference"))
  (set `self.OtherActorRef` OtherActor)
  (`/Engine/EditorBlueprintResources/StandardMacros.DoOnce` false :!label _label
    (:`Completed`
      (`self.DamageOtherActor` (`self.OtherActorRef`)))))

(event `self.StaticMesh.OnComponentHit`
  (params (HitComponent :type "PrimitiveComponent Object Reference") (OtherActor :type "Actor Object Reference") (OtherComp :type "PrimitiveComponent Object Reference") (NormalImpulse :type "Vector Structure") (Hit :type "HitResult Structure (by ref)"))
  (set `self.OtherActorRef` OtherActor)
  (goto _label))

(fn `DamageOtherActor`
  (params (OtherActor :type "Actor Object Reference"))
  (bind _returnvalue (`self.GetOwner`))
  (bind _damage (`self.Damage`))
  (bind _returnvalue_2 (`self.K2_GetActorLocation` _returnvalue))
  (if (!= OtherActor _returnvalue)
    (`AISense_Damage.ReportDamageEvent` OtherActor _returnvalue _damage _returnvalue_2 _returnvalue_2)
    (message `/Game/_VisionProtocol/Core/DMG-HP/BPI_Damageable.TakeDamage` OtherActor _damage)
    (if (`self.DestroyOnHit`)
      (`self.K2_DestroyActor`))))

(fn `UserConstructionScript`
  (bind _projectilemovement (`self.ProjectileMovement`))
  (set `ProjectileMovementComponent.ProjectileGravityScale` 0.2 (`self.ProjectileMovement`))
  (bind _output_get (set `ProjectileMovementComponent.InitialSpeed` (`self.NewSpeed`) _projectilemovement))
  (set `ProjectileMovementComponent.MaxSpeed` _output_get _projectilemovement))
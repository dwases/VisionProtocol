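; Shotgun shell projectile that acts as a one-shot spawner, bursting into BP_ShotgunPellet actors on BeginPlay and then destroying itself.
; Each of the NumOfPellets pellets spawns at the shell's transform, with pitch and yaw offset by random deviations scaled by Spread.
; The random offsets are weighted by absolute value over 2D vector length, intended to remap the square distribution into a circular spread.
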(event `self.ReceiveBeginPlay`
  (bind _returnvalue (`self.GetTransform`))
  (bind _returnvalue_2 (`KismetMathLibrary.RandomFloatInRange` -1.0 1.0))
  (bind _returnvalue_3 (`KismetMathLibrary.RandomFloatInRange` -1.0 1.0))
  (bind _spread (`self.Spread`))
  (bind _returnvalue_4 (`KismetMathLibrary.VSize2D` (`KismetMathLibrary.MakeVector2D` _returnvalue_2 _returnvalue_3)))
  (for _ (range 1 (+ (`self.NumOfPellets`) 1))
    (`|SpawnActorFromClass` "/Game/_VisionProtocol/Core/Weapons/Projectiles/BP_ShotgunPellet.BP_ShotgunPellet_C" (`KismetMathLibrary.MakeTransform` (.location _returnvalue) (`KismetMathLibrary.MakeRotator` (.roll (.rotation _returnvalue)) (+ (.pitch (.rotation _returnvalue)) (* (/ (* _returnvalue_2 (`KismetMathLibrary.Abs` _returnvalue_2)) _returnvalue_4) _spread)) (+ (.yaw (.rotation _returnvalue)) (* (/ (* _returnvalue_3 (`KismetMathLibrary.Abs` _returnvalue_3)) _returnvalue_4) _spread))) (.scale _returnvalue)) "Undefined" "MultiplyWithRoot" null null))
  (`self.K2_DestroyActor`))

(fn `UserConstructionScript`)
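; BP_ProjectileBase is a weapon projectile that damages actors it overlaps, ignoring its owner.
; The construction script feeds speed and gravity scale into ProjectileMovement.
; On BeginPlay it sets all static meshes to the Projectile collision profile and destroys itself after its lifetime.
; Overlaps report a damage event, using the owner's location for both event and hit, send TakeDamageMessage and optionally destroy the projectile.
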(event `self.ReceiveBeginPlay`
  (for _array_element (`self.K2_GetComponentsByClass` "/Script/Engine.StaticMeshComponent")
    (`PrimitiveComponent.SetCollisionProfileName` _array_element "Projectile" true))
  (`KismetSystemLibrary.Delay` (`self.Lifetime`))
  (`self.K2_DestroyActor`))

(event `self.ReceiveActorBeginOverlap`
  (params (OtherActor :type "Actor Object Reference"))
  (bind _returnvalue (`self.GetOwner`))
  (bind _damage (`self.Damage`))
  (bind _returnvalue_2 (`self.K2_GetActorLocation` _returnvalue))
  (if (!= OtherActor _returnvalue)
    (`AISense_Damage.ReportDamageEvent` OtherActor _returnvalue _damage _returnvalue_2 _returnvalue_2)
    (message `/Game/_VisionProtocol/Core/DMG-HP/BPI_Damageable.TakeDamage` OtherActor _damage)
    (if (`self.DestroyOnHit`)
      (`self.K2_DestroyActor`))))

(fn `UserConstructionScript`
  (bind _projectilemovement (`self.ProjectileMovement`))
  (set `ProjectileMovementComponent.InitialSpeed` (`self.Speed`) _projectilemovement)
  (set `ProjectileMovementComponent.ProjectileGravityScale` (`self.GravityScale`) _projectilemovement))
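; BP_Rocket is a rocket projectile that explodes when its Box component hits something, and self-destructs silently after a fixed lifetime.
; A hit sends direct damage to the struck actor via TakeDamageMessage, then a sphere overlap applies rounded, linear-falloff splash damage, skipping zero results.
; The splash query ignores the rocket and player character 0.
; A RadialForce impulse, explosion sound and particle effect fire before the rocket is destroyed.
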(event `self.ReceiveBeginPlay`
  (`KismetSystemLibrary.Delay` 10.0)
  (`self.K2_DestroyActor`))

(event `self.Box.OnComponentHit`
  (params (HitComponent :type "PrimitiveComponent Object Reference") (OtherActor :type "Actor Object Reference") (OtherComp :type "PrimitiveComponent Object Reference") (NormalImpulse :type "Vector Structure") (Hit :type "HitResult Structure (by ref)"))
  (bind _returnvalue (`self.K2_GetActorLocation`))
  (bind _returnvalue_2 (`self.K2_GetActorLocation`))
  (bind _explosionradius (`self.ExplosionRadius`))
  (message `/Game/_VisionProtocol/Core/DMG-HP/BPI_Damageable.TakeDamage` OtherActor (`self.DirectDamage`))
  (bind _outactors (`KismetSystemLibrary.SphereOverlapActors` _returnvalue_2 (`self.ExplosionRadius`) (`|MakeArray` "ObjectTypeQuery1" "ObjectTypeQuery2" "ObjectTypeQuery3" "ObjectTypeQuery4" "ObjectTypeQuery6" "ObjectTypeQuery1" "ObjectTypeQuery5" "ObjectTypeQuery7" :!type "EObjectTypeQuery Enum") null (`|MakeArray` self (`GameplayStatics.GetPlayerCharacter` 0) :!type "Actor Object Reference")))
  (for _array_element _outactors
    (`/Engine/EditorBlueprintResources/StandardMacros.IsValid` _array_element
      (:`Is Valid`
        (bind _returnvalue_3 (`KismetMathLibrary.Conv_IntToDouble` (`KismetMathLibrary.Round` (* (`self.SplashDamage`) (`KismetMathLibrary.FClamp` (/ (- _explosionradius (`KismetMathLibrary.Vector_Distance` _returnvalue_2 (`self.K2_GetActorLocation` _array_element))) _explosionradius))))))
        (if (not (== _returnvalue_3 0.0))
          (message `/Game/_VisionProtocol/Core/DMG-HP/BPI_Damageable.TakeDamage` _array_element _returnvalue_3)))))
  (`RadialForceComponent.FireImpulse` (`self.RadialForce`))
  (`GameplayStatics.PlaySoundAtLocation` "/Game/StarterContent/Audio/Explosion_Cue.Explosion_Cue" _returnvalue (struct) 1.0 1.0 0.0 null null null null)
  (`GameplayStatics.SpawnEmitterAtLocation` "/Game/StarterContent/Particles/P_Explosion.P_Explosion" _returnvalue (struct) (3.0 3.0 3.0))
  (`self.K2_DestroyActor`))

(fn `UserConstructionScript`)
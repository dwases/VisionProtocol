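; BP_ShotgunPellet is a short-lived shotgun projectile that damages what it hits.
; Every tick it shrinks its Box component's world scale at a fixed per-axis rate, slightly faster along X.
; When the Box hits something, it sends a fixed-damage TakeDamageMessage to that actor and destroys itself.
; Otherwise, a BeginPlay delay destroys it after a fraction of a second, limiting its range.
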(event `self.ReceiveBeginPlay`
  (`KismetSystemLibrary.Delay` 0.5)
  (`self.K2_DestroyActor`))

(event `self.ReceiveTick`
  (params (DeltaSeconds :type "Float (single-precision)"))
  (bind _box (`self.Box`))
  (`SceneComponent.SetWorldScale3D` _box (- (`SceneComponent.K2_GetComponentScale` _box) (* (0.8 0.6 0.6) DeltaSeconds))))

(event `self.Box.OnComponentHit`
  (params (HitComponent :type "PrimitiveComponent Object Reference") (OtherActor :type "Actor Object Reference") (OtherComp :type "PrimitiveComponent Object Reference") (NormalImpulse :type "Vector Structure") (Hit :type "HitResult Structure (by ref)"))
  (message `/Game/_VisionProtocol/Core/DMG-HP/BPI_Damageable.TakeDamage` OtherActor 5.0)
  (`self.K2_DestroyActor`))

(fn `UserConstructionScript`)
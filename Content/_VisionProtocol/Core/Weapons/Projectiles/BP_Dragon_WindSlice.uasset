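; BP_Dragon_WindSlice is a projectile Blueprint, named as a dragon's wind slice attack.
; Its construction script sets the projectile movement's initial speed from the NewSpeed variable.
; On BeginPlay it sets the static mesh's world roll from the Rotation variable, keeping the mesh's current pitch and yaw.
; Overlap and tick events are disabled, so this graph adds no hit or per-frame logic.
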(event `self.ReceiveBeginPlay`
  (bind _staticmesh_0 (`self.StaticMesh_0`))
  (bind _rotation_roll (`KismetMathLibrary.BreakRotator` (`self.Rotation`)))
  (bind (_returnvalue_roll _returnvalue_pitch _returnvalue_yaw) (`KismetMathLibrary.BreakRotator` (`SceneComponent.K2_GetComponentRotation` _staticmesh_0)))
  (`parent.ReceiveBeginPlay`)
  (`SceneComponent.K2_SetWorldRotation` _staticmesh_0 (`KismetMathLibrary.MakeRotator` _rotation_roll _returnvalue_pitch _returnvalue_yaw) false false))

(fn `UserConstructionScript`
  (`parent.UserConstructionScript`)
  (set `ProjectileMovementComponent.InitialSpeed` (`self.NewSpeed`) (`self.ProjectileMovement`)))
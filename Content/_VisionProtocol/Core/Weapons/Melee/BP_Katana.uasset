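; BP_Katana is an interactable pickup that unlocks the katana melee weapon for the player.
; On Interact it queues two Polish HUD pop-ups announcing the weapon and its attack key, then adds the RottenKatana gameplay tag to the player melee component's MeleeWeaponTags and destroys itself.
; It supplies a "Pick up" interaction name and always shows the interact key widget.
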(event `/Game/_VisionProtocol/Core/InteractionFramework/BPI_Interactable.Interact`
  (params (Interactor :type "Actor Object Reference") (InteracteeComponent :type "PrimitiveComponent Object Reference"))
  (bind _asplayer_hud (cast `/Game/_VisionProtocol/Core/PlayerHUD` (`PlayerController.GetHUD` (`GameplayStatics.GetPlayerController` 0))))
  (bind _popupwidget (`/Game/_VisionProtocol/Core/PlayerHUD.PopUpWidget` _asplayer_hud))
  (`/Game/_VisionProtocol/Widgets/Dialogues/WBP_PopUp.AddPopUp` _popupwidget "Gratulacje, zdobyłeś nową broń – smocza katana. Jest skuteczna do walki z bliska.")
  (`/Game/_VisionProtocol/Widgets/Dialogues/WBP_PopUp.AddPopUp` _popupwidget "Naciśnij [V] aby zaatakować kataną.")
  (bind _asbp_vpplayer_character (cast `/Game/_VisionProtocol/Core/BP_VPPlayerCharacter` (`GameplayStatics.GetPlayerCharacter` 0)))
  (`BlueprintGameplayTagLibrary.AddGameplayTag` (`/Game/_VisionProtocol/Core/Melee/BP_PlayerMeleeComponent.MeleeWeaponTags` (`/Game/_VisionProtocol/Core/BP_VPPlayerCharacter.BP_PlayerMeleeComponent` _asbp_vpplayer_character)) (struct :`TagName` "Player.AvailableWeapon.Melee.RottenKatana"))
  (`self.K2_DestroyActor`))

(fn `GetInteractionName`
  (returns (InteractionName :type Text))
  (return "Pick up"))

(fn `GetIsInteractKeyWidgetVisible`
  (returns (IsInteractKeyWidgetVisible :type Boolean))
  (return true))

(fn `UserConstructionScript`)
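; Player controller that switches Enhanced Input mapping contexts to match the player's movement or dialog state.
; BeginPlay adds default, parkour, interaction and weapons contexts.
; Paired Initiate/Exit events for dashing, sliding, horizontal wall running, grappling hook and dialog swap default and parkour out for a state-specific context, then restore them.
; Only dialog also removes weapons and uses a higher priority; interaction is never removed.
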(event `self.ReceiveBeginPlay`
  (bind _returnvalue (subsystem `EnhancedInputLocalPlayerSubsystem`))
  (`parent.ReceiveBeginPlay`)
  (`/Engine/EditorBlueprintResources/StandardMacros.IsValid` _returnvalue
    (:`Is Valid`
      (`EnhancedInputSubsystemInterface.AddMappingContext` _returnvalue "/Game/FirstPerson/Input/IMC_Default.IMC_Default" 0 (struct))
      (`EnhancedInputSubsystemInterface.AddMappingContext` _returnvalue "/Game/_VisionProtocol/Core/Input/IMC_Parkour.IMC_Parkour" 0 (struct))
      (`EnhancedInputSubsystemInterface.AddMappingContext` _returnvalue "/Game/_VisionProtocol/Core/InteractionFramework/Input/InputMappingContexts/IMC_Interaction.IMC_Interaction" 0 (struct))
      (`EnhancedInputSubsystemInterface.AddMappingContext` _returnvalue "/Game/_VisionProtocol/Core/Input/IMC_Weapons.IMC_Weapons" 0 (struct)))))

(event `InitiateDashingContext`
  (bind _returnvalue (subsystem `EnhancedInputLocalPlayerSubsystem`))
  (`/Engine/EditorBlueprintResources/StandardMacros.IsValid` _returnvalue
    (:`Is Valid`
      (`EnhancedInputSubsystemInterface.RemoveMappingContext` _returnvalue "/Game/FirstPerson/Input/IMC_Default.IMC_Default" (struct))
      (`EnhancedInputSubsystemInterface.RemoveMappingContext` _returnvalue "/Game/_VisionProtocol/Core/Input/IMC_Parkour.IMC_Parkour" (struct))
      (`EnhancedInputSubsystemInterface.AddMappingContext` _returnvalue "/Game/_VisionProtocol/Core/Input/ActionSpecificInputMappingContexts/IMC_Dashing.IMC_Dashing" 0 (struct))
      (`EnhancedInputSubsystemInterface.RemoveMappingContext` _returnvalue "/Game/_VisionProtocol/Core/Input/ActionSpecificInputMappingContexts/IMC_Sliding.IMC_Sliding" (struct)))))

(event `ExitDashingContext`
  (bind _returnvalue (subsystem `EnhancedInputLocalPlayerSubsystem`))
  (`/Engine/EditorBlueprintResources/StandardMacros.IsValid` _returnvalue
    (:`Is Valid`
      (`EnhancedInputSubsystemInterface.AddMappingContext` _returnvalue "/Game/FirstPerson/Input/IMC_Default.IMC_Default" 0 (struct))
      (`EnhancedInputSubsystemInterface.AddMappingContext` _returnvalue "/Game/_VisionProtocol/Core/Input/IMC_Parkour.IMC_Parkour" 0 (struct))
      (`EnhancedInputSubsystemInterface.RemoveMappingContext` _returnvalue "/Game/_VisionProtocol/Core/Input/ActionSpecificInputMappingContexts/IMC_Dashing.IMC_Dashing" (struct)))))

(event `InitiateSlidingContext`
  (bind _returnvalue (subsystem `EnhancedInputLocalPlayerSubsystem`))
  (`/Engine/EditorBlueprintResources/StandardMacros.IsValid` _returnvalue
    (:`Is Valid`
      (`EnhancedInputSubsystemInterface.RemoveMappingContext` _returnvalue "/Game/FirstPerson/Input/IMC_Default.IMC_Default" (struct))
      (`EnhancedInputSubsystemInterface.RemoveMappingContext` _returnvalue "/Game/_VisionProtocol/Core/Input/IMC_Parkour.IMC_Parkour" (struct))
      (`EnhancedInputSubsystemInterface.RemoveMappingContext` _returnvalue "/Game/_VisionProtocol/Core/Input/ActionSpecificInputMappingContexts/IMC_Dashing.IMC_Dashing" (struct))
      (`EnhancedInputSubsystemInterface.AddMappingContext` _returnvalue "/Game/_VisionProtocol/Core/Input/ActionSpecificInputMappingContexts/IMC_Sliding.IMC_Sliding" 0 (struct)))))

(event `ExitSlidingContext`
  (bind _returnvalue (subsystem `EnhancedInputLocalPlayerSubsystem`))
  (`/Engine/EditorBlueprintResources/StandardMacros.IsValid` _returnvalue
    (:`Is Valid`
      (`EnhancedInputSubsystemInterface.AddMappingContext` _returnvalue "/Game/FirstPerson/Input/IMC_Default.IMC_Default" 0 (struct))
      (`EnhancedInputSubsystemInterface.AddMappingContext` _returnvalue "/Game/_VisionProtocol/Core/Input/IMC_Parkour.IMC_Parkour" 0 (struct))
      (`EnhancedInputSubsystemInterface.RemoveMappingContext` _returnvalue "/Game/_VisionProtocol/Core/Input/ActionSpecificInputMappingContexts/IMC_Sliding.IMC_Sliding" (struct)))))

(event `InitiateHorizontalWallRunningContext`
  (bind _returnvalue (subsystem `EnhancedInputLocalPlayerSubsystem`))
  (`/Engine/EditorBlueprintResources/StandardMacros.IsValid` _returnvalue
    (:`Is Valid`
      (`EnhancedInputSubsystemInterface.RemoveMappingContext` _returnvalue "/Game/FirstPerson/Input/IMC_Default.IMC_Default" (struct))
      (`EnhancedInputSubsystemInterface.RemoveMappingContext` _returnvalue "/Game/_VisionProtocol/Core/Input/IMC_Parkour.IMC_Parkour" (struct))
      (`EnhancedInputSubsystemInterface.RemoveMappingContext` _returnvalue "/Game/_VisionProtocol/Core/Input/ActionSpecificInputMappingContexts/IMC_Dashing.IMC_Dashing" (struct))
      (`EnhancedInputSubsystemInterface.AddMappingContext` _returnvalue "/Game/_VisionProtocol/Core/Input/ActionSpecificInputMappingContexts/IMC_HorizontalWallRunning.IMC_HorizontalWallRunning" 0 (struct)))))

(event `ExitHorizontalWallRunningContext`
  (bind _returnvalue (subsystem `EnhancedInputLocalPlayerSubsystem`))
  (`/Engine/EditorBlueprintResources/StandardMacros.IsValid` _returnvalue
    (:`Is Valid`
      (`EnhancedInputSubsystemInterface.AddMappingContext` _returnvalue "/Game/FirstPerson/Input/IMC_Default.IMC_Default" 0 (struct))
      (`EnhancedInputSubsystemInterface.AddMappingContext` _returnvalue "/Game/_VisionProtocol/Core/Input/IMC_Parkour.IMC_Parkour" 0 (struct))
      (`EnhancedInputSubsystemInterface.RemoveMappingContext` _returnvalue "/Game/_VisionProtocol/Core/Input/ActionSpecificInputMappingContexts/IMC_HorizontalWallRunning.IMC_HorizontalWallRunning" (struct)))))

(event `InitiateGrapplingHookContext`
  (bind _returnvalue (subsystem `EnhancedInputLocalPlayerSubsystem`))
  (`/Engine/EditorBlueprintResources/StandardMacros.IsValid` _returnvalue
    (:`Is Valid`
      (`EnhancedInputSubsystemInterface.RemoveMappingContext` _returnvalue "/Game/FirstPerson/Input/IMC_Default.IMC_Default" (struct))
      (`EnhancedInputSubsystemInterface.RemoveMappingContext` _returnvalue "/Game/_VisionProtocol/Core/Input/IMC_Parkour.IMC_Parkour" (struct))
      (`EnhancedInputSubsystemInterface.RemoveMappingContext` _returnvalue "/Game/_VisionProtocol/Core/Input/ActionSpecificInputMappingContexts/IMC_Dashing.IMC_Dashing" (struct))
      (`EnhancedInputSubsystemInterface.AddMappingContext` _returnvalue "/Game/_VisionProtocol/Core/Input/ActionSpecificInputMappingContexts/IMC_GrapplingHook.IMC_GrapplingHook" 0 (struct)))))

(event `ExitGrapplingHookContext`
  (bind _returnvalue (subsystem `EnhancedInputLocalPlayerSubsystem`))
  (`/Engine/EditorBlueprintResources/StandardMacros.IsValid` _returnvalue
    (:`Is Valid`
      (`EnhancedInputSubsystemInterface.AddMappingContext` _returnvalue "/Game/FirstPerson/Input/IMC_Default.IMC_Default" 0 (struct))
      (`EnhancedInputSubsystemInterface.AddMappingContext` _returnvalue "/Game/_VisionProtocol/Core/Input/IMC_Parkour.IMC_Parkour" 0 (struct))
      (`EnhancedInputSubsystemInterface.RemoveMappingContext` _returnvalue "/Game/_VisionProtocol/Core/Input/ActionSpecificInputMappingContexts/IMC_GrapplingHook.IMC_GrapplingHook" (struct)))))

(event `InitiateDialogContext`
  (bind _returnvalue (subsystem `EnhancedInputLocalPlayerSubsystem`))
  (`/Engine/EditorBlueprintResources/StandardMacros.IsValid` _returnvalue
    (:`Is Valid`
      (`EnhancedInputSubsystemInterface.RemoveMappingContext` _returnvalue "/Game/FirstPerson/Input/IMC_Default.IMC_Default" (struct))
      (`EnhancedInputSubsystemInterface.RemoveMappingContext` _returnvalue "/Game/_VisionProtocol/Core/Input/IMC_Parkour.IMC_Parkour" (struct))
      (`EnhancedInputSubsystemInterface.RemoveMappingContext` _returnvalue "/Game/_VisionProtocol/Core/Input/ActionSpecificInputMappingContexts/IMC_Dashing.IMC_Dashing" (struct))
      (`EnhancedInputSubsystemInterface.RemoveMappingContext` _returnvalue "/Game/_VisionProtocol/Core/Input/IMC_Weapons.IMC_Weapons" (struct))
      (`EnhancedInputSubsystemInterface.AddMappingContext` _returnvalue "/Game/_VisionProtocol/Core/Input/IMC_Dialog.IMC_Dialog" 1 (struct)))))

(event `ExitDialogContext`
  (bind _returnvalue (subsystem `EnhancedInputLocalPlayerSubsystem`))
  (`/Engine/EditorBlueprintResources/StandardMacros.IsValid` _returnvalue
    (:`Is Valid`
      (`EnhancedInputSubsystemInterface.AddMappingContext` _returnvalue "/Game/FirstPerson/Input/IMC_Default.IMC_Default" 0 (struct))
      (`EnhancedInputSubsystemInterface.AddMappingContext` _returnvalue "/Game/_VisionProtocol/Core/Input/IMC_Parkour.IMC_Parkour" 0 (struct))
      (`EnhancedInputSubsystemInterface.AddMappingContext` _returnvalue "/Game/_VisionProtocol/Core/Input/IMC_Weapons.IMC_Weapons" 0 (struct))
      (`EnhancedInputSubsystemInterface.RemoveMappingContext` _returnvalue "/Game/_VisionProtocol/Core/Input/IMC_Dialog.IMC_Dialog" (struct)))))

(fn `UserConstructionScript`
  (`parent.UserConstructionScript`))
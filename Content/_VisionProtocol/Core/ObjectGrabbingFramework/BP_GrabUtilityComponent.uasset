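; Grab utility component that lets a grabber pick up and carry a primitive component in front of the first-person camera.
; OnGrabbed alternates via FlipFlop between grabbing the component with the grabber's PhysicsHandle and releasing it.
; While grabbed, Tick moves the handle target to a fixed distance along the player camera's forward vector, matching camera rotation.
; It always follows player 0's BP_FirstPersonCharacter camera, regardless of the grabber.
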(event `OnGrabbed`
  (params (Grabber :type "Actor Object Reference") (GrabbedComponent :type "PrimitiveComponent Object Reference"))
  (bind _returnvalue (`Actor.GetComponentByClass` Grabber "/Script/Engine.PhysicsHandleComponent"))
  ;[1 1 1] Grabbing and Releasing Logic
  (`/Engine/EditorBlueprintResources/StandardMacros.FlipFlop`
    (:`A`
      (set `self.GraberPhysicsHandle` _returnvalue)
      (`/Engine/EditorBlueprintResources/StandardMacros.IsValid` _returnvalue
        (:`Is Valid`
          (`KismetSystemLibrary.PrintString` "valid")
          (`PhysicsHandleComponent.GrabComponentAtLocationWithRotation` (`self.GraberPhysicsHandle`) GrabbedComponent "None" (`SceneComponent.K2_GetComponentLocation` GrabbedComponent) (`SceneComponent.K2_GetComponentRotation` GrabbedComponent))
          (set `self.IsPrimitiveGrabbed` true))
        (:`Is Not Valid`
          (`KismetSystemLibrary.PrintString` "inwalida"))))
    (:`B`
      (`PhysicsHandleComponent.ReleaseComponent` (`self.GraberPhysicsHandle`))
      (set `self.IsPrimitiveGrabbed` false))))

(event `self.ReceiveTick`
  (params (DeltaSeconds :type "Float (single-precision)"))
  (bind _asbp_first_person_character (cast `/Game/FirstPerson/Blueprints/BP_FirstPersonCharacter` (`GameplayStatics.GetPlayerPawn` 0)))
  (if (`self.IsPrimitiveGrabbed`)
    (bind _returnvalue (`SceneComponent.K2_GetComponentRotation` (`/Game/FirstPerson/Blueprints/BP_FirstPersonCharacter.FirstPersonCamera` _asbp_first_person_character)))
    (`PhysicsHandleComponent.SetTargetLocationAndRotation` (`self.GraberPhysicsHandle`) (+ (`SceneComponent.K2_GetComponentLocation` (`/Game/FirstPerson/Blueprints/BP_FirstPersonCharacter.FirstPersonCamera` _asbp_first_person_character)) (* (`KismetMathLibrary.GetForwardVector` _returnvalue) 350.0)) _returnvalue)))
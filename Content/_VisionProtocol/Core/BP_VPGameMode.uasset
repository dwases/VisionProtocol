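; Game mode for Vision Protocol that acts as a simple background music controller, with play, stop, pause and resume events.
; PlayMusic fades out any active player and fades in a new 2D sound flagged to persist across level transitions, producing a crossfade.
; StopMusic copies the active player into a separate fade-out reference, while pause and resume act directly on the active player.
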(event `/Game/_VisionProtocol/Core/MusicPlayer/BPI_MusicPlayer.PlayMusic`
  (params (Music :type "SoundBase Object Reference") (OldFadeOutTime :type "Float (double-precision)") (NewFadeInTime :type "Float (double-precision)"))
  (set `self.Music` Music)
  (set `self.Old Fade Out Time` OldFadeOutTime)
  (set `self.New Fade in Time` NewFadeInTime)
  (`/Engine/EditorBlueprintResources/StandardMacros.IsValid` (`self.ActiveMusicPlayer`)
    (:`Is Valid`
      (`self.StopMusic` (`self.Old Fade Out Time`)))
    (:`Is Not Valid`
      _))
  (bind _returnvalue (`GameplayStatics.CreateSound2D` (`self.Music`) 1.0 1.0 0.0 null true))
  (bind _output_get (set `self.ActiveMusicPlayer` _returnvalue))
  (`AudioComponent.FadeIn` _output_get (`self.New Fade in Time`) 1.0 0.0 "Linear"))

(event `/Game/_VisionProtocol/Core/MusicPlayer/BPI_MusicPlayer.StopMusic`
  (params (FadeOutTime :type "Float (double-precision)"))
  (bind _output_get (set `self.FadeOutMusicPlayer` (`self.ActiveMusicPlayer`)))
  (`AudioComponent.FadeOut` _output_get FadeOutTime 0.0 "Linear"))

(event `/Game/_VisionProtocol/Core/MusicPlayer/BPI_MusicPlayer.PauseMusic`
  (`AudioComponent.SetPaused` (`self.ActiveMusicPlayer`) true))

(event `/Game/_VisionProtocol/Core/MusicPlayer/BPI_MusicPlayer.ResumeMusic`
  (`AudioComponent.SetPaused` (`self.ActiveMusicPlayer`) false))

(fn `UserConstructionScript`
  (`parent.UserConstructionScript`))
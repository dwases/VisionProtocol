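; Dialog system component that plays branching conversations from a data table, addressing rows by numeric ID.
; BeginDialog caches row names, and each NextDialog call prints the speaker and line and swaps the 2D voice audio.
; Branching rows spawn a choice widget whose selection sets the next ID and advances, while linear rows await another NextDialog call.
; IDs are decremented into zero-based indices, with a negative result ending the dialog.
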(fn `BeginDialog`
  (params (DialogScript :type "DataTable Object Reference"))
  (if (`self.DialogOngoing`)
    (`KismetSystemLibrary.PrintString` "Cannot begin new dialog, because there is an ongoing dialog!")
    (else
      (bind _output_get (set `self.DialogScript` DialogScript))
      (bind _outrownames (`DataTableFunctionLibrary.GetDataTableRowNames` _output_get))
      (set `self.RowNames` _outrownames)
      (set `self.DialogID` 1)
      (set `self.DialogOngoing` true)
      (`self.NextDialog`))))

(fn `ChosenDialogueOption`
  (params (ChosenOption :type Integer))
  (bind _returnvalue (`|GetDataTableRow` (`self.DialogScript`) (`|GetArrayItem` (`self.RowNames`) (`self.DialogID`)))
    (:`then`
      (bind (_rozmowca _tekst _dzwiek _wybory _nastepnedialogi) (break `/Game/_VisionProtocol/Core/DialogSystem/ST_DialogData` _returnvalue))
      ;[1 1 1] TODO: Usunąć wypisywanie odpowiedzi gracza
      (`KismetSystemLibrary.PrintText` (`|GetArrayItem` _wybory ChosenOption))
      (bind _output (`|GetArrayItem` _nastepnedialogi ChosenOption))
      (`KismetSystemLibrary.PrintString` (`KismetStringLibrary.Conv_IntToString` _output))
      (set `self.DialogID` _output)
      (`self.NextDialog`))))

(fn `NextDialog`
  (bind _activeaudioplayer (`self.ActiveAudioPlayer`))
  (if (`self.DialogOngoing`)
    (bind _result (`/Engine/EditorBlueprintResources/StandardMacros.DecrementInt` (`self.DialogID`))
      (:`  `
        (if (< _result 0)
          (set `self.DialogOngoing` false)
          (`KismetSystemLibrary.PrintString` "KONIEC!")
          (else
            (bind _returnvalue (`|GetDataTableRow` (`self.DialogScript`) (`|GetArrayItem` (`self.RowNames`) (`self.DialogID`)))
              (:`then`
                (bind (_rozmowca _tekst _dzwiek _wybory _nastepnedialogi _nastepnydialog) (break `/Game/_VisionProtocol/Core/DialogSystem/ST_DialogData` _returnvalue))
                (`KismetSystemLibrary.PrintString` (`KismetTextLibrary.Conv_TextToString` (`|FormatText` "{Rozmowca}: \n{Tekst}" _rozmowca _tekst)) true true (struct :`G` 0.66 :`B` 1.0 :`A` 1.0) 5.0)
                ;[1 1 1] Play audio
                (`/Engine/EditorBlueprintResources/StandardMacros.IsValid` _activeaudioplayer
                  (:`Is Valid`
                    (`AudioComponent.Stop` _activeaudioplayer))
                  (:`Is Not Valid`
                    _))
                (bind _returnvalue_2 (`GameplayStatics.CreateSound2D` _dzwiek 1.0 1.0 0.0 null))
                (bind _output_get (set `self.ActiveAudioPlayer` _returnvalue_2))
                (`AudioComponent.Play` _output_get 0.0)
                (if (`KismetArrayLibrary.Array_IsNotEmpty` _nastepnedialogi)
                  (bind _returnvalue_3 (`|CreateWidget` "/Game/_VisionProtocol/Widgets/Dialogues/WBP_Dialog_Choice.WBP_Dialog_Choice_C"))
                  (add `/Game/_VisionProtocol/Widgets/Dialogues/WBP_Dialog_Choice.DialogueChosenDispatcher` _returnvalue_3 (`|CreateDelegate` :!event `ChosenDialogueOption`))
                  (`UserWidget.AddToViewport` _returnvalue_3 0)
                  (`/Game/_VisionProtocol/Widgets/Dialogues/WBP_Dialog_Choice.AddDialogueOptions` _returnvalue_3 _wybory)
                  (else
                    (set `self.DialogID` _nastepnydialog)))))))))))
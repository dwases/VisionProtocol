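; BP_DragonBase is a base dragon boss character exposing health, damage and movement-speed functions, with health handled by the CDMGHP component.
; On BeginPlay it prepares path locations and per-move speeds, resetting mismatched speeds to defaults, and converts fly-point offsets to world space from its start transform.
; When a move completes with the Start state tag, it shows a boss health bar, removed on visibility change.
; Patrol route and location point getters are stubs.
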(event `self.ReceiveBeginPlay`
  (`|ExecutionSequence`
    (:`then_0`
      (set `self.BaseLocation` (`SceneComponent.K2_GetComponentLocation` (`self.CapsuleComponent`)))
      (`self.AddFirstVector`)
      (if (== (- (`KismetArrayLibrary.Array_Length` (`self.ArrayLocations`)) 1) (`KismetArrayLibrary.Array_Length` (`self.ArrayofSpeeds`)))
        ;[1 1 1] jeżeli Locations i Speeds mają tyle samo wartosci, to prędkosci się ustawią, w przeciwnym wypadku będą domyslne czyli 1s
        (`self.SetArrayOfSpeeds` (`self.ArrayofSpeeds`))
        (else
          (`self.SetArrayOfSpeeds` _)
          (`KismetSystemLibrary.LogString` "Array of Speeds is not the same lenght as Array of Locations"))))
    (:`then_1`
      (add `self.OnMoveCompleted` (delegate `AddHPBar`)))
    (:`then_2`
      (for _array_element (`self.ArrayofFlyPointLocations`)
        (`KismetArrayLibrary.Array_Add` (`self.StaticAOFPL`) (+ (`self.BaseLocation`) (`KismetMathLibrary.GreaterGreater_VectorRotator` _array_element (`self.K2_GetActorRotation`))))))))

(event `AddHPBar`
  (if (`BlueprintGameplayTagLibrary.HasTag` (`self.GTC`) (struct :`TagName` "Dragons.State.Start"))
    (bind _returnvalue (`|CreateWidget` "/Game/_VisionProtocol/TestingPlayground/Filip/T_Smok/WBP_BossHealthBar.WBP_BossHealthBar_C" null self))
    (set `self.HP Widger Ref` _returnvalue)
    (add `UserWidget.OnVisibilityChanged` _returnvalue (delegate `OnVisibilityChanged_Event`))
    (`UserWidget.AddToViewport` _returnvalue 0)))

(event `OnVisibilityChanged_Event`
  (params (InVisibility :type "ESlateVisibility Enum" :default "Visible"))
  (`Widget.RemoveFromParent` (stale `AddHPBar` _returnvalue)))

(fn `AddFirstVector`
  (bind _arraylocations (`self.ArrayLocations`))
  (if (not (== (`|GetArrayItem` _arraylocations) (0.0 0.0 0.0)))
    (`KismetArrayLibrary.Array_Reverse` _arraylocations)
    (`KismetArrayLibrary.Array_AddUnique` _arraylocations)
    (`KismetArrayLibrary.Array_Reverse` _arraylocations)))

(fn `GetCurrentHealth`
  (returns (Health :type "Float (double-precision)"))
  (return (`/Game/_VisionProtocol/Core/DMG-HP/C_DMG-HP.CurrentHealth` (`self.C_DMG-HP`))))

(fn `GetIdealRange`
  (returns (AttackRadius :type "Float (double-precision)") (DefenseRadius :type "Float (double-precision)"))
  (return 100.0 400.0))

(fn `GetLocationPoint`
  (returns (Location :type "Vector Structure"))
  (return (0.0 0.0 0.0)))

(fn `GetMaxHealth`
  (returns (MaxHealth :type "Float (double-precision)"))
  (return (`/Game/_VisionProtocol/Core/DMG-HP/C_DMG-HP.MaximumHealth` (`self.C_DMG-HP`))))

(fn `GetPatrolRoute`
  (returns (PatrolRoute :type "/Game/_VisionProtocol/Core/AI/BP_PatrolPath1 Object Reference"))
  (return null))

(fn `Heal`
  (params (HP_Amount :type "Float (double-precision)"))
  (returns (`New Health` :type "Float (double-precision)"))
  (bind _new_health (`/Game/_VisionProtocol/Core/DMG-HP/C_DMG-HP.Heal` (`self.C_DMG-HP`) HP_Amount))
  (return _new_health))

(fn `IsDead`
  (returns (Dead :type Boolean))
  (return (`/Game/_VisionProtocol/Core/DMG-HP/C_DMG-HP.isDead` (`self.C_DMG-HP`))))

(fn `SetArrayOfSpeeds`
  (params (NewParam :type "Array of Float (double-precision)"))
  (bind _arraylocations (`self.ArrayLocations`))
  (bind _arrayofspeeds (`self.ArrayofSpeeds`))
  (if (`KismetArrayLibrary.Array_IsEmpty` NewParam)
    (`KismetArrayLibrary.Array_Clear` _arrayofspeeds)
    (for (_ _array_index) _arraylocations
      (if (not (== (`KismetArrayLibrary.Array_Length` _arraylocations) (- _array_index 1)))
        (`KismetArrayLibrary.Array_Add` _arrayofspeeds)))
    (else
      (set `self.ArrayofSpeeds` NewParam))))

(fn `SetMovementSpeed`
  (params (Speed :type "/Game/_VisionProtocol/Core/AI/Enums/E_MovementSpeed Enum" :default "NewEnumerator0"))
  (returns (SpeedValue :type "Float (double-precision)"))
  (bind _output_get (set `CharacterMovementComponent.MaxWalkSpeed` (select `/Game/_VisionProtocol/Core/AI/Enums/E_MovementSpeed` Speed :`NewEnumerator1` 10000.0 :`NewEnumerator2` 150.0 :`NewEnumerator3` 350.0 :`NewEnumerator4` 450.0 :`NewEnumerator5` 700.0) (`self.CharacterMovement`)))
  (return _output_get))

(fn `TakeDamage`
  (params (Amount :type "Float (double-precision)"))
  (returns (`Was Damaged` :type Boolean))
  (bind _c_dmg_hp (`self.C_DMG-HP`))
  (bind _was_damaged (`/Game/_VisionProtocol/Core/DMG-HP/C_DMG-HP.TakeDamage` _c_dmg_hp Amount))
  (`/Game/_VisionProtocol/Core/DMG-HP/C_DMG-HP.BasicDamageResponse` _c_dmg_hp)
  (return _was_damaged))

(fn `UserConstructionScript`
  (bind _c_dmg_hp (`self.C_DMG-HP`))
  (`SceneComponent.K2_SetRelativeLocation` (`self.StartTrigger`) (`self.StartTriggerLocation`) false false)
  (bind _output_get (set `/Game/_VisionProtocol/Core/DMG-HP/C_DMG-HP.MaximumHealth` 500.0 _c_dmg_hp))
  (set `/Game/_VisionProtocol/Core/DMG-HP/C_DMG-HP.CurrentHealth` _output_get _c_dmg_hp))
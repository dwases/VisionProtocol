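; Tutorial dragon boss that flies in along a waypoint path, fights the player and announces a rocket-boots reward on death.
; A player trigger starts an invisible elevator that carries it, then is destroyed to begin the fight.
; Gameplay tags track phases for AI tasks running wind-slice volleys, tail spins and biting rushes.
; Rushing into pillars stuns it; each accepted hit removes one sixth of health, with Invincible tags gating normal damage.
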(event `/Game/_VisionProtocol/TestingPlayground/Filip/Urojony_Smok/BT/BPI_Urojony.SwitchFunction`
  (params (`Event Name` :type Name) (Task :type "BTTask_BlueprintBase Object Reference") (RotationSpeed :type "Float (double-precision)"))
  (bind _gtc (`self.GTC`))
  (bind _gtc_2 (`self.GTC`))
  (bind _gtc_3 (`self.GTC`))
  (switch `name` `Event Name`
    (:`FinishZero`
      (`BlueprintGameplayTagLibrary.RemoveGameplayTag` _gtc (struct :`TagName` "Dragons.Urojony.StateZero"))
      (`BlueprintGameplayTagLibrary.AddGameplayTag` _gtc (struct :`TagName` "Dragons.Attack.WindAttack"))
      (`BlueprintGameplayTagLibrary.RemoveGameplayTag` _gtc (struct :`TagName` "Dragons.Attack.RushAttack"))
      (`BlueprintGameplayTagLibrary.RemoveGameplayTag` _gtc (struct :`TagName` "Dragons.State.Moving")))
    (:`SetTask`
      (set `self.Task` Task))
    (:`RushAttack`
      (`BlueprintGameplayTagLibrary.RemoveGameplayTag` _gtc_3 (struct :`TagName` "Dragons.Attack.WindAttack"))
      (`BlueprintGameplayTagLibrary.AddGameplayTag` _gtc_3 (struct :`TagName` "Dragons.Attack.RushAttack"))
      (`BlueprintGameplayTagLibrary.AddGameplayTag` _gtc_3 (struct :`TagName` "Dragons.State.Moving")))
    (:`WindAttack`
      (`BlueprintGameplayTagLibrary.RemoveGameplayTag` _gtc_2 (struct :`TagName` "Dragons.Attack.RushAttack"))
      (`BlueprintGameplayTagLibrary.RemoveGameplayTag` _gtc_2 (struct :`TagName` "Dragons.Attack.Biting"))
      (`BlueprintGameplayTagLibrary.RemoveGameplayTag` _gtc_2 (struct :`TagName` "Dragons.State.Moving"))
      (`BlueprintGameplayTagLibrary.AddGameplayTag` _gtc_2 (struct :`TagName` "Dragons.Attack.WindAttack")))))

(event `Fly To`
  (params (Location :type "Vector Structure") (Task :type "BTTask_BlueprintBase Object Reference"))
  (set `self.BaseLocation` (`self.K2_GetActorLocation`))
  (if (`BlueprintGameplayTagLibrary.HasTag` (`self.GTC`) (struct :`TagName` "Dragons.State.Moving"))
    (`TimelineComponent.SetPlayRate` (`self.FlyTo`) 0.4)
    (bind (_direction _1_5s) (`Timeline|FlyTo` :!via `PlayFromStart` :!label _label)
      (:`Update`
        (`self.K2_SetActorLocation` (`KismetMathLibrary.VLerp` (`self.BaseLocation`) Location _1_5s) false true))
      (:`Finished`
        (`BTTask_BlueprintBase.FinishExecute` Task true)
        (if (`BlueprintGameplayTagLibrary.HasTag` (`self.GTC`) (struct :`TagName` "Dragons.State.Moving"))
          (`TimelineComponent.SetPlayRate` (`self.FlyTo`) 1.0))))
    (else
      (goto _label :!via `PlayFromStart`))))

(event `Landing`
  (params (Location :type "Vector Structure"))
  (set `self.BaseLocation` (`self.K2_GetActorLocation`))
  (bind (_direction _1_5s) (`Timeline|LandingHP` :!via `PlayFromStart`)
    (:`Update`
      (`self.K2_SetActorLocation` (`KismetMathLibrary.VLerp` (`self.BaseLocation`) Location _1_5s) false true))
    (:`Finished`
      (`BlueprintGameplayTagLibrary.AddGameplayTag` (`self.GTC`) (struct :`TagName` "Dragons.State.Landed")))))

(event `Death`
  (bind _mesh (`self.Mesh`))
  (bind (_actorrotation_roll _actorrotation_pitch _actorrotation_yaw) (`KismetMathLibrary.BreakRotator` (`self.ActorRotation`)))
  (bind (_relativelocation_x _relativelocation_y) (`KismetMathLibrary.BreakVector` (`SceneComponent.RelativeLocation` _mesh)))
  (`BlueprintGameplayTagLibrary.AddGameplayTag` (`self.GTC`) (struct :`TagName` "Dragons.State.Dead"))
  (clear `self.OnDeath`)
  (`GameplayStatics.PlaySoundAtLocation` "/Game/_VisionProtocol/Audio/SFX/NewSFX/smok_ryk.smok_ryk" (`self.K2_GetActorLocation`) (struct) 0.5 1.0 0.0 null null null null)
  (`/Engine/EditorBlueprintResources/StandardMacros.Do N` 1
    (:`Exit`
      (set `self.ActorRotation` (`self.K2_GetActorRotation`))
      (`BrainComponent.StopLogic` (`AIController.BrainComponent` (`AIBlueprintHelperLibrary.GetAIController` self)) "")
      (bind (_direction _0_5_sec) (`Timeline|Smierc` :!via `PlayFromStart`)
        (:`Update`
          (`SceneComponent.K2_SetRelativeRotation` (`self.Mesh`) (`KismetMathLibrary.MakeRotator` _actorrotation_roll (+ (* _0_5_sec 90.0) _actorrotation_pitch) _actorrotation_yaw) false false))
        (:`Finished`
          (bind (_direction_2 _2_sec) (`Timeline|Smierc2` :!via `PlayFromStart`)
            (:`Update`
              (`SceneComponent.K2_SetRelativeLocation` _mesh (`KismetMathLibrary.MakeVector` _relativelocation_x _relativelocation_y (* _2_sec -1500.0)) false false))
            (:`Finished`
              (`Widget.SetVisibility` (`self.HP Widger Ref`) "Hidden")
              (`KismetSystemLibrary.Delay` 3.0)
              (bind _asplayer_hud (cast `/Game/_VisionProtocol/Core/PlayerHUD` (`PlayerController.GetHUD` (`GameplayStatics.GetPlayerController` 0))))
              (`/Game/_VisionProtocol/Widgets/Dialogues/WBP_PopUp.AddPopUp` (`/Game/_VisionProtocol/Core/PlayerHUD.PopUpWidget` _asplayer_hud) "Gratulacje, zdobyłeś nową część – buty rakietowe. Pozwalają na skakanie w powietrzu.")
              (`KismetSystemLibrary.Delay` 0.5)
              (`self.K2_DestroyActor`))))))))

(event `Destroy Elevator`
  (bind _c_dmg_hp (`self.C_DMG-HP`))
  (bind (_returnvalue_roll _returnvalue_pitch _returnvalue_yaw) (`KismetMathLibrary.BreakRotator` (`KismetMathLibrary.FindLookAtRotation` (`self.K2_GetActorLocation`) (`self.K2_GetActorLocation` (`GameplayStatics.GetPlayerCharacter` 0)))))
  (`self.K2_DestroyActor` (`self.ElevatorRef`))
  (set `self.ElevatorRef` null)
  (`self.K2_SetActorRotation` (`KismetMathLibrary.MakeRotator` 0.0 0.0 _returnvalue_yaw))
  (`KismetSystemLibrary.Delay` 1.0)
  (`BlueprintGameplayTagLibrary.AddGameplayTag` (`self.GTC`) (struct :`TagName` "Dragons.State.Start"))
  (`self.OnMoveCompleted`)
  (set `/Game/_VisionProtocol/Core/DMG-HP/C_DMG-HP.CurrentHealth` (`/Game/_VisionProtocol/Core/DMG-HP/C_DMG-HP.MaximumHealth` _c_dmg_hp) _c_dmg_hp))

(event `self.ReceiveBeginPlay`
  (bind _arraylocations (`self.ArrayLocations`))
  (bind _output (`|GetArrayItem` (`self.ArrayofSpeeds`) (`self.IndexOfLocation`)))
  (`parent.ReceiveBeginPlay`)
  (`SceneComponent.SetHiddenInGame` (`self.Mesh`) true false)
  (bind _returnvalue (`|SpawnActorFromClass` "/Game/_VisionProtocol/Objects/BP_ElevatorPlatform.BP_ElevatorPlatform_C" (`self.GetTransform`) "Undefined" "MultiplyWithRoot" null false 2.0 0.0 null))
  (add `/Game/_VisionProtocol/Objects/BP_MovingPlatform.OnStopped` _returnvalue (delegate `Destroy Elevator`))
  (bind _output_get (set `self.ElevatorRef` _returnvalue))
  (bind _cube (`/Game/_VisionProtocol/Objects/BP_MovingPlatform.Cube` _output_get))
  (`PrimitiveComponent.SetMaterial` _cube 0 "/Engine/Engine_MI_Shaders/Instances/M_Shader_SimpleTranslucent_Invis.M_Shader_SimpleTranslucent_Invis")
  (`PrimitiveComponent.SetCollisionResponseToAllChannels` _cube "ECR_Ignore")
  (for (_array_element _array_index) _arraylocations
    ;[1 1 1] każdy punkt z arraya przygotowujemy tak, aby naprawić punkty względem rotacji smoka
    (`KismetArrayLibrary.Array_Set` _arraylocations _array_index (`KismetMathLibrary.GreaterGreater_VectorRotator` _array_element (`self.K2_GetActorRotation`))))
  (set `/Game/_VisionProtocol/Objects/BP_MovingPlatform.TargetLocations` _arraylocations _returnvalue)
  (`self.K2_AttachToActor` _returnvalue "None" "SnapToTarget" "KeepWorld" "KeepWorld")
  (add `/Game/_VisionProtocol/Objects/BP_MovingPlatform.OnPointReached` _returnvalue (delegate `SetNewSpeed`))
  (if (not (== _output 0.0))
    (set `/Game/_VisionProtocol/Objects/BP_MovingPlatform.TimeToReachDestination` _output (`self.ElevatorRef`)))
  (`/Engine/EditorBlueprintResources/StandardMacros.IncrementInt` (`self.IndexOfLocation`)
    (:`  `
      (`self.RotateTowards`))))

(event `SetNewSpeed`
  (bind _output (`|GetArrayItem` (`self.ArrayofSpeeds`) (`self.IndexOfLocation`)))
  ;[1 1 1] Ustaw prędkosc na prędkosc z ArrayOfSpeeds, jezeli ta prędkosc to 0, zostaw domyslną
  (if (not (== _output 0.0))
    (set `/Game/_VisionProtocol/Objects/BP_MovingPlatform.TimeToReachDestination` _output (`self.ElevatorRef`)))
  (`/Engine/EditorBlueprintResources/StandardMacros.IncrementInt` (`self.IndexOfLocation`)
    (:`  `
      (`self.RotateTowards`))))

(event `self.StartTrigger.OnComponentBeginOverlap`
  (params (OverlappedComponent :type "PrimitiveComponent Object Reference") (OtherActor :type "Actor Object Reference") (OtherComp :type "PrimitiveComponent Object Reference") (OtherBodyIndex :type Integer) (bFromSweep :type Boolean) (SweepResult :type "HitResult Structure (by ref)"))
  (cast `/Game/_VisionProtocol/Core/BP_VPPlayerCharacter` OtherActor)
  (`self.Start`))

(event `RotateTowards`
  (bind (_returnvalue_roll _returnvalue_pitch _returnvalue_yaw) (`KismetMathLibrary.BreakRotator` (`KismetMathLibrary.FindLookAtRotation` (`SceneComponent.K2_GetComponentLocation` (`self.CapsuleComponent`)) (+ (`self.BaseLocation`) (`|GetArrayItem` (`self.ArrayLocations`) (`self.IndexOfLocation`))))))
  (`self.K2_SetActorRotation` (`KismetMathLibrary.MakeRotator` 0.0 0.0 _returnvalue_yaw)))

(event `/Game/_VisionProtocol/Core/AI/BPI_Enemy.SpecialAttack2`
  (bind (_actorrotation_roll _actorrotation_pitch _actorrotation_yaw) (`KismetMathLibrary.BreakRotator` (`self.ActorRotation`)))
  ;[1 1 1] ATAK OGONEM
  (`GameplayStatics.PlaySoundAtLocation` "/Game/_VisionProtocol/Audio/SFX/NewSFX/dragonTail.dragonTail" (`self.K2_GetActorLocation`) (struct) 1.0 1.0 0.0 null null null null)
  (set `self.ActorRotation` (`self.K2_GetActorRotation`))
  (bind (_direction _1sec) (`Timeline|TailAttack` :!via `PlayFromStart`)
    (:`Update`
      (`self.K2_SetActorRotation` (`KismetMathLibrary.MakeRotator` _actorrotation_roll _actorrotation_pitch (+ (* _1sec 360.0) _actorrotation_yaw))))))

(event `/Game/_VisionProtocol/Core/AI/BPI_Enemy.SpecialAttack1`
  (bind _returnvalue_x (`KismetMathLibrary.BreakVector` (`SceneComponent.K2_GetComponentScale` (`self.Mesh`))))
  (bind _returnvalue_location (`KismetMathLibrary.BreakTransform` (`SceneComponent.K2_GetComponentToWorld` (`self.ProjectileSpawn`))))
  (bind _returnvalue_location_2 (`KismetMathLibrary.BreakTransform` (`SceneComponent.K2_GetComponentToWorld` (`self.ProjectileSpawn`))))
  (bind (_returnvalue_roll _returnvalue_pitch _returnvalue_yaw) (`KismetMathLibrary.BreakRotator` (`KismetMathLibrary.FindLookAtRotation` _returnvalue_location_2 (`self.K2_GetActorLocation` (`GameplayStatics.GetPlayerCharacter` 0)))))
  (bind _returnvalue (* (`KismetMathLibrary.FMin` (* _returnvalue_x 0.5) 1.0) 15000.0))
  ;[1 1 1] Tylko dla wizualnego efektu. Czekamy na animacje.
  (`SceneComponent.K2_AddRelativeLocation` (`self.CapsuleComponent`) (0.0 0.0 200.0) false false)
  (if (< (`self.Bullet_I`) 5) :!label _label_2
    (if (`KismetMathLibrary.RandomBool`)
      (for _index (range 3)
        (`|SpawnActorFromClass` "/Game/_VisionProtocol/Core/Weapons/Projectiles/BP_Dragon_WindSlice.BP_Dragon_WindSlice_C" (`KismetMathLibrary.MakeTransform` _returnvalue_location_2 (`KismetMathLibrary.MakeRotator` _returnvalue_roll _returnvalue_pitch (+ (* _index 2) _returnvalue_yaw))) "AdjustIfPossibleButAlwaysSpawn" "MultiplyWithRoot" self (struct) _returnvalue null)
        (`GameplayStatics.PlaySoundAtLocation` "/Game/_VisionProtocol/Audio/SFX/NewSFX/dash.dash" _returnvalue_location_2 (struct) 0.5 1.0 0.0 null null null null))
      (else
        (for _index_2 (range 3)
          (`|SpawnActorFromClass` "/Game/_VisionProtocol/Core/Weapons/Projectiles/BP_Dragon_WindSlice.BP_Dragon_WindSlice_C" (`KismetMathLibrary.MakeTransform` _returnvalue_location (`KismetMathLibrary.MakeRotator` 0.0 (+ (* _index_2 2) _returnvalue_pitch) _returnvalue_yaw)) "AdjustIfPossibleButAlwaysSpawn" "MultiplyWithRoot" self (struct :`Roll` 90.0) _returnvalue null)
          (`GameplayStatics.PlaySoundAtLocation` "/Game/_VisionProtocol/Audio/SFX/NewSFX/dash.dash" _returnvalue_location (struct) 0.5 1.0 0.0 null null null null))))
    (`KismetSystemLibrary.Delay` 0.5)
    (`/Engine/EditorBlueprintResources/StandardMacros.IncrementInt` (`self.Bullet_I`)
      (:`  `
        (goto _label_2)))
    (else
      ;[1 1 1] Tylko dla wizualnego efektu. Czekamy na animacje.
      (`SceneComponent.K2_AddRelativeLocation` (`self.CapsuleComponent`) (0.0 0.0 -200.0) false false)
      (`KismetSystemLibrary.Delay` 1.0)
      (set `self.Bullet_I` 0)
      (`BTTask_BlueprintBase.FinishExecute` (`self.Task`) true))))

(event `ClearHitTable`
  (`KismetArrayLibrary.Array_Clear` (`self.HitTable`)))

(event `self.TailHitBox.OnComponentBeginOverlap`
  (params (OverlappedComponent :type "PrimitiveComponent Object Reference") (OtherActor :type "Actor Object Reference") (OtherComp :type "PrimitiveComponent Object Reference") (OtherBodyIndex :type Integer) (bFromSweep :type Boolean) (SweepResult :type "HitResult Structure (by ref)"))
  (bind _hittable (`self.HitTable`))
  (bind _asbp_vpplayer_character (cast `/Game/_VisionProtocol/Core/BP_VPPlayerCharacter` OtherActor))
  (if (not (`KismetArrayLibrary.Array_Contains` _hittable _asbp_vpplayer_character))
    (`KismetArrayLibrary.Array_AddUnique` _hittable _asbp_vpplayer_character)
    (`KismetSystemLibrary.K2_SetTimerDelegate` (`|CreateDelegate` :!event `ClearHitTable`) 1.0)
    (message `/Game/_VisionProtocol/Core/DMG-HP/BPI_Damageable.TakeDamage` OtherActor 25.0)
    (`RadialForceComponent.FireImpulse` (`self.RadialForce`))))

(event `/Game/_VisionProtocol/Core/AI/BPI_Enemy.SpecialAttack3`
  (bind _returnvalue (`self.K2_GetActorLocation`))
  (bind _returnvalue_x (`KismetMathLibrary.BreakVector` (`SceneComponent.K2_GetComponentScale` (`self.Mesh`))))
  (bind _returnvalue_2 (+ (* (`KismetMathLibrary.Normal` (- (`BlackboardComponent.GetValueAsVector` (`AIBlueprintHelperLibrary.GetBlackboard` null) "Location") _returnvalue)) 400.0) _returnvalue))
  (`GameplayStatics.PlaySoundAtLocation` "/Game/_VisionProtocol/Audio/SFX/NewSFX/biegSmoka.biegSmoka" (`self.K2_GetActorLocation`) (struct) 1.0 1.0 0.0 null null null null)
  (`|AIMoveTo` self (`BlackboardComponent.GetValueAsVector` (`AIBlueprintHelperLibrary.GetBlackboard` null) "Location") null 100.0
    (:`then`
      (bind (_outhit _returnvalue_3) (`KismetSystemLibrary.SphereTraceSingleForObjects` :`Start` _returnvalue_2 :`End` _returnvalue_2 :`Radius` (* _returnvalue_x 150.0) :`ObjectTypes` (`|MakeArray` "ObjectTypeQuery9" :!type "EObjectTypeQuery Enum") :`DrawDebugType` "ForDuration" :!label _label_3))
      (if _returnvalue_3
        (`RadialForceComponent.FireImpulse` (`self.RadialForce`))
        (`/Engine/EditorBlueprintResources/StandardMacros.DoOnce` false :!label _label_4
          (:`Completed`
            (message `/Game/_VisionProtocol/Core/DMG-HP/BPI_Damageable.TakeDamage` (`.HitActor` (`GameplayStatics.BreakHitResult` _outhit)) 35.0)
            (`GameplayStatics.PlaySoundAtLocation` "/Game/_VisionProtocol/Audio/SFX/NewSFX/smok_gryz.smok_gryz" (`self.K2_GetActorLocation`) (struct) 1.0 1.0 0.0 null null null null))))
      (`KismetSystemLibrary.Delay` 0.1)
      (if (`BlueprintGameplayTagLibrary.HasAnyTags` (`self.GTC`) (`BlueprintGameplayTagLibrary.MakeLiteralGameplayTagContainer` (struct :`GameplayTags` (struct :`(TagName` "Dragons.Urojony.StateZero") :`(TagName` "Dragons.Attack.RushAttack")))))
        (goto _label_3)))
    (:`OnSuccess`
      (`BTTask_BlueprintBase.FinishExecute` (`self.Task`) true :!label _label_5)
      (goto _label_4 :!via `Reset`))
    (:`OnFail`
      (goto _label_5))))

(event `Start`
  (bind _elevatorref (`self.ElevatorRef`))
  (`/Engine/EditorBlueprintResources/StandardMacros.IsValid` _elevatorref
    (:`Is Valid`
      (`/Game/_VisionProtocol/Objects/BP_ElevatorPlatform.ActivateMovement` _elevatorref null)
      (`SceneComponent.SetHiddenInGame` (`self.Mesh`) false false)
      (`ActorComponent.K2_DestroyComponent` (`self.StartTrigger`)))))

(event `self.PillarChecker.OnComponentBeginOverlap`
  (params (OverlappedComponent :type "PrimitiveComponent Object Reference") (OtherActor :type "Actor Object Reference") (OtherComp :type "PrimitiveComponent Object Reference") (OtherBodyIndex :type Integer) (bFromSweep :type Boolean) (SweepResult :type "HitResult Structure (by ref)"))
  (bind _gtc (`self.GTC`))
  (if (`self.ActorHasTag` OtherActor "Pillar")
    (if (`BlueprintGameplayTagLibrary.HasTag` (`self.GTC`) (struct :`TagName` "Dragons.Attack.RushAttack"))
      (`BlueprintGameplayTagLibrary.AddGameplayTag` (`self.GTC`) (struct :`TagName` "Dragons.State.Stun"))
      (`self.TakeDamage` 0.0)
      (`BlueprintGameplayTagLibrary.RemoveGameplayTag` (`self.GTC`) (struct :`TagName` "Dragons.Attack.RushAttack"))
      (message `/Game/_VisionProtocol/TestingPlayground/Filip/Urojony_Smok/BT/BPI_Urojony.SwitchFunction` OtherActor "None" null 150.0)
      (`MovementComponent.StopMovementImmediately` (`self.CharacterMovement`))
      (`BlueprintGameplayTagLibrary.RemoveGameplayTag` (`self.GTC`) (struct :`TagName` "Dragons.State.Moving"))
      (`KismetSystemLibrary.Delay` 5.0)
      (`BlueprintGameplayTagLibrary.AddGameplayTag` _gtc (struct :`TagName` "Dragons.Attack.WindAttack"))
      (`BlueprintGameplayTagLibrary.RemoveGameplayTag` _gtc (struct :`TagName` "Dragons.Urojony.StateZero"))
      (`BlueprintGameplayTagLibrary.RemoveGameplayTag` _gtc (struct :`TagName` "Dragons.State.Stun")))))

(fn `GetGTC`
  (returns (Container :type "GameplayTagContainer Structure"))
  (return))

(fn `GetIdealRange`
  (returns (AttackRadius :type "Float (double-precision)") (DefenseRadius :type "Float (double-precision)"))
  (bind _returnvalue_x (`KismetMathLibrary.BreakVector` (`SceneComponent.K2_GetComponentScale` (`self.Mesh`))))
  (return 0.0 (* _returnvalue_x 375.0)))

(fn `GetLocationPoint`
  (returns (Location :type "Vector Structure"))
  (bind _staticaofpl (`self.StaticAOFPL`))
  (if (not (`BlueprintGameplayTagLibrary.HasTag` (`self.GTC`) (struct :`TagName` "Dragons.State.Moving")))
    (return (`|GetArrayItem` (`self.StaticAOFPL`) (`KismetMathLibrary.RandomIntegerInRange` 0 (- (`KismetArrayLibrary.Array_Length` (`self.StaticAOFPL`)) 2))))
    (else
      (return (`|GetArrayItem` _staticaofpl (- (`KismetArrayLibrary.Array_Length` _staticaofpl) 1))))))

(fn `SetMovementSpeed`
  (params (Speed :type "/Game/_VisionProtocol/Core/AI/Enums/E_MovementSpeed Enum" :default "NewEnumerator0"))
  (returns (SpeedValue :type "Float (double-precision)"))
  (bind _returnvalue_x (`KismetMathLibrary.BreakVector` (`SceneComponent.K2_GetComponentScale` (`self.Mesh`))))
  (bind _output_get (set `CharacterMovementComponent.MaxFlySpeed` (select `/Game/_VisionProtocol/Core/AI/Enums/E_MovementSpeed` Speed :`NewEnumerator1` 100.0 :`NewEnumerator2` 250.0 :`NewEnumerator3` 500.0 :`NewEnumerator4` 800.0 :`NewEnumerator5` (* _returnvalue_x 1800.0)) (`self.CharacterMovement`)))
  (return _output_get))

(fn `TakeDamage`
  (params (Amount :type "Float (double-precision)"))
  (returns (`Was Damaged` :type Boolean))
  (bind _c_dmg_hp (`self.C_DMG-HP`))
  (bind _c_dmg_hp_2 (`self.C_DMG-HP`))
  (bind _gtc (`self.GTC`))
  (if (== Amount 0.0)
    (bind _was_damaged (`/Game/_VisionProtocol/Core/DMG-HP/C_DMG-HP.TakeDamage` _c_dmg_hp (/ (`/Game/_VisionProtocol/Core/DMG-HP/C_DMG-HP.MaximumHealth` _c_dmg_hp) 6.0)))
    (return _was_damaged)
    (elif (`BlueprintGameplayTagLibrary.HasTag` (`self.GTC`) (struct :`TagName` "Dragons.State.Invincible"))
      (return false)
      (else
        (bind _was_damaged_2 (`/Game/_VisionProtocol/Core/DMG-HP/C_DMG-HP.TakeDamage` _c_dmg_hp_2 (/ (`/Game/_VisionProtocol/Core/DMG-HP/C_DMG-HP.MaximumHealth` _c_dmg_hp_2) 6.0)))
        (`RadialForceComponent.FireImpulse` (`self.RadialForce`))
        (`BlueprintGameplayTagLibrary.AddGameplayTag` (`self.GTC`) (struct :`TagName` "Dragons.State.Invincible"))
        (`BlueprintGameplayTagLibrary.RemoveGameplayTag` _gtc (struct :`TagName` "Dragons.State.Moving"))
        (`BlueprintGameplayTagLibrary.AddGameplayTag` _gtc (struct :`TagName` "Dragons.Attack.WindAttack"))
        (`BlueprintGameplayTagLibrary.RemoveGameplayTag` _gtc (struct :`TagName` "Dragons.State.Stun"))
        (return _was_damaged_2)))))

(fn `UserConstructionScript`
  (bind _c_dmg_hp (`self.C_DMG-HP`))
  (`parent.UserConstructionScript`)
  (bind _output_get (set `/Game/_VisionProtocol/Core/DMG-HP/C_DMG-HP.MaximumHealth` 1200.0 _c_dmg_hp))
  (set `/Game/_VisionProtocol/Core/DMG-HP/C_DMG-HP.CurrentHealth` _output_get _c_dmg_hp)
  (add `/Game/_VisionProtocol/Core/DMG-HP/C_DMG-HP.OnDeath` _c_dmg_hp (`|CreateDelegate` :!event `Death`)))
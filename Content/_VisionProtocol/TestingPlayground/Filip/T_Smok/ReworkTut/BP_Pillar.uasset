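; Neon pillar actor that jitters and then sinks downward when its SwitchFunction event fires.
; BeginPlay creates a red dynamic instance of MI_NeonPillar.
; SwitchFunction passes that material to Niagara and sets its jitter, then after a delay plays the Ruined timeline, which lowers the actor a fixed step per update, so descent depends on frame rate.
; GetInteractionName and GetGTC are empty stubs.
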(event `self.ReceiveBeginPlay`
  (bind _returnvalue (`KismetMaterialLibrary.CreateDynamicMaterialInstance` "/Game/_VisionProtocol/TestingPlayground/Filip/T_Smok/ReworkTut/MI_NeonPillar.MI_NeonPillar"))
  (bind _output_get (set `self.Material` _returnvalue))
  (`MaterialInstanceDynamic.SetVectorParameterValue` _returnvalue "Color" (struct :`R` 1.0 :`A` 1.0))
  (`MaterialInstanceDynamic.SetVectorParameterValue` _output_get "Color" (struct :`R` 1.0 :`A` 1.0)))

(event `/Game/_VisionProtocol/TestingPlayground/Filip/Urojony_Smok/BT/BPI_Urojony.SwitchFunction`
  (params (`Event Name` :type Name) (Task :type "BTTask_BlueprintBase Object Reference") (RotationSpeed :type "Float (double-precision)"))
  (bind _niagara (`self.Niagara`))
  (`NiagaraComponent.SetVariableMaterial` _niagara "NeonColor" (`self.Material`))
  (`FXSystemComponent.SetFloatParameter` _niagara "Jitter" 5.0)
  (`KismetSystemLibrary.Delay` 2.0)
  (`Timeline|Ruined` :!via `PlayFromStart`
    (:`Update`
      (`self.K2_AddActorWorldTransform` (`KismetMathLibrary.MakeTransform` (0.0 0.0 -20.0))))))

(fn `GetGTC`
  (returns (Container :type "GameplayTagContainer Structure"))
  (return))

(fn `GetInteractionName`
  (returns (InteractionName :type Text))
  (return ""))

(fn `UserConstructionScript`)
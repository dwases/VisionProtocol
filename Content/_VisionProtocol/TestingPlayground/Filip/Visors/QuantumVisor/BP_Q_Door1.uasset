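; Quantum visor door that changes its look and pawn collision with the player's visor and its own QHidden state.
; BeginPlay applies QHidden and binds to the player visor component's quantum activation and deactivation events.
; Activation applies a fluctuating overlay via dynamic material and lets pawns through; deactivation either hides the door or restores its cached material and blocking.
; Refresh retunes overlay parameters, visibility and collision from QHidden; the interaction name is "QUANTUM".
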(event `Refresh`
  (bind _dynamic_ref (`self.Dynamic Ref`))
  (bind _dynamic_ref_2 (`self.Dynamic Ref`))
  (if (`/Game/_VisionProtocol/TestingPlayground/Filip/Visors/C_Visors.Q_Hidden` (`self.C_Visors`))
    (`MaterialInstanceDynamic.SetScalarParameterValue` _dynamic_ref_2 "OverlayLuminance" 150.0)
    (`MaterialInstanceDynamic.SetScalarParameterValue` _dynamic_ref_2 "FresnelExponent" 15.0)
    (`MaterialInstanceDynamic.SetScalarParameterValue` _dynamic_ref_2 "FresnelBaseReflectFractionIn" 0.002)
    (`SceneComponent.SetVisibility` (`self.Door`) (`/Game/_VisionProtocol/TestingPlayground/Filip/Visors/C_Visors.Q_Hidden` (`self.C_Visors`)) false)
    (`PrimitiveComponent.SetCollisionResponseToChannel` (`self.Door`) "ECC_Pawn" "ECR_Ignore")
    (`KismetSystemLibrary.PrintString` "Hide")
    (else
      (`MaterialInstanceDynamic.SetScalarParameterValue` _dynamic_ref "OverlayLuminance" 300.0)
      (`MaterialInstanceDynamic.SetScalarParameterValue` _dynamic_ref "FresnelExponent" 0.0)
      (`MaterialInstanceDynamic.SetScalarParameterValue` _dynamic_ref "FresnelBaseReflectFractionIn" 0.01)
      (`SceneComponent.SetVisibility` (`self.Door`) (not (`/Game/_VisionProtocol/TestingPlayground/Filip/Visors/C_Visors.Q_Hidden` (`self.C_Visors`))) false)
      (`PrimitiveComponent.SetCollisionResponseToChannel` (`self.Door`) "ECC_Pawn" "ECR_Block")
      (`KismetSystemLibrary.PrintString` "Unhide"))))

(event `self.ReceiveBeginPlay`
  (`SceneComponent.SetVisibility` (`self.Door`) (not (`/Game/_VisionProtocol/TestingPlayground/Filip/Visors/C_Visors.Q_Hidden` (`self.C_Visors`))) false)
  (bind _asbp_vpplayer_character (cast `/Game/_VisionProtocol/Core/BP_VPPlayerCharacter` (`GameplayStatics.GetPlayerCharacter` 0)))
  (bind _output_get (set `self.Player_VIsor` (`/Game/_VisionProtocol/Core/BP_VPPlayerCharacter.C_Visors` _asbp_vpplayer_character)))
  (add `/Game/_VisionProtocol/TestingPlayground/Filip/Visors/C_Visors.OnQActivation` _output_get (`|CreateDelegate` :!event `Q Activated`))
  (add `/Game/_VisionProtocol/TestingPlayground/Filip/Visors/C_Visors.OnQDeactivation` _output_get (`|CreateDelegate` :!event `Q Deactivation`))
  (if (`/Game/_VisionProtocol/TestingPlayground/Filip/Visors/C_Visors.Q_Hidden` (`self.C_Visors`))
    (`PrimitiveComponent.SetCollisionResponseToChannel` (`self.Door`) "ECC_Pawn" "ECR_Ignore")
    (`PrimitiveComponent.SetCollisionResponseToChannel` (`self.Door`) "ECC_Visibility" "ECR_Ignore")))

(event `Q Activated`
  (`KismetSystemLibrary.PrintString` "Activated")
  (bind _returnvalue (`PrimitiveComponent.CreateDynamicMaterialInstance` (`self.Door`) 0 "/Game/_VisionProtocol/TechArt/OverlayMaterials/MI_QuantumvisorFluctuateOverlay.MI_QuantumvisorFluctuateOverlay" "None"))
  (bind _output_get (set `self.Dynamic Ref` _returnvalue))
  (`MaterialInstanceDynamic.SetScalarParameterValue` _output_get "OverlayLuminance" 150.0)
  (`MaterialInstanceDynamic.SetScalarParameterValue` _output_get "FresnelExponent" 15.0)
  (`MaterialInstanceDynamic.SetScalarParameterValue` _output_get "FresnelBaseReflectFractionIn" 0.002)
  (`PrimitiveComponent.SetCollisionResponseToChannel` (`self.Door`) "ECC_Pawn" "ECR_Ignore"))

(event `Q Deactivation`
  (`KismetSystemLibrary.PrintString` "Deactivated")
  (if (`/Game/_VisionProtocol/TestingPlayground/Filip/Visors/C_Visors.Q_Hidden` (`self.C_Visors`))
    (`SceneComponent.SetVisibility` (`self.Door`) (not (`/Game/_VisionProtocol/TestingPlayground/Filip/Visors/C_Visors.Q_Hidden` (`self.C_Visors`))) false)
    (`PrimitiveComponent.SetCollisionResponseToChannel` (`self.Door`) "ECC_Visibility" "ECR_Ignore")
    (else
      (`PrimitiveComponent.SetMaterial` (`self.Door`) 0 (`self.BaseMaterial`))
      (`PrimitiveComponent.SetCollisionResponseToChannel` (`self.Door`) "ECC_Pawn" "ECR_Block"))))

(fn `GetInteractionName`
  (returns (InteractionName :type Text))
  (return "QUANTUM"))

(fn `UserConstructionScript`
  (set `self.BaseMaterial` (`PrimitiveComponent.GetMaterial` (`self.Door`) 0)))
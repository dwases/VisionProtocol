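; Quantum-visor world object whose visibility, Pawn collision and overlay material respond to the player's Quantum visor.
; It binds to the player visor's activation and deactivation events, applying a dynamic fluctuating overlay and restoring the base material on visible objects.
; Interactable objects reveal themselves when hidden and let Interact toggle their persistent QHidden state while the visor is active.
; Non-interactable objects temporarily invert: hidden ones become solid, visible ones become passable.
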(event `Refresh`
  (bind _dynamic_ref (`self.Dynamic Ref`))
  (bind _dynamic_ref_2 (`self.Dynamic Ref`))
  (if (`/Game/_VisionProtocol/TestingPlayground/Filip/Visors/C_Visors.Q_Hidden` (`self.C_Visors`))
    (`MaterialInstanceDynamic.SetScalarParameterValue` _dynamic_ref_2 "OverlayLuminance" 150.0)
    (`MaterialInstanceDynamic.SetScalarParameterValue` _dynamic_ref_2 "FresnelExponent" 15.0)
    (`MaterialInstanceDynamic.SetScalarParameterValue` _dynamic_ref_2 "FresnelBaseReflectFractionIn" 0.002)
    (`self.SetActorHiddenInGame` (not (`/Game/_VisionProtocol/TestingPlayground/Filip/Visors/C_Visors.Q_Hidden` (`self.C_Visors`))))
    (`PrimitiveComponent.SetCollisionResponseToChannel` (`self.StaticMesh`) "ECC_Pawn" "ECR_Ignore")
    (else
      (`MaterialInstanceDynamic.SetScalarParameterValue` _dynamic_ref "OverlayLuminance" 300.0)
      (`MaterialInstanceDynamic.SetScalarParameterValue` _dynamic_ref "FresnelExponent" 0.0)
      (`MaterialInstanceDynamic.SetScalarParameterValue` _dynamic_ref "FresnelBaseReflectFractionIn" 0.01)
      (`self.SetActorHiddenInGame` (`/Game/_VisionProtocol/TestingPlayground/Filip/Visors/C_Visors.Q_Hidden` (`self.C_Visors`)))
      (`PrimitiveComponent.SetCollisionResponseToChannel` (`self.StaticMesh`) "ECC_Pawn" "ECR_Block"))))

(event `self.ReceiveBeginPlay`
  (`self.SetActorHiddenInGame` (`/Game/_VisionProtocol/TestingPlayground/Filip/Visors/C_Visors.Q_Hidden` (`self.C_Visors`)))
  (bind _asbp_vpplayer_character (cast `/Game/_VisionProtocol/Core/BP_VPPlayerCharacter` (`GameplayStatics.GetPlayerCharacter` 0)))
  (bind _output_get (set `self.Player_VIsor` (`/Game/_VisionProtocol/Core/BP_VPPlayerCharacter.C_Visors` _asbp_vpplayer_character)))
  (add `/Game/_VisionProtocol/TestingPlayground/Filip/Visors/C_Visors.OnQActivation` _output_get (`|CreateDelegate` :!event `Q Activated`))
  (add `/Game/_VisionProtocol/TestingPlayground/Filip/Visors/C_Visors.OnQDeactivation` _output_get (`|CreateDelegate` :!event `Q Deactivation`))
  (if (`/Game/_VisionProtocol/TestingPlayground/Filip/Visors/C_Visors.Q_Hidden` (`self.C_Visors`))
    (`PrimitiveComponent.SetCollisionResponseToChannel` (`self.StaticMesh`) "ECC_Pawn" "ECR_Ignore")
    (`PrimitiveComponent.SetCollisionResponseToChannel` (`self.StaticMesh`) "ECC_Visibility" "ECR_Ignore")))

(event `/Game/_VisionProtocol/Core/InteractionFramework/BPI_Interactable.Interact`
  (params (Interactor :type "Actor Object Reference") (InteracteeComponent :type "PrimitiveComponent Object Reference"))
  (bind _c_visors (`self.C_Visors`))
  (if (`self.Q_Interactable`)
    (if (`/Game/_VisionProtocol/TestingPlayground/Filip/Visors/C_Visors.Q_Active` (`self.Player_VIsor`))
      (set `/Game/_VisionProtocol/TestingPlayground/Filip/Visors/C_Visors.Q_Hidden` (not (`/Game/_VisionProtocol/TestingPlayground/Filip/Visors/C_Visors.Q_Hidden` _c_visors)) _c_visors)
      (`self.Refresh`))))

(event `Q Activated`
  (bind _q_hidden (`/Game/_VisionProtocol/TestingPlayground/Filip/Visors/C_Visors.Q_Hidden` (`self.C_Visors`)))
  (if (`self.Q_Interactable`)
    (set `self.Q_Hide` false)
    (bind _returnvalue (`PrimitiveComponent.CreateDynamicMaterialInstance` (`self.StaticMesh`) 0 "/Game/_VisionProtocol/TechArt/OverlayMaterials/MI_QuantumvisorFluctuateOverlay.MI_QuantumvisorFluctuateOverlay" "None"))
    (bind _output_get (set `self.Dynamic Ref` _returnvalue))
    (if (`/Game/_VisionProtocol/TestingPlayground/Filip/Visors/C_Visors.Q_Hidden` (`self.C_Visors`))
      (`MaterialInstanceDynamic.SetScalarParameterValue` _output_get "OverlayLuminance" 150.0)
      (`MaterialInstanceDynamic.SetScalarParameterValue` _output_get "FresnelExponent" 15.0)
      (`MaterialInstanceDynamic.SetScalarParameterValue` _output_get "FresnelBaseReflectFractionIn" 0.002)
      (`self.SetActorHiddenInGame` (not (`/Game/_VisionProtocol/TestingPlayground/Filip/Visors/C_Visors.Q_Hidden` (`self.C_Visors`))))
      (`PrimitiveComponent.SetCollisionResponseToChannel` (`self.StaticMesh`) "ECC_Visibility" "ECR_Block"))
    (else
      (bind _returnvalue_2 (`PrimitiveComponent.CreateDynamicMaterialInstance` (`self.StaticMesh`) 0 "/Game/_VisionProtocol/TechArt/OverlayMaterials/MI_QuantumvisorFluctuateOverlay.MI_QuantumvisorFluctuateOverlay" "None"))
      (bind _output_get_2 (set `self.Dynamic Ref` _returnvalue_2))
      (if _q_hidden
        (`self.SetActorHiddenInGame` (not _q_hidden))
        (`PrimitiveComponent.SetCollisionResponseToChannel` (`self.StaticMesh`) "ECC_Pawn" "ECR_Block")
        (else
          (`MaterialInstanceDynamic.SetScalarParameterValue` _output_get_2 "OverlayLuminance" 150.0)
          (`MaterialInstanceDynamic.SetScalarParameterValue` _output_get_2 "FresnelExponent" 15.0)
          (`MaterialInstanceDynamic.SetScalarParameterValue` _output_get_2 "FresnelBaseReflectFractionIn" 0.002)
          (`PrimitiveComponent.SetCollisionResponseToChannel` (`self.StaticMesh`) "ECC_Pawn" "ECR_Ignore"))))))

(event `Q Deactivation`
  (bind _staticmesh (`self.StaticMesh`))
  (bind _q_hidden (`/Game/_VisionProtocol/TestingPlayground/Filip/Visors/C_Visors.Q_Hidden` (`self.C_Visors`)))
  (if (`self.Q_Interactable`)
    (set `self.Q_Hide` true)
    (if _q_hidden
      (`self.SetActorHiddenInGame` _q_hidden)
      (`PrimitiveComponent.SetCollisionResponseToChannel` (`self.StaticMesh`) "ECC_Visibility" "ECR_Ignore")
      (else
        (`PrimitiveComponent.SetMaterial` (`self.StaticMesh`) 0 (`self.BaseMaterial`))))
    (elif (`/Game/_VisionProtocol/TestingPlayground/Filip/Visors/C_Visors.Q_Hidden` (`self.C_Visors`))
      (`self.SetActorHiddenInGame` (`/Game/_VisionProtocol/TestingPlayground/Filip/Visors/C_Visors.Q_Hidden` (`self.C_Visors`)))
      (`PrimitiveComponent.SetCollisionResponseToChannel` _staticmesh "ECC_Pawn" "ECR_Ignore")
      (else
        (`PrimitiveComponent.SetMaterial` (`self.StaticMesh`) 0 (`self.BaseMaterial`))
        (`PrimitiveComponent.SetCollisionResponseToChannel` _staticmesh "ECC_Pawn" "ECR_Block")))))

(fn `GetInteractionName`
  (returns (InteractionName :type Text))
  (return "QUANTUM"))

(fn `UserConstructionScript`
  (set `self.BaseMaterial` (`PrimitiveComponent.GetMaterial` (`self.StaticMesh`) 0))
  (set `self.Q_Hide` true))
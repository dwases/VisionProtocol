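; BP_EnemyBase is an AI enemy character that provides health, movement speed, patrol route and combat range functions.
; A CDMGHP component handles damage, healing and death state, with health filled on BeginPlay if an AIC_Enemy controller is present.
; Its OnDeath event ragdolls the mesh, stops the controller's brain logic, disables capsule collision, then destroys the actor after a short delay.
; Movement speed maps named tiers to CharacterMovement walk speeds.
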(event `self.ReceiveBeginPlay`
  (bind _c_dmg_hp (`self.C_DMG-HP`))
  (bind _asaic_enemy (cast `/Game/_VisionProtocol/TestingPlayground/Filip/AI/AIC_Enemy` (`AIBlueprintHelperLibrary.GetAIController` self)))
  (set `self.AIC Enemy` _asaic_enemy)
  (add `/Game/_VisionProtocol/Core/DMG-HP/C_DMG-HP.OnDeath` _c_dmg_hp (`|CreateDelegate` :!event `Event On Death`))
  (bind _output_get (set `/Game/_VisionProtocol/Core/DMG-HP/C_DMG-HP.MaximumHealth` 100.0 _c_dmg_hp))
  (set `/Game/_VisionProtocol/Core/DMG-HP/C_DMG-HP.CurrentHealth` _output_get _c_dmg_hp))

(event `Event On Death`
  (bind _mesh (`self.Mesh`))
  (`PrimitiveComponent.SetSimulatePhysics` _mesh true)
  (`PrimitiveComponent.SetCollisionEnabled` _mesh "PhysicsOnly")
  (`BrainComponent.StopLogic` (`AIController.BrainComponent` (`self.AIC Enemy`)) "")
  (`PrimitiveComponent.SetCollisionEnabled` (`self.CapsuleComponent`) "NoCollision")
  (`KismetSystemLibrary.Delay` 2.0)
  (`self.K2_DestroyActor`))

(fn `GetCurrentHealth`
  (returns (Health :type "Float (double-precision)"))
  (return (`/Game/_VisionProtocol/Core/DMG-HP/C_DMG-HP.CurrentHealth` (`self.C_DMG-HP`))))

(fn `GetIdealRange`
  (returns (AttackRadius :type "Float (double-precision)") (DefenseRadius :type "Float (double-precision)"))
  (return 20.0 400.0))

(fn `GetMaxHealth`
  (returns (MaxHealth :type "Float (double-precision)"))
  (return (`/Game/_VisionProtocol/Core/DMG-HP/C_DMG-HP.MaximumHealth` (`self.C_DMG-HP`))))

(fn `GetPatrolRoute`
  (returns (PatrolRoute :type "/Game/_VisionProtocol/TestingPlayground/Filip/AI/BP_PatrolPath1 Object Reference"))
  (return (`self.Patrol Route`)))

(fn `Heal`
  (params (HP_Amount :type "Float (double-precision)"))
  (returns (`New Health` :type "Float (double-precision)"))
  (bind _new_health (`/Game/_VisionProtocol/Core/DMG-HP/C_DMG-HP.Heal` (`self.C_DMG-HP`) HP_Amount))
  (return _new_health))

(fn `IsDead`
  (returns (Dead :type Boolean))
  (return (`/Game/_VisionProtocol/Core/DMG-HP/C_DMG-HP.isDead` (`self.C_DMG-HP`))))

(fn `SetMovementSpeed`
  (params (Speed :type "/Game/_VisionProtocol/TestingPlayground/Filip/AI/Enums/E_MovementSpeed Enum" :default "NewEnumerator0"))
  (returns (SpeedValue :type "Float (double-precision)"))
  (bind _output_get (set `CharacterMovementComponent.MaxWalkSpeed` (select `/Game/_VisionProtocol/TestingPlayground/Filip/AI/Enums/E_MovementSpeed` Speed :`NewEnumerator1` 50.0 :`NewEnumerator2` 125.0 :`NewEnumerator3` 350.0 :`NewEnumerator4` 500.0 :`NewEnumerator5` 700.0 :!type "Float (single-precision)") (`self.CharacterMovement`)))
  (return _output_get))

(fn `TakeDamage`
  (params (Amount :type "Float (double-precision)"))
  (returns (`Was Damaged` :type Boolean))
  (bind _was_damaged (`/Game/_VisionProtocol/Core/DMG-HP/C_DMG-HP.TakeDamage` (`self.C_DMG-HP`) Amount))
  (return _was_damaged))

(fn `UserConstructionScript`)
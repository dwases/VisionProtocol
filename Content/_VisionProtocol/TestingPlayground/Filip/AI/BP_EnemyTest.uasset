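; BP_EnemyTest is a test enemy character with a melee attack, exposing getters and setters for AI range, speed and patrol route.
; Attack1 runs a debug-drawn sphere trace just ahead for pawns, then sends a damage message to the hit actor and prints it.
; Damage, healing, health and death queries forward to the CDMGHP component.
; SetMovementSpeed maps speed tiers to walk speed, while GetIdealRange returns fixed attack and defense radii.
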(event `self.ReceiveBeginPlay`
  (`parent.ReceiveBeginPlay`))

(event `/Game/_VisionProtocol/TestingPlayground/Filip/AI/BPI_Enemy.Attack1`
  (bind _returnvalue (`self.K2_GetActorLocation`))
  (bind (_outhit _returnvalue_2) (`KismetSystemLibrary.SphereTraceSingleForObjects` :`Start` _returnvalue :`End` (+ _returnvalue (* (`self.GetActorForwardVector`) 100.0)) :`Radius` 150.0 :`ObjectTypes` (`|MakeArray` "ObjectTypeQuery3" :!type "EObjectTypeQuery Enum") :`DrawDebugType` "ForDuration" :`DrawTime` 2.0))
  (if _returnvalue_2
    (bind (_bblockinghit _binitialoverlap _time _distance _location _impactpoint _normal _impactnormal _physmat _hitactor) (`GameplayStatics.BreakHitResult` _outhit))
    (message `/Game/_VisionProtocol/Core/DMG-HP/BPI_Damageable.TakeDamage` _hitactor 10.0)
    (`KismetSystemLibrary.PrintString` (`KismetStringLibrary.Conv_ObjectToString` _hitactor))))

(fn `GetCurrentHealth`
  (returns (Health :type "Float (double-precision)"))
  (return (`/Game/_VisionProtocol/Core/DMG-HP/C_DMG-HP.CurrentHealth` (`self.C_DMG-HP`))))

(fn `GetIdealRange`
  (returns (AttackRadius :type "Float (double-precision)") (DefenseRadius :type "Float (double-precision)"))
  (return 80.0 400.0))

(fn `GetMaxHealth`
  (returns (MaxHealth :type "Float (double-precision)"))
  (return (`/Game/_VisionProtocol/Core/DMG-HP/C_DMG-HP.MaximumHealth` (`self.C_DMG-HP`))))

(fn `GetPatrolRoute`
  (returns (PatrolRoute :type "/Game/_VisionProtocol/TestingPlayground/Filip/AI/BP_PatrolPath1 Object Reference"))
  (return (`self.Patrol Route`)))

(fn `Heal`
  (params (HP_Amount :type "Float (double-precision)"))
  (returns (`New Health` :type "Float (double-precision)"))
  (bind _new_health (`/Game/_VisionProtocol/Core/DMG-HP/C_DMG-HP.Heal` (`self.C_DMG-HP`) HP_Amount))
  (return _new_health))

(fn `IsDead`
  (returns (Dead :type Boolean))
  (return (`/Game/_VisionProtocol/Core/DMG-HP/C_DMG-HP.isDead` (`self.C_DMG-HP`))))

(fn `SetMovementSpeed`
  (params (Speed :type "/Game/_VisionProtocol/TestingPlayground/Filip/AI/Enums/E_MovementSpeed Enum" :default "NewEnumerator0"))
  (returns (SpeedValue :type "Float (double-precision)"))
  (bind _output_get (set `CharacterMovementComponent.MaxWalkSpeed` (select `/Game/_VisionProtocol/TestingPlayground/Filip/AI/Enums/E_MovementSpeed` Speed :`NewEnumerator1` 50.0 :`NewEnumerator2` 125.0 :`NewEnumerator3` 350.0 :`NewEnumerator4` 500.0 :`NewEnumerator5` 700.0 :!type "Float (single-precision)") (`self.CharacterMovement`)))
  (return _output_get))

(fn `TakeDamage`
  (params (Amount :type "Float (double-precision)"))
  (returns (`Was Damaged` :type Boolean))
  (bind _was_damaged (`/Game/_VisionProtocol/Core/DMG-HP/C_DMG-HP.TakeDamage` (`self.C_DMG-HP`) Amount))
  (return _was_damaged))

(fn `UserConstructionScript`
  (`parent.UserConstructionScript`))
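; BP_FloatingRockMain is a floating rock projectile that stays non-colliding until a named switch event hurls it at the player.
; FlyToPlayer enables overlaps and sets velocity and capsule rotation once toward the player's current position, without homing.
; A player overlap within the capsule's forward cone deals damage, applies upward-biased knockback and disables collision.
; Overlapping a "Floating"-tagged actor stops it after a short delay with an explosion sound.
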(event `FlyToPlayer`
  (bind _projectilemovement (`self.ProjectileMovement`))
  (bind _returnvalue (`self.K2_GetActorLocation` (`GameplayStatics.GetPlayerCharacter` 0)))
  (`PrimitiveComponent.SetCollisionResponseToAllChannels` (`self.CapsuleCollision`) "ECR_Overlap")
  (set `MovementComponent.Velocity` (* (`KismetMathLibrary.Normal` (- _returnvalue (`self.K2_GetActorLocation`))) (`ProjectileMovementComponent.InitialSpeed` _projectilemovement)) _projectilemovement)
  (`SceneComponent.K2_SetWorldRotation` (`self.CapsuleCollision`) (`KismetMathLibrary.MakeRotator` (.roll (`KismetMathLibrary.FindLookAtRotation` (`SceneComponent.K2_GetComponentLocation` (`self.CapsuleCollision`)) _returnvalue)) (.pitch (`KismetMathLibrary.FindLookAtRotation` (`SceneComponent.K2_GetComponentLocation` (`self.CapsuleCollision`)) _returnvalue)) (.yaw (`KismetMathLibrary.FindLookAtRotation` (`SceneComponent.K2_GetComponentLocation` (`self.CapsuleCollision`)) _returnvalue))) false false))

(event `/Game/_VisionProtocol/TestingPlayground/Filip/Urojony_Smok/BT/BPI_Urojony.SwitchFunction`
  (params (`Event Name` :type Name) (Task :type "BTTask_BlueprintBase Object Reference") (RotationSpeed :type "Float (double-precision)"))
  (switch `name` `Event Name`
    (:`FlyToPlayer`
      (`self.FlyToPlayer`))))

(event `self.ReceiveBeginPlay`
  (`PrimitiveComponent.SetCollisionResponseToAllChannels` (`self.CapsuleCollision`) "ECR_Ignore"))

(event `self.CapsuleCollision.OnComponentBeginOverlap`
  (params (OverlappedComponent :type "PrimitiveComponent Object Reference") (OtherActor :type "Actor Object Reference") (OtherComp :type "PrimitiveComponent Object Reference") (OtherBodyIndex :type Integer) (bFromSweep :type Boolean) (SweepResult :type "HitResult Structure (by ref)"))
  (bind _returnvalue (`GameplayStatics.GetPlayerCharacter` 0))
  (if (== OtherActor (`GameplayStatics.GetPlayerCharacter` 0))
    (if (> (`KismetMathLibrary.Dot_VectorVector` (`KismetMathLibrary.Normal` (- (`self.K2_GetActorLocation` (`GameplayStatics.GetPlayerCharacter` 0)) (`self.K2_GetActorLocation`))) (`SceneComponent.GetForwardVector` (`self.CapsuleCollision`))) 0.7)
      (message `/Game/_VisionProtocol/Core/DMG-HP/BPI_Damageable.TakeDamage` (`GameplayStatics.GetPlayerCharacter` 0) 50.0)
      (`PrimitiveComponent.SetCollisionResponseToAllChannels` (`self.CapsuleCollision`) "ECR_Ignore")
      (`Character.LaunchCharacter` _returnvalue (`KismetMathLibrary.MakeVector` (.x (* (`KismetMathLibrary.Normal` (- (`self.K2_GetActorLocation` _returnvalue) (`self.K2_GetActorLocation`))) 1200.0)) (.y (* (`KismetMathLibrary.Normal` (- (`self.K2_GetActorLocation` _returnvalue) (`self.K2_GetActorLocation`))) 1200.0)) (`KismetMathLibrary.FMax` (.z (* (`KismetMathLibrary.Normal` (- (`self.K2_GetActorLocation` _returnvalue) (`self.K2_GetActorLocation`))) 1200.0)) 400.0)) true true))
    (elif (`self.ActorHasTag` OtherActor "Floating")
      (`KismetSystemLibrary.Delay` 0.5) ; Może się bugować-góra sie przerwie przez delay
      (set `MovementComponent.Velocity` (0.0 0.0 0.0) (`self.ProjectileMovement`))
      (`GameplayStatics.PlaySoundAtLocation` "/Game/_VisionProtocol/Audio/SFX/explosion.explosion" (`self.K2_GetActorLocation`) (struct) 1.0 1.0 0.0 null null null null)
      (`PrimitiveComponent.SetCollisionResponseToAllChannels` (`self.CapsuleCollision`) "ECR_Ignore"))))

(fn `GetGTC`
  (returns (Container :type "GameplayTagContainer Structure"))
  (return))

(fn `UserConstructionScript`)
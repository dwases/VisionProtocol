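; Temporary mist line actor that stretches a damaging, blinding fog volume between itself and its owner, then destroys itself after a fixed lifetime.
; A looping timer scales the Niagara height and spawn rate, plus the damage box, with owner distance until MaxDistance is reached.
; Box overlaps toggle a second timer that sends damage messages and notify the overlapping actor of blindness changes.
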(event `Update`
  (bind _niagara (`self.Niagara`))
  (bind _returnvalue (`KismetMathLibrary.Vector_Distance` (`self.K2_GetActorLocation` (`self.GetOwner`)) (`self.K2_GetActorLocation`)))
  (bind _returnvalue_2 (/ _returnvalue 2.0))
  (if (< _returnvalue (`self.MaxDistance`))
    (`NiagaraComponent.SetVariableFloat` _niagara "Height" _returnvalue)
    (`NiagaraComponent.SetVariableFloat` _niagara "SpawnRate" (/ _returnvalue 20.0))
    (`BoxComponent.SetBoxExtent` (`self.DMG`) (`KismetMathLibrary.MakeVector` _returnvalue_2 450.0 450.0) true)
    (`SceneComponent.K2_SetRelativeLocation` (`self.DMG`) (`KismetMathLibrary.MakeVector` _returnvalue_2) false false)
    (else
      (`KismetSystemLibrary.K2_ClearAndInvalidateTimerHandle` (stale `self.ReceiveBeginPlay` _returnvalue)))))

(event `self.ReceiveBeginPlay`
  (bind _returnvalue (`KismetSystemLibrary.K2_SetTimerDelegate` (delegate `Update`) 0.1 true))
  (`KismetSystemLibrary.Delay` 30.0)
  (`self.K2_DestroyActor`))

(event `self.DMG.OnComponentEndOverlap`
  (params (OverlappedComponent :type "PrimitiveComponent Object Reference") (OtherActor :type "Actor Object Reference") (OtherComp :type "PrimitiveComponent Object Reference") (OtherBodyIndex :type Integer))
  (`KismetSystemLibrary.K2_ClearAndInvalidateTimerHandle` (stale `self.DMG.OnComponentBeginOverlap` _returnvalue))
  (message `/Game/_VisionProtocol/TestingPlayground/Filip/Urojony_Smok/BPI_ToPlayer.BlindnessZero` (stale `self.DMG.OnComponentBeginOverlap` OtherActor) true))

(event `self.DMG.OnComponentBeginOverlap`
  (params (OverlappedComponent :type "PrimitiveComponent Object Reference") (OtherActor :type "Actor Object Reference") (OtherComp :type "PrimitiveComponent Object Reference") (OtherBodyIndex :type Integer) (bFromSweep :type Boolean) (SweepResult :type "HitResult Structure (by ref)"))
  (bind _returnvalue (`KismetSystemLibrary.K2_SetTimer` null "MistDMG" 0.1 true))
  (message `/Game/_VisionProtocol/TestingPlayground/Filip/Urojony_Smok/BPI_ToPlayer.BlindnessZero` OtherActor false))

(event `MistDMG`
  (`/Engine/EditorBlueprintResources/StandardMacros.IsValid` (stale `self.DMG.OnComponentBeginOverlap` OtherActor)
    (:`Is Valid`
      (message `/Game/_VisionProtocol/Core/DMG-HP/BPI_Damageable.TakeDamage` (stale `self.DMG.OnComponentBeginOverlap` OtherActor) 0.5))))

(fn `UserConstructionScript`)
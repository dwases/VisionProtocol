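; Niagara mist hazard that damages and toggles a blindness effect on overlapping actors not tagged "Smok".
; Size parameters drive the particles and trigger box, while a looping timer damages the last entering actor until an overlap ends.
; In SpawnTentacle mode it spawns six smaller-sized mists along the axes and sphere-traces for a "FloatingActor" to send flying at the player.
; It self-destroys after a delay, unless Infinite outside that mode.
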(event `self.ReceiveBeginPlay`
  (bind _niagara (`self.Niagara`))
  (`FXSystemComponent.SetFloatParameter` _niagara "MinSize" (`self.MinSize`))
  (`FXSystemComponent.SetFloatParameter` _niagara "MaxSize" (`self.MaxSize`))
  (`BoxComponent.SetBoxExtent` (`self.DMGTrigger`) (`KismetMathLibrary.Conv_DoubleToVector` (/ (`self.MaxSize`) 4.0)) true)
  (if (`self.bSpawnTentacle`)
    (`self.SpawnTentacle`)
    (elif (not (`self.Infinite`))
      (`KismetSystemLibrary.Delay` 8.0)
      (`self.K2_DestroyActor`))))

(event `self.DMGTrigger.OnComponentEndOverlap`
  (params (OverlappedComponent :type "PrimitiveComponent Object Reference") (OtherActor :type "Actor Object Reference") (OtherComp :type "PrimitiveComponent Object Reference") (OtherBodyIndex :type Integer))
  (`KismetSystemLibrary.K2_ClearAndInvalidateTimerHandle` (stale `self.DMGTrigger.OnComponentBeginOverlap` _returnvalue))
  (message `/Game/_VisionProtocol/TestingPlayground/Filip/Urojony_Smok/BPI_ToPlayer.BlindnessZero` (`self.TargetActor`) true))

(event `self.DMGTrigger.OnComponentBeginOverlap`
  (params (OverlappedComponent :type "PrimitiveComponent Object Reference") (OtherActor :type "Actor Object Reference") (OtherComp :type "PrimitiveComponent Object Reference") (OtherBodyIndex :type Integer) (bFromSweep :type Boolean) (SweepResult :type "HitResult Structure (by ref)"))
  (if (not (`self.ActorHasTag` OtherActor "Smok"))
    (set `self.TargetActor` OtherActor)
    (bind _returnvalue (`KismetSystemLibrary.K2_SetTimer` null "MistDMG" 0.1 true))
    (message `/Game/_VisionProtocol/TestingPlayground/Filip/Urojony_Smok/BPI_ToPlayer.BlindnessZero` (`self.TargetActor`) false)))

(event `MistDMG`
  (bind _targetactor (`self.TargetActor`))
  (`/Engine/EditorBlueprintResources/StandardMacros.IsValid` _targetactor
    (:`Is Valid`
      (message `/Game/_VisionProtocol/Core/DMG-HP/BPI_Damageable.TakeDamage` _targetactor 0.5))))

(event `SpawnTentacle`
  (bind _returnvalue (`self.K2_GetActorLocation`))
  (for _array_element (`|MakeArray` (200.0 0.0 0.0) (-200.0 0.0 0.0) (0.0 200.0 0.0) (0.0 -200.0 0.0) (0.0 0.0 200.0) (0.0 0.0 -200.0) :!type "Vector Structure")
    (`|SpawnActorFromClass` "BP_NiagaraMist_C" (`KismetMathLibrary.MakeTransform` (+ _array_element (`self.K2_GetActorLocation`))) "AlwaysSpawn" "MultiplyWithRoot" null false false 200.0 350.0 null))
  (bind _outhits (`KismetSystemLibrary.SphereTraceMultiForObjects` _returnvalue _returnvalue 7500.0 (`|MakeArray` "ObjectTypeQuery1" "ObjectTypeQuery2" :!type "EObjectTypeQuery Enum")))
  (for _array_element_2 _outhits
    (bind (_bblockinghit _binitialoverlap _time _distance _location _impactpoint _normal _impactnormal _physmat _hitactor) (`GameplayStatics.BreakHitResult` _array_element_2))
    (if (`self.ActorHasTag` _hitactor "FloatingActor")
      (break)))
  (message `/Game/_VisionProtocol/TestingPlayground/Filip/Urojony_Smok/BT/BPI_Urojony.SwitchFunction` _hitactor "FlyToPlayer" null 150.0)
  (`KismetSystemLibrary.Delay` 8.0)
  (`self.K2_DestroyActor`))

(fn `UserConstructionScript`)
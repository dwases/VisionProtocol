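; Zerowy dragon boss: a flying, mist-trailing enemy with a health bar, run by behavior tree BT_Zerowy.
; SwitchFunction dispatches timeline-driven flights between data-asset points, mist tentacle and projectile attacks, and phase changes to flight and player grappling-hook speeds.
; Its rush attack teleports it to a random path point, then flies along a mist line to the next.
; Gameplay tags gate damage, hits briefly remove its grapple tag, and contact launches the player.
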(event `SpawnMistTentacle`
  (`|SpawnActorFromClass` "/Game/_VisionProtocol/TestingPlayground/Filip/Zerowy_Smok/BP_NiagaraMist.BP_NiagaraMist_C" (`KismetMathLibrary.MakeTransform` (`SceneComponent.K2_GetComponentLocation` (`self.NiagaraMistSpawn`))) "AlwaysSpawn" "MultiplyWithRoot" null true false 90.0 190.0 null))

(event `SpawnMistTail`
  (`|SpawnActorFromClass` "/Game/_VisionProtocol/TestingPlayground/Filip/Zerowy_Smok/BP_NiagaraMist.BP_NiagaraMist_C" (`KismetMathLibrary.MakeTransform` (`SceneComponent.K2_GetComponentLocation` (`self.NiagaraMistSpawn`))) "AlwaysSpawn" "MultiplyWithRoot" null false false 1000.0 2000.0 null))

(event `self.ReceiveBeginPlay`
  (bind _returnvalue (`AIBlueprintHelperLibrary.GetAIController` self))
  (`/Engine/EditorBlueprintResources/StandardMacros.IsValid` _returnvalue :!label _label
    (:`Is Valid`
      (`BlueprintGameplayTagLibrary.AddGameplayTag` (`self.GTC`) (struct :`TagName` "Dragons.Urojony.StateOne"))
      (`AIController.RunBehaviorTree` _returnvalue "/Game/_VisionProtocol/TestingPlayground/Filip/Zerowy_Smok/BT_Zerowy.BT_Zerowy")
      (bind _returnvalue_2 (`KismetSystemLibrary.K2_SetTimer` null "SpawnMistTail" 0.1 true))
      (set `self.Timer1` _returnvalue_2)
      (`self.Add HP Bar`)
      (message `/Game/_VisionProtocol/TestingPlayground/Filip/Urojony_Smok/BPI_ToPlayer.ZeroStart` (`GameplayStatics.GetPlayerCharacter` 0)))
    (:`Is Not Valid`
      (`KismetSystemLibrary.DelayUntilNextTick`)
      (goto _label))))

(event `Add HP Bar`
  (bind _returnvalue (`|CreateWidget` "/Game/_VisionProtocol/TestingPlayground/Filip/T_Smok/WBP_BossHealthBar.WBP_BossHealthBar_C" null self))
  (bind _output_get (set `self.HPBar` _returnvalue))
  (add `UserWidget.OnVisibilityChanged` _output_get (delegate `OnVisibilityChanged_Event`))
  (`UserWidget.AddToViewport` _output_get 0))

(event `/Game/_VisionProtocol/TestingPlayground/Filip/Urojony_Smok/BT/BPI_Urojony.SetPath`
  (params (`New Path` :type "/Game/_VisionProtocol/TestingPlayground/Filip/Urojony_Smok/DA_SmokUrojony_Locations_Fight Object Reference"))
  (set `self.DA Flight Locations` `New Path`))

(event `/Game/_VisionProtocol/TestingPlayground/Filip/Urojony_Smok/BT/BPI_Urojony.SetGTC`
  (params (GTC :type "GameplayTagContainer Structure"))
  (set `self.GTC` GTC))

(event `DisapearPointPart`
  (`|SpawnActorFromClass` "/Game/_VisionProtocol/TestingPlayground/Filip/Zerowy_Smok/BP_NiagaraMist.BP_NiagaraMist_C" (`KismetMathLibrary.MakeTransform` (`SceneComponent.K2_GetComponentLocation` (`self.DisapearPoint`))) "AlwaysSpawn" "MultiplyWithRoot" null false false 1800.0 3800.0 null))

(event `OnVisibilityChanged_Event`
  (params (InVisibility :type "ESlateVisibility Enum" :default "Visible"))
  (`Widget.RemoveFromParent` (stale `Add HP Bar` _output_get)))

(event `Move Completed`
  (`BlueprintGameplayTagLibrary.RemoveGameplayTag` (`self.GTC`) (struct :`TagName` "Dragons.State.Moving"))
  (bind _task (`self.Task`)
    (:`then`
      (`BTTask_BlueprintBase.FinishExecute` _task true))
    (:`else`)))

(event `FlyToNextPoint`
  (params (Task :type "BTTask_BlueprintBase Object Reference") (Taget :type "Actor Object Reference") (RotationSpeed :type "Float (double-precision)"))
  (bind _location_fight (`/Game/_VisionProtocol/TestingPlayground/Filip/Urojony_Smok/DA_SmokUrojony_Locations_Fight.Location_Fight` (`self.DA Flight Locations`)))
  (bind _output (`|GetArrayItem` _location_fight (`KismetMathLibrary.RandomIntegerInRange` 0 (- (`KismetArrayLibrary.Array_Length` _location_fight) 1))))
  (bind _output_get (set `self.Task` Task))
  (if (>= (`KismetMathLibrary.Vector_Distance` _output (`self.K2_GetActorLocation`)) 500.0)
    (`self.FlyAndRotateTo` _output Taget RotationSpeed)
    (else
      (`BTTask_BlueprintBase.FinishExecute` _output_get false))))

(event `RotateTo`
  (params (Location :type "Vector Structure") (Target :type "Actor Object Reference") (RotationAngleSpeed :type "Float (double-precision)" :default 150.0))
  (bind _returnvalue (`self.K2_GetActorLocation`))
  (bind (_returnvalue_roll _returnvalue_pitch _returnvalue_yaw) (`KismetMathLibrary.BreakRotator` (`self.K2_GetActorRotation`)))
  (bind (_finalrotation_roll _finalrotation_pitch _finalrotation_yaw) (`KismetMathLibrary.BreakRotator` (`self.FinalRotation`)))
  (set `self.SavedRotation` (`self.K2_GetActorRotation`))
  (`/Engine/EditorBlueprintResources/StandardMacros.IsValid` Target
    (:`Is Valid`
      (set `self.FinalRotation` (`KismetMathLibrary.FindLookAtRotation` _returnvalue (`self.K2_GetActorLocation` Target))))
    (:`Is Not Valid`
      (set `self.FinalRotation` (`KismetMathLibrary.FindLookAtRotation` _returnvalue Location))))
  (`TimelineComponent.SetPlayRate` (`self.Timeline Rotation to Target or Location`) (/ 1.0 (/ (`KismetMathLibrary.Abs` (- (mod (`KismetMathLibrary.FTrunc` (+ (- _finalrotation_yaw _returnvalue_yaw) 180.0)) 360) 180)) RotationAngleSpeed)))
  (bind (_direction _smooth0_1) (`Timeline|Timeline Rotation to Target or Location` :!via `PlayFromStart` :!label _label_2)
    (:`Update`
      (`self.K2_SetActorRotation` (`KismetMathLibrary.RLerp` (`self.SavedRotation`) (`self.FinalRotation`) _smooth0_1 true)))))

(event `StraightLineAttack`
  (bind _returnvalue (`self.K2_GetActorLocation`))
  (bind _charactermovement (`self.CharacterMovement`))
  (`BlueprintGameplayTagLibrary.AddGameplayTag` (`self.GTC`) (struct :`TagName` "Dragons.Attack.RushAttack"))
  (bind _returnvalue_2 (`KismetSystemLibrary.K2_SetTimerDelegate` (delegate `DisapearPointPart`) 0.1 true))
  (`self.FlyAndRotateTo` (+ (`self.K2_GetActorLocation`) (* (`self.GetActorForwardVector`) 18750.0)) null 150.0)
  (`KismetSystemLibrary.Delay` 3.0)
  (`KismetSystemLibrary.K2_ClearAndInvalidateTimerHandle` _returnvalue_2)
  (`self.Stop Move`)
  (if (`BlueprintGameplayTagLibrary.HasTag` (`self.GTC`) (struct :`TagName` "Dragons.Urojony.StateTwo"))
    (set `CharacterMovementComponent.MaxFlySpeed` 10000.0 _charactermovement)
    (else
      (set `CharacterMovementComponent.MaxFlySpeed` 18000.0 _charactermovement)))
  (bind _destination (`self.GetOddPoint`))
  (`KismetSystemLibrary.K2_ClearAndInvalidateTimerHandle` (`self.Timer1`))
  (bind _returnvalue_3 (`KismetMathLibrary.Vector_Distance` _destination _returnvalue))
  (set `self.MaxDistance` _returnvalue_3)
  (`|SpawnActorFromClass` "/Game/_VisionProtocol/TestingPlayground/Filip/Zerowy_Smok/BP_MistLine.BP_MistLine_C" (`KismetMathLibrary.MakeTransform` _returnvalue (`KismetMathLibrary.FindLookAtRotation` _returnvalue _destination)) "AlwaysSpawn" "MultiplyWithRoot" self _returnvalue_3 null)
  (if (`BlueprintGameplayTagLibrary.HasTag` (`self.GTC`) (struct :`TagName` "Dragons.State.Moving")) :!label _label_3
    (`KismetSystemLibrary.Delay` 0.5)
    (goto _label_3)
    (else
      (`self.Change Speed`)
      (`self.SetPath` "/Game/_VisionProtocol/TestingPlayground/Filip/Zerowy_Smok/DA_ZerowyState1.DA_ZerowyState1")
      (`KismetSystemLibrary.K2_SetTimer` null "SpawnMistTail" 0.1 true)
      (`BlueprintGameplayTagLibrary.RemoveGameplayTag` (`self.GTC`) (struct :`TagName` "Dragons.Attack.RushAttack")))))

(event `Stop Move`
  (bind _finallocation (`self.FinalLocation`))
  (`|ExecutionSequence`
    (:`then_0`
      (goto _label_2 :!via `Stop`))
    (:`then_1`
      (bind (_direction _smooth0_1) (`Timeline|Timeline Movement to Target or Location` :!via `Stop` :!label _label_4)
        (:`Update`
          (if (not (<= (`KismetMathLibrary.Vector_Distance` _finallocation (`self.K2_GetActorLocation`)) 50.0))
            (`self.K2_SetActorLocation` (`KismetMathLibrary.VLerp` (`self.SavedLocation`) _finallocation _smooth0_1))))
        (:`Finished`
          (`self.Move Completed`))))
    (:`then_2`
      (`self.Move Completed`))))

(event `Move To`
  (params (Location :type "Vector Structure") (Target :type "Actor Object Reference"))
  (set `self.SavedLocation` (`self.K2_GetActorLocation`))
  (`/Engine/EditorBlueprintResources/StandardMacros.IsValid` Target
    (:`Is Valid`
      (set `self.FinalLocation` (`self.K2_GetActorLocation` Target)))
    (:`Is Not Valid`
      (set `self.FinalLocation` Location)))
  (`TimelineComponent.SetPlayRate` (`self.Timeline Movement to Target or Location `) (/ 1.0 (/ (`KismetMathLibrary.Vector_Distance` (`self.FinalLocation`) (`self.K2_GetActorLocation`)) (`CharacterMovementComponent.MaxFlySpeed` (`self.CharacterMovement`)))))
  (goto _label_4 :!via `PlayFromStart`))

(event `Death`
  (`BlueprintGameplayTagLibrary.AddGameplayTag` (`self.GTC`) (struct :`TagName` "Dragons.State.Dead"))
  (`self.Stop Move`)
  (bind _component (message `/Game/_VisionProtocol/TestingPlayground/Filip/Urojony_Smok/BPI_ToPlayer.GetParkourComponent` (`GameplayStatics.GetPlayerCharacter` 0)))
  (`/Game/_VisionProtocol/Core/Parkour/BP_CharacterParkourComponent.AttemptAbortGrappling` _component)
  (`RadialForceComponent.FireImpulse` (`self.RadialForce`))
  (`KismetSystemLibrary.Delay` 1.0)
  (for _index (range 11)
    (`|SpawnActorFromClass` "/Game/_VisionProtocol/TestingPlayground/Filip/Zerowy_Smok/BP_NiagaraMist.BP_NiagaraMist_C" (`KismetMathLibrary.MakeTransform` (+ (`SceneComponent.K2_GetComponentLocation` (`self.DisapearPoint`)) (* (`self.GetActorForwardVector`) (- 5000.0 (* 2000.0 _index))))) "AlwaysSpawn" "MultiplyWithRoot" null false false 900.0 1900.0 null))
  (`Widget.SetVisibility` (`self.HPBar`) "Hidden")
  (`KismetSystemLibrary.Delay` 3.0)
  (`self.K2_DestroyActor`))

(event `/Game/_VisionProtocol/TestingPlayground/Filip/Urojony_Smok/BT/BPI_Urojony.SwitchFunction`
  (params (`Event Name` :type Name) (Task :type "BTTask_BlueprintBase Object Reference") (RotationSpeed :type "Float (double-precision)"))
  (switch `name` `Event Name`
    (:`FlyToNextPoint`
      (`self.FlyToNextPoint` Task null RotationSpeed))
    (:`MistTentacleSpawn`
      (`self.SpawnMistTentacle`))
    (:`PhaseTwo`
      (`/Engine/EditorBlueprintResources/StandardMacros.DoOnce` false
        (:`Completed`
          (`self.PhaseTwo`))))
    (:`StraightLineAttack`
      (`self.StraightLineAttack`))
    (:`PhaseThree`
      (`self.PhaseThree`))
    (:`MistProjectile`
      (`self.MistProjectile`))))

(event `PhaseTwo`
  (`self.Change Speed`)
  (`self.DestoryRocks`)
  (message `/Game/_VisionProtocol/TestingPlayground/Filip/Urojony_Smok/BPI_ToPlayer.ChangeGrapplingHookSpeed` (`GameplayStatics.GetPlayerCharacter` 0) 6000.0)
  (`KismetSystemLibrary.Delay` 5.0 :!label _label_5)
  (`BlueprintGameplayTagLibrary.RemoveGameplayTag` (`self.GTC`) (struct :`TagName` "Dragons.State.Evade")))

(event `PhaseThree`
  (`self.Change Speed`)
  (message `/Game/_VisionProtocol/TestingPlayground/Filip/Urojony_Smok/BPI_ToPlayer.ChangeGrapplingHookSpeed` (`GameplayStatics.GetPlayerCharacter` 0) 9000.0)
  (goto _label_5))

(event `Change Speed`
  (bind _charactermovement (`self.CharacterMovement`))
  (if (`BlueprintGameplayTagLibrary.HasTag` (`self.GTC`) (struct :`TagName` "Dragons.Urojony.StateTwo"))
    (set `CharacterMovementComponent.MaxFlySpeed` 4000.0 _charactermovement)
    (else
      (set `CharacterMovementComponent.MaxFlySpeed` 7000.0 _charactermovement))))

(event `Spawner`
  (`|SpawnActorFromClass` "/Game/_VisionProtocol/TestingPlayground/Filip/Zerowy_Smok/BP_NiagaraMist.BP_NiagaraMist_C" (`KismetMathLibrary.MakeTransform` (`SceneComponent.K2_GetComponentLocation` (`self.NiagaraMistSpawn`))) "AlwaysSpawn" "MultiplyWithRoot" null false false 700.0 1500.0 null))

(event `self.RockChecker.OnComponentBeginOverlap`
  (params (OverlappedComponent :type "PrimitiveComponent Object Reference") (OtherActor :type "Actor Object Reference") (OtherComp :type "PrimitiveComponent Object Reference") (OtherBodyIndex :type Integer) (bFromSweep :type Boolean) (SweepResult :type "HitResult Structure (by ref)"))
  (bind _returnvalue (`GameplayStatics.GetPlayerCharacter` 0))
  (if (`self.ActorHasTag` OtherActor "Floating")
    _
    (elif (== (`GameplayStatics.GetPlayerCharacter` 0) OtherActor)
      (bind _component (message `/Game/_VisionProtocol/TestingPlayground/Filip/Urojony_Smok/BPI_ToPlayer.GetParkourComponent` (`GameplayStatics.GetPlayerCharacter` 0)))
      (`/Game/_VisionProtocol/Core/Parkour/BP_CharacterParkourComponent.AttemptAbortGrappling` _component)
      (message `/Game/_VisionProtocol/Core/DMG-HP/BPI_Damageable.TakeDamage` _returnvalue 30.0)
      (`self.LaunchCharacter` _returnvalue (`KismetMathLibrary.MakeVector` (.x (* (`KismetMathLibrary.Normal` (- (`self.K2_GetActorLocation` _returnvalue) (`self.K2_GetActorLocation`))) 12000.0)) (.y (* (`KismetMathLibrary.Normal` (- (`self.K2_GetActorLocation` _returnvalue) (`self.K2_GetActorLocation`))) 12000.0)) (`KismetMathLibrary.FMax` (.z (* (`KismetMathLibrary.Normal` (- (`self.K2_GetActorLocation` _returnvalue) (`self.K2_GetActorLocation`))) 12000.0)) 2000.0)) true true))))

(event `MistProjectile`
  (if (not (`BlueprintGameplayTagLibrary.HasTag` (`self.GTC`) (struct :`TagName` "Dragons.Attack.RushAttack")))
    (bind _niagaramistspawn (`self.NiagaraMistSpawn`)
      (:`then`
        (bind _returnvalue (`|SpawnActorFromClass` "/Game/_VisionProtocol/TestingPlayground/Filip/Zerowy_Smok/BP_NiagaraMist.BP_NiagaraMist_C" (`KismetMathLibrary.MakeTransform` (`SceneComponent.K2_GetComponentLocation` _niagaramistspawn)) "AlwaysSpawn" "MultiplyWithRoot" null false false 500.0 500.0 null))
        (`KismetSystemLibrary.Delay` 2.0)
        (`/Engine/EditorBlueprintResources/StandardMacros.IsValid` _returnvalue
          (:`Is Valid`
            (bind _returnvalue_2 (`self.K2_GetActorLocation` _returnvalue))
            (bind _returnvalue_3 (`|SpawnActorFromClass` "/Game/_VisionProtocol/TestingPlayground/Filip/Zerowy_Smok/BP_MistProjectile.BP_MistProjectile_C" (`KismetMathLibrary.MakeTransform` _returnvalue_2 (`KismetMathLibrary.FindLookAtRotation` _returnvalue_2 (`self.K2_GetActorLocation` (`GameplayStatics.GetPlayerCharacter` 0)))) "AlwaysSpawn" "MultiplyWithRoot" null false true 400.0 500.0 null))
            (`KismetSystemLibrary.Delay` 2.0)
            (`/Engine/EditorBlueprintResources/StandardMacros.IsValid` _returnvalue
              (:`Is Valid`
                (`self.K2_DestroyActor` _returnvalue)
                (`KismetSystemLibrary.Delay` 20.0)
                (`/Engine/EditorBlueprintResources/StandardMacros.IsValid` _returnvalue_3
                  (:`Is Valid`
                    (`self.K2_DestroyActor` _returnvalue_3))))))))
      (:`else`))))

(event `self.RockChecker.OnComponentEndOverlap`
  (params (OverlappedComponent :type "PrimitiveComponent Object Reference") (OtherActor :type "Actor Object Reference") (OtherComp :type "PrimitiveComponent Object Reference") (OtherBodyIndex :type Integer)))

(fn `AddGrapplingTag`
  (`KismetArrayLibrary.Array_AddUnique` (`self.Tags`) "GrapplingHook"))

(fn `DestoryRocks`
  (locals (LocalActors :type "Array of /Game/_VisionProtocol/TestingPlayground/Filip/Zerowy_Smok/BP_FloatingRockMain Object Reference"))
  (bind _outactors (`GameplayStatics.GetAllActorsOfClass` "/Game/_VisionProtocol/TestingPlayground/Filip/Zerowy_Smok/BP_FloatingRockMain.BP_FloatingRockMain_C"))
  (bind _output_get (set `local.LocalActors` _outactors)))

(fn `FlyAndRotateTo`
  (params (Location :type "Vector Structure") (Target :type "Actor Object Reference") (RotationSpeed :type "Float (double-precision)"))
  (`BlueprintGameplayTagLibrary.AddGameplayTag` (`self.GTC`) (struct :`TagName` "Dragons.State.Moving"))
  (`self.RotateTo` Location Target RotationSpeed)
  (`self.Move To` Location Target)
  (return))

(fn `GetCurrentHealth`
  (returns (Health :type "Float (double-precision)"))
  (return (`/Game/_VisionProtocol/Core/DMG-HP/C_DMG-HP.CurrentHealth` (`self.C_DMG-HP`))))

(fn `GetGTC`
  (returns (Container :type "GameplayTagContainer Structure"))
  (return (`self.GTC`)))

(fn `GetMaxHealth`
  (returns (MaxHealth :type "Float (double-precision)"))
  (return (`/Game/_VisionProtocol/Core/DMG-HP/C_DMG-HP.MaximumHealth` (`self.C_DMG-HP`))))

(fn `GetOddPoint`
  (returns (Destination :type "Vector Structure"))
  (locals (Index :type Integer) (StartLocation :type "Vector Structure") (SelectedLocation :type "Vector Structure") (NewLocalVar :type Integer :default 0))
  (bind _location_fight (`/Game/_VisionProtocol/TestingPlayground/Filip/Urojony_Smok/DA_SmokUrojony_Locations_Fight.Location_Fight` (`self.DA Flight Locations`)))
  (bind _output (`|GetArrayItem` (`/Game/_VisionProtocol/TestingPlayground/Filip/Urojony_Smok/DA_SmokUrojony_Locations_Fight.Location_Fight` (`self.DA Flight Locations`)) (+ (`local.Index`) 1)))
  (bind _output_2 (`|GetArrayItem` (`/Game/_VisionProtocol/TestingPlayground/Filip/Urojony_Smok/DA_SmokUrojony_Locations_Fight.Location_Fight` (`self.DA Flight Locations`))))
  (set `local.Index` (`.OutIndex` (`KismetArrayLibrary.Array_Random` _location_fight)))
  (`self.K2_SetActorLocation` (`|GetArrayItem` _location_fight (`local.Index`)))
  (if (== (`KismetArrayLibrary.Array_LastIndex` _location_fight) (`local.Index`))
    (set `local.SelectedLocation` _output_2)
    (`self.FlyAndRotateTo` _output_2 null 150.0)
    (else
      (set `local.SelectedLocation` _output)
      (`self.FlyAndRotateTo` _output null 150.0)))
  (return (`local.SelectedLocation`)))

(fn `Heal`
  (params (HP_Amount :type "Float (double-precision)"))
  (returns (`New Health` :type "Float (double-precision)"))
  (bind _new_health (`/Game/_VisionProtocol/Core/DMG-HP/C_DMG-HP.Heal` (`self.C_DMG-HP`) HP_Amount))
  (return _new_health))

(fn `IsDead`
  (returns (Dead :type Boolean))
  (return (`/Game/_VisionProtocol/Core/DMG-HP/C_DMG-HP.isDead` (`self.C_DMG-HP`))))

(fn `TakeDamage`
  (params (Amount :type "Float (double-precision)"))
  (returns (`Was Damaged` :type Boolean))
  (bind _gtc (`self.GTC`))
  (if (`BlueprintGameplayTagLibrary.HasTag` _gtc (struct :`TagName` "Dragons.State.Evade"))
    (bind _component (message `/Game/_VisionProtocol/TestingPlayground/Filip/Urojony_Smok/BPI_ToPlayer.GetParkourComponent` (`GameplayStatics.GetPlayerCharacter` 0)))
    (`/Game/_VisionProtocol/Core/Parkour/BP_CharacterParkourComponent.AttemptAbortGrappling` _component)
    (return false)
    (elif (`BlueprintGameplayTagLibrary.HasTag` _gtc (struct :`TagName` "Dragons.State.Invincible"))
      (return false)
      (else
        (bind _was_damaged (`/Game/_VisionProtocol/Core/DMG-HP/C_DMG-HP.TakeDamage` (`self.C_DMG-HP`) Amount))
        (`KismetArrayLibrary.Array_RemoveItem` (`self.Tags`) "GrapplingHook")
        (`|ExecutionSequence`
          (:`then_0`
            (`KismetSystemLibrary.K2_SetTimer` null "AddGrapplingTag" 10.0))
          (:`then_1`
            (return _was_damaged)))))))

(fn `UserConstructionScript`
  (locals (IndexLine :type Integer :default 1))
  (bind _c_dmg_hp (`self.C_DMG-HP`))
  (add `/Game/_VisionProtocol/Core/DMG-HP/C_DMG-HP.OnDeath` _c_dmg_hp (`|CreateDelegate` :!event `Death`))
  (bind _output_get (set `/Game/_VisionProtocol/Core/DMG-HP/C_DMG-HP.MaximumHealth` 550.0 _c_dmg_hp))
  (set `/Game/_VisionProtocol/Core/DMG-HP/C_DMG-HP.CurrentHealth` _output_get _c_dmg_hp))
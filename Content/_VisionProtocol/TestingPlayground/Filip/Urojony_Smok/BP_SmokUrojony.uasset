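; Urojony Smok flying dragon boss, driven by a behavior tree that dispatches actions through SwitchFunction.
; Timeline-based flight follows data-asset points, with gameplay tags tracking state and move completion finishing tasks.
; Attacks include acid shots and sprays, a diving charge, and QVisor-visible eye lasers that spawn random actors above the player.
; Phase three grants invincibility and polls a count of spawned actors touching the dragon, with its fall still unimplemented.
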(event `/Game/_VisionProtocol/TestingPlayground/Filip/T_Smok/BPI_Dragons.LineTraceHit`
  (if (`self.bPhaseThree`)
    (if (not (`BlueprintGameplayTagLibrary.HasTag` (`self.GTC`) (struct :`TagName` "Dragons.Attack.SpamAttack")))
      (`self.StopMove`)
      (`self.FlyToNextPoint` (`self.Task`) true))))

(event `BelowDmg`
  (if (`self.bInvincible`)
    (message `/Game/_VisionProtocol/Core/DMG-HP/BPI_Damageable.TakeDamage` (`GameplayStatics.GetPlayerCharacter` 0) 3.0)
    (`KismetSystemLibrary.PrintString` "Gracz otrzymal obrazenia od BELOW DMG")))

(event `AcidSpamAttack`
  (set `self.Index` 0)
  (`/Game/_VisionProtocol/Core/Visors/Quantovisor/SC_Quantum.OnSpamAttack` (`self.SC_Quantum`))
  (`BlueprintGameplayTagLibrary.AddGameplayTag` (`self.GTC`) (struct :`TagName` "Dragons.Attack.SpamAttack"))
  (if (<= (`self.Index`) 100) :!label _label
    (`self.RotateTo` (0.0 0.0 0.0) (`GameplayStatics.GetPlayerCharacter` 0))
    (`self.Acid`)
    (`KismetSystemLibrary.Delay` 0.1)
    (`/Engine/EditorBlueprintResources/StandardMacros.IncrementInt` (`self.Index`)
      (:`  `
        (goto _label)))
    (else
      (`BlueprintGameplayTagLibrary.RemoveGameplayTag` (`self.GTC`) (struct :`TagName` "Dragons.Attack.SpamAttack"))
      (`/Game/_VisionProtocol/Core/Visors/Quantovisor/SC_Quantum.OnSpamAttack` (`self.SC_Quantum`)))))

(event `Phase3TickCheckQuantoAtt`
  (`KismetSystemLibrary.PrintString` (`KismetStringLibrary.Concat_StrStr` "Aktualna liczba Attach do smoka: " (`KismetStringLibrary.Conv_IntToString` (`self.QuantoAttached`))) true true (struct :`G` 0.66 :`B` 1.0 :`A` 1.0) 2.0 "Attached")
  (if (>= (`self.Index`) 5)
    (set `self.QuantoAttached` 0) ; Tutaj będzie spadanie smoka (po Delay)
  ))

(event `PhaseThree`
  (set `self.bPhaseThree` true)
  (`BlueprintGameplayTagLibrary.AddGameplayTag` (`self.GTC`) (struct :`TagName` "Dragons.State.Invincible"))
  (`KismetSystemLibrary.K2_SetTimerDelegate` (delegate `Phase3TickCheckQuantoAtt`) 1.0 true))

(event `LaserTick`
  (bind _savedlocation (`self.SavedLocation`))
  (bind _savedlocation_2 (`self.SavedLocation`))
  (bind _activated (message `/Game/_VisionProtocol/TestingPlayground/Filip/Urojony_Smok/BPI_ToPlayer.Get Q Visor Status` (`GameplayStatics.GetPlayerCharacter` 0)))
  (if _activated
    _
    (else
      _))
  (bind _returnvalue (not _activated))
  (`SceneComponent.SetHiddenInGame` (`self.LaserEye2`) _returnvalue false)
  (`SceneComponent.SetHiddenInGame` (`self.ImpactLaser2`) _returnvalue false)
  (`SceneComponent.SetHiddenInGame` (`self.LaserEye1`) _returnvalue false)
  (`SceneComponent.SetHiddenInGame` (`self.ImpactLaser1`) _returnvalue false)
  (`|ExecutionSequence`
    (:`then_0`
      (`NiagaraComponent.SetVariableVec3` (`self.LaserEye1`) "LaserEnd" _savedlocation_2)
      (`SceneComponent.K2_SetWorldLocation` (`self.ImpactLaser1`) _savedlocation_2 false false))
    (:`then_1`
      (`NiagaraComponent.SetVariableVec3` (`self.LaserEye2`) "LaserEnd" _savedlocation)
      (`SceneComponent.K2_SetWorldLocation` (`self.ImpactLaser2`) _savedlocation false false))))

(event `AddBar`
  (bind _returnvalue (`|CreateWidget` "/Game/_VisionProtocol/TestingPlayground/Filip/T_Smok/WBP_BossHealthBar.WBP_BossHealthBar_C" null self))
  (bind _output_get (set `self.HPBar` _returnvalue))
  (add `UserWidget.OnVisibilityChanged` _output_get (delegate `OnVisibilityChanged_Event`))
  (`UserWidget.AddToViewport` _output_get 0))

(event `LaserAttack`
  (bind _spawnarray (`self.SpawnArray`))
  (`BlueprintGameplayTagLibrary.AddGameplayTag` (`self.GTC`) (struct :`TagName` "Dragons.Attack.LaserAttack"))
  (set `self.SavedLocation` (+ (`self.K2_GetActorLocation` (`GameplayStatics.GetPlayerCharacter` 0)) (`KismetMathLibrary.MakeVector` (`KismetMathLibrary.RandomFloatInRange` -10.0 10.0) (`KismetMathLibrary.RandomFloatInRange` -10.0 10.0) 1900.0)))
  (bind _returnvalue (`KismetSystemLibrary.K2_SetTimer` null "LaserTick" 0.01 true))
  (`KismetSystemLibrary.Delay` 1.5)
  (bind _class (`|LoadAssetClass` (`|GetArrayItem` _spawnarray (`KismetMathLibrary.RandomIntegerInRange` 0 (- (`KismetArrayLibrary.Array_Length` _spawnarray) 1))))
    (:`Completed`
      (bind _asactor (castclass `Actor` _class))
      (`|SpawnActorFromClass` _asactor (`KismetMathLibrary.MakeTransform` (`self.SavedLocation`)) "Undefined" "MultiplyWithRoot" null null)
      (`KismetSystemLibrary.Delay` 0.5)
      (`KismetSystemLibrary.K2_ClearAndInvalidateTimerHandle` _returnvalue)
      (`SceneComponent.SetHiddenInGame` (`self.LaserEye2`) true false)
      (`SceneComponent.SetHiddenInGame` (`self.ImpactLaser2`) true false)
      (`SceneComponent.SetHiddenInGame` (`self.LaserEye1`) true false)
      (`SceneComponent.SetHiddenInGame` (`self.ImpactLaser1`) true false)
      (`BlueprintGameplayTagLibrary.RemoveGameplayTag` (`self.GTC`) (struct :`TagName` "Dragons.Attack.LaserAttack")))))

(event `OnVisibilityChanged_Event`
  (params (InVisibility :type "ESlateVisibility Enum" :default "Visible"))
  (`Widget.RemoveFromParent` (stale `AddBar` _output_get)))

(event `Acid`
  (bind _returnvalue (`SceneComponent.K2_GetComponentToWorld` (`self.SpawnBullet`)))
  (`|SpawnActorFromClass` "/Game/_VisionProtocol/TestingPlayground/Filip/Urojony_Smok/Efekty/BP_AcitTest.BP_AcitTest_C" (`KismetMathLibrary.MakeTransform` (.location _returnvalue) (`KismetMathLibrary.MakeRotator` (.roll (.rotation _returnvalue)) (+ (.pitch (.rotation _returnvalue)) (`KismetMathLibrary.RandomFloatInRange` -5.0 5.0)) (+ (.yaw (.rotation _returnvalue)) (`KismetMathLibrary.RandomFloatInRange` -5.0 5.0))) (.scale _returnvalue)) "Undefined" "MultiplyWithRoot" null null))

(event `FlyToNextPoint`
  (params (Task :type "BTTask_BlueprintBase Object Reference") (Random :type Boolean))
  (bind _location_fight (`/Game/_VisionProtocol/TestingPlayground/Filip/Urojony_Smok/DA_SmokUrojony_Locations_Fight.Location_Fight` (`self.DA_FightLocations`)))
  (bind _location_fight_2 (`/Game/_VisionProtocol/TestingPlayground/Filip/Urojony_Smok/DA_SmokUrojony_Locations_Fight.Location_Fight` (`self.DA_FightLocations`)))
  (bind _output (`|GetArrayItem` _location_fight (`KismetMathLibrary.RandomInteger` (- (`KismetArrayLibrary.Array_Length` _location_fight) 1))))
  (if Random
    (if (>= (`KismetMathLibrary.Vector_Distance` _output (`self.K2_GetActorLocation`)) 100.0) :!label _label_2
      (`self.TaskFaRt` _output null Task)
      (else
        (`KismetSystemLibrary.RetriggerableDelay` 0.1)
        (goto _label_2)))
    (elif (< (`self.Index`) (`KismetArrayLibrary.Array_Length` (`/Game/_VisionProtocol/TestingPlayground/Filip/Urojony_Smok/DA_SmokUrojony_Locations_Fight.Location_Fight` (`self.DA_FightLocations`))))
      (if (== (`self.Index`) 0)
        (`self.TaskFaRt` (`|GetArrayItem` _location_fight_2) null Task :!label _label_3)
        (`/Engine/EditorBlueprintResources/StandardMacros.IncrementInt` (`self.Index`))
        (else
          (`self.TaskFaRt` (`|GetArrayItem` _location_fight_2) null Task)
          (`/Engine/EditorBlueprintResources/StandardMacros.IncrementInt` (`self.Index`))))
      (else
        (set `self.Index` 0)
        (goto _label_3)))))

(event `/Game/_VisionProtocol/TestingPlayground/Filip/Urojony_Smok/BT/BPI_Urojony.SetPath`
  (params (`New Path` :type "/Game/_VisionProtocol/TestingPlayground/Filip/Urojony_Smok/DA_SmokUrojony_Locations_Fight Object Reference"))
  (set `self.DA_FightLocations` `New Path`))

(event `/Game/_VisionProtocol/TestingPlayground/Filip/Urojony_Smok/BT/BPI_Urojony.SetGTC`
  (params (GTC :type "GameplayTagContainer Structure"))
  (set `self.GTC` GTC))

(event `self.ReceiveBeginPlay`
  (`KismetSystemLibrary.DelayUntilNextTick`)
  (`AIController.RunBehaviorTree` (`AIBlueprintHelperLibrary.GetAIController` self) (`self.BehaviorTree`))
  (add `self.OnStopMovement` (`|CreateDelegate` :!event `StopMove`))
  (add `self.OnMoveCompleted` (`|CreateDelegate` :!event `DoneMoving`))
  (message `/Game/_VisionProtocol/TestingPlayground/Filip/Urojony_Smok/BPI_ToPlayer.UrojonyStart` (`GameplayStatics.GetPlayerCharacter` 0) self)
  (add `/Game/_VisionProtocol/Core/Visors/Quantovisor/SC_Quantum.OnDoneMoving` (`self.SC_Quantum`) (`|CreateDelegate` :!event `AttachActorToDragon`)))

(event `/Game/_VisionProtocol/TestingPlayground/Filip/Urojony_Smok/BT/BPI_Urojony.SwitchFunction`
  (params (`Event Name` :type Name) (Task :type "BTTask_BlueprintBase Object Reference"))
  (switch `name` `Event Name`
    (:`Arriving`
      (`self.Arriving` null))
    (:`FlyToNextPoint`
      (`self.FlyToNextPoint` Task true))
    (:`AcidAttack`
      (`self.Acid`))
    (:`ChargeAttack`
      (`self.ChargeAttack`))
    (:`LaserAttack`
      (`self.LaserAttack`))
    (:`PhaseThree`
      (`/Engine/EditorBlueprintResources/StandardMacros.DoOnce` false
        (:`Completed`
          (`self.PhaseThree`))))
    (:`SpamAttack`
      (`self.AcidSpamAttack`))))

(event `Arriving`
  (params (Task :type "BTTask_BlueprintBase Object Reference"))
  (bind _gtc (`self.GTC`))
  (bind _index (`self.Index`))
  (if (< (`self.Index`) (`KismetArrayLibrary.Array_Length` (`/Game/_VisionProtocol/TestingPlayground/Filip/Urojony_Smok/DA_SmokUrojony_Locations_Fight.Location_Fight` (`self.DA_FightLocations`))))
    (if (== _index 0)
      (`/Engine/EditorBlueprintResources/StandardMacros.IncrementInt` (`self.Index`)
        (:`  `
          (`self.TaskFaRt` (`|GetArrayItem` (`/Game/_VisionProtocol/TestingPlayground/Filip/Urojony_Smok/DA_SmokUrojony_Locations_Fight.Location_Fight` (`self.DA_FightLocations`))) null Task)))
      (else
        (`self.TaskFaRt` (`|GetArrayItem` (`/Game/_VisionProtocol/TestingPlayground/Filip/Urojony_Smok/DA_SmokUrojony_Locations_Fight.Location_Fight` (`self.DA_FightLocations`)) _index) null Task)
        (`/Engine/EditorBlueprintResources/StandardMacros.IncrementInt` (`self.Index`))))
    (else
      (set `self.DA_FightLocations` "/Game/_VisionProtocol/TestingPlayground/Filip/Urojony_Smok/DA_Phase1_Path.DA_Phase1_Path")
      (`BlueprintGameplayTagLibrary.RemoveGameplayTag` _gtc (struct :`TagName` "Dragons.Urojony.StateZero"))
      (`BlueprintGameplayTagLibrary.AddGameplayTag` _gtc (struct :`TagName` "Dragons.Urojony.StateOne"))
      (set `self.Index` 0)
      (`self.DoneMoving`)
      (`self.AddBar`))))

(event `ChargeAttack`
  (bind _returnvalue (`self.K2_GetActorLocation`))
  (bind _charactermovement (`self.CharacterMovement`))
  (bind _returnvalue_2 (`self.K2_GetActorLocation` (`GameplayStatics.GetPlayerCharacter` 0)))
  (`BlueprintGameplayTagLibrary.AddGameplayTag` (`self.GTC`) (struct :`TagName` "Dragons.Attack.RushAttack"))
  (bind _outhit (`KismetSystemLibrary.LineTraceSingle` _returnvalue (`KismetMathLibrary.MakeVector` (.x _returnvalue) (.y _returnvalue) -10000.0) "TraceTypeQuery1"))
  (`self.FlyAndRotateTo` (+ (`.Location` (`GameplayStatics.BreakHitResult` _outhit)) (0.0 0.0 300.0)) null 250.0)
  (if (not (`BlueprintGameplayTagLibrary.HasTag` (`self.GTC`) (struct :`TagName` "Dragons.State.Moving"))) :!label _label_4
    (set `CharacterMovementComponent.MaxFlySpeed` 3500.0 _charactermovement)
    (`self.FlyAndRotateTo` (+ (+ (* (`KismetMathLibrary.Normal` (- _returnvalue_2 (`self.K2_GetActorLocation`))) 200.0) _returnvalue_2) (0.0 0.0 70.0)) null 240.0)
    (if (not (`BlueprintGameplayTagLibrary.HasTag` (`self.GTC`) (struct :`TagName` "Dragons.State.Moving"))) :!label _label_5
      (set `CharacterMovementComponent.MaxFlySpeed` 1400.0 _charactermovement)
      (`self.FlyAndRotateTo` (+ (`self.K2_GetActorLocation`) (0.0 0.0 1000.0)) null 240.0)
      (`KismetSystemLibrary.Delay` 0.25)
      (`self.FlyToNextPoint` null true)
      (`KismetSystemLibrary.Delay` 1.0)
      (`BlueprintGameplayTagLibrary.RemoveGameplayTag` (`self.GTC`) (struct :`TagName` "Dragons.Attack.RushAttack"))
      (else
        (`KismetSystemLibrary.Delay` 0.25)
        (goto _label_5)))
    (else
      (`KismetSystemLibrary.Delay` 0.25)
      (goto _label_4))))

(event `OnDeath`
  (message `/Game/_VisionProtocol/TestingPlayground/Filip/Urojony_Smok/BPI_ToPlayer.DragonIsDead` (`GameplayStatics.GetPlayerCharacter` 0)))

(event `RotateTo`
  (params (Location :type "Vector Structure") (Target :type "Actor Object Reference") (RotationAngleSpeed :type "Float (double-precision)" :default 150.0))
  (bind _returnvalue (`self.K2_GetActorLocation`))
  (bind (_returnvalue_roll _returnvalue_pitch _returnvalue_yaw) (`KismetMathLibrary.BreakRotator` (`self.K2_GetActorRotation`)))
  (bind (_finalrotation_roll _finalrotation_pitch _finalrotation_yaw) (`KismetMathLibrary.BreakRotator` (`self.FinalRotation`)))
  (set `self.SavedRotation` (`self.K2_GetActorRotation`))
  (`/Engine/EditorBlueprintResources/StandardMacros.IsValid` Target
    (:`Is Valid`
      (set `self.FinalRotation` (`KismetMathLibrary.FindLookAtRotation` _returnvalue (`self.K2_GetActorLocation` Target))))
    (:`Is Not Valid`
      (set `self.FinalRotation` (`KismetMathLibrary.FindLookAtRotation` _returnvalue Location))))
  (`TimelineComponent.SetPlayRate` (`self.TimelineRotationToTargetOrLocation`) (/ 1.0 (/ (`KismetMathLibrary.Abs` (- (mod (`KismetMathLibrary.FTrunc` (+ (- _finalrotation_yaw _returnvalue_yaw) 180.0)) 360) 180)) RotationAngleSpeed)))
  (bind (_direction _smooth0_1) (`Timeline|TimelineRotationToTargetOrLocation` :!via `PlayFromStart` :!label _label_6)
    (:`Update`
      (`self.K2_SetActorRotation` (`KismetMathLibrary.RLerp` (`self.SavedRotation`) (`self.FinalRotation`) _smooth0_1 true)))))

(event `self.ChargeBox.OnComponentBeginOverlap`
  (params (OverlappedComponent :type "PrimitiveComponent Object Reference") (OtherActor :type "Actor Object Reference") (OtherComp :type "PrimitiveComponent Object Reference") (OtherBodyIndex :type Integer) (bFromSweep :type Boolean) (SweepResult :type "HitResult Structure (by ref)"))
  (`KismetSystemLibrary.PrintString` "Overlap ChargeBox")
  (if (== (`GameplayStatics.GetObjectClass` OtherActor) (`self.PlayerRefSoft`))
    (message `/Game/_VisionProtocol/Core/DMG-HP/BPI_Damageable.TakeDamage` OtherActor 35.0)
    (`KismetSystemLibrary.PrintString` "Zadano obrazenia")))

(event `DoneMoving`
  (bind _task (`self.Task`))
  (`BlueprintGameplayTagLibrary.RemoveGameplayTag` (`self.GTC`) (struct :`TagName` "Dragons.State.Moving"))
  (`/Engine/EditorBlueprintResources/StandardMacros.IsValid` _task
    (:`Is Valid`
      (`BTTask_BlueprintBase.FinishExecute` _task true))
    (:`Is Not Valid`
      (if (`BlueprintGameplayTagLibrary.HasTag` (`self.GTC`) (struct :`TagName` "Dragons.Urojony.StateZero"))
        (`self.Arriving` null)))))

(event `StopMove`
  (bind _finallocation (`self.FinalLocation`))
  (`|ExecutionSequence`
    (:`then_0`
      (bind (_direction _smooth0_1) (`Timeline|TimelineMovementToTargetOrLocation` :!via `Stop` :!label _label_7)
        (:`Update`
          (if (not (<= (`KismetMathLibrary.Vector_Distance` _finallocation (`self.K2_GetActorLocation`)) 50.0))
            (`self.K2_SetActorLocation` (`KismetMathLibrary.VLerp` (`self.SavedLocation`) _finallocation _smooth0_1))))
        (:`Finished`
          (`self.OnMoveCompleted`))))
    (:`then_1`
      (goto _label_6 :!via `Stop`))))

(event `Move To`
  (params (Location :type "Vector Structure") (Target :type "Actor Object Reference"))
  (set `self.SavedLocation` (`self.K2_GetActorLocation`))
  (`/Engine/EditorBlueprintResources/StandardMacros.IsValid` Target
    (:`Is Valid`
      (set `self.FinalLocation` (`self.K2_GetActorLocation` Target)))
    (:`Is Not Valid`
      (set `self.FinalLocation` Location)))
  (`TimelineComponent.SetPlayRate` (`self.TimelineMovementToTargetOrLocation`) (/ 1.0 (/ (`KismetMathLibrary.Vector_Distance` (`self.FinalLocation`) (`self.K2_GetActorLocation`)) (`CharacterMovementComponent.MaxFlySpeed` (`self.CharacterMovement`)))))
  (goto _label_7 :!via `PlayFromStart`))

(event `self.QuantoChecker.OnComponentBeginOverlap`
  (params (OverlappedComponent :type "PrimitiveComponent Object Reference") (OtherActor :type "Actor Object Reference") (OtherComp :type "PrimitiveComponent Object Reference") (OtherBodyIndex :type Integer) (bFromSweep :type Boolean) (SweepResult :type "HitResult Structure (by ref)"))
  (if (not (== OtherActor self))
    (for _array_element (`self.SpawnArray`)
      (if (== (`GameplayStatics.GetObjectClass` OtherActor) _array_element)
        (set `self.QMain` OtherActor)
        (`/Engine/EditorBlueprintResources/StandardMacros.IncrementInt` (`self.QuantoAttached`))))))

(event `AttachActorToDragon`
  (`self.K2_AttachToActor` (`self.QMain`) self "None" "KeepRelative" "KeepRelative" "KeepRelative" true))

(fn `FlyAndRotateTo`
  (params (Location :type "Vector Structure") (Target :type "Actor Object Reference") (Angle :type "Float (double-precision)" :default 150.0))
  (`BlueprintGameplayTagLibrary.AddGameplayTag` (`self.GTC`) (struct :`TagName` "Dragons.State.Moving"))
  (`self.RotateTo` Location Target Angle)
  (`self.Move To` Location Target))

(fn `GetCurrentHealth`
  (returns (Health :type "Float (double-precision)"))
  (return (`/Game/_VisionProtocol/Core/DMG-HP/C_DMG-HP.CurrentHealth` (`self.C_DMG-HP`))))

(fn `GetGTC`
  (returns (Container :type "GameplayTagContainer Structure"))
  (return (`self.GTC`)))

(fn `GetLocationPoint`
  (returns (Location :type "Vector Structure"))
  (return (0.0 0.0 0.0)))

(fn `GetMaxHealth`
  (returns (MaxHealth :type "Float (double-precision)"))
  (return (`/Game/_VisionProtocol/Core/DMG-HP/C_DMG-HP.MaximumHealth` (`self.C_DMG-HP`))))

(fn `Heal`
  (params (HP_Amount :type "Float (double-precision)"))
  (returns (`New Health` :type "Float (double-precision)"))
  (bind _new_health (`/Game/_VisionProtocol/Core/DMG-HP/C_DMG-HP.Heal` (`self.C_DMG-HP`) HP_Amount))
  (return _new_health))

(fn `IsDead`
  (returns (Dead :type Boolean))
  (return (`/Game/_VisionProtocol/Core/DMG-HP/C_DMG-HP.isDead` (`self.C_DMG-HP`))))

(fn `TakeDamage`
  (params (Amount :type "Float (double-precision)"))
  (returns (`Was Damaged` :type Boolean))
  (if (`BlueprintGameplayTagLibrary.HasTag` (`self.GTC`) (struct :`TagName` "Dragons.State.Invincible"))
    (return false)
    (else
      (bind _was_damaged (`/Game/_VisionProtocol/Core/DMG-HP/C_DMG-HP.TakeDamage` (`self.C_DMG-HP`) Amount))
      (return _was_damaged))))

(fn `TaskFaRt`
  (params (Location :type "Vector Structure") (Actor :type "Actor Object Reference") (Task :type "BTTask_BlueprintBase Object Reference"))
  (set `self.Task` Task)
  (`self.FlyAndRotateTo` Location Actor))

(fn `UserConstructionScript`
  (locals (IndexLine :type Integer :default 1))
  (bind _returnvalue (`self.K2_GetActorLocation`))
  (bind _c_dmg_hp (`self.C_DMG-HP`))
  (bind _location_fight (`/Game/_VisionProtocol/TestingPlayground/Filip/Urojony_Smok/DA_SmokUrojony_Locations_Fight.Location_Fight` (`self.DA_FightLocations`)))
  (bind _output (`|GetArrayItem` _location_fight (`local.IndexLine`)))
  (bind _output_get (set `/Game/_VisionProtocol/Core/DMG-HP/C_DMG-HP.MaximumHealth` 500.0 _c_dmg_hp))
  (set `/Game/_VisionProtocol/Core/DMG-HP/C_DMG-HP.CurrentHealth` _output_get _c_dmg_hp)
  (for (_array_element _array_index) _location_fight
    (if (< _array_index (- (`KismetArrayLibrary.Array_Length` _location_fight) 1))
      (`KismetSystemLibrary.DrawDebugLine` _array_element _output (struct :`R` 0.883377 :`B` 1.0 :`A` 1.0) 25.0 10.0)
      (`/Engine/EditorBlueprintResources/StandardMacros.IncrementInt` (`local.IndexLine`))
      (else
        (set `local.IndexLine` 0)
        (`KismetSystemLibrary.DrawDebugLine` _array_element _output (struct :`R` 0.883377 :`B` 1.0 :`A` 1.0) 25.0 10.0))))
  (`NiagaraComponent.SetVariableVec3` (`self.LaserEye1`) "LaserEnd" _returnvalue)
  (`NiagaraComponent.SetVariableVec3` (`self.LaserEye2`) "LaserEnd" _returnvalue)
  (`SceneComponent.SetHiddenInGame` (`self.LaserEye2`) true false)
  (`SceneComponent.SetHiddenInGame` (`self.ImpactLaser2`) true false)
  (`SceneComponent.SetHiddenInGame` (`self.LaserEye1`) true false)
  (`SceneComponent.SetHiddenInGame` (`self.ImpactLaser1`) true false))
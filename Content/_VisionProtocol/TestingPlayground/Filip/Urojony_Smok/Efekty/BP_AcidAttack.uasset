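; BP_AcidAttack is an acid attack actor that destroys itself when its sphere collision begins overlapping.
; BeginPlay binds AcidNiagara to the actor's destroyed event, but that handler is empty, so no effect or damage logic follows destruction.
; The actor overlap event only calls the parent, and the Niagara texture and debug print nodes are unconnected leftovers.
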(event `self.ReceiveBeginPlay`
  (`parent.ReceiveBeginPlay`)
  (add `self.OnDestroyed` (delegate `AcidNiagara`)))

(event `self.ReceiveActorBeginOverlap`
  (params (OtherActor :type "Actor Object Reference"))
  (`parent.ReceiveActorBeginOverlap` OtherActor))

(event `AcidNiagara` :!signature `self.OnDestroyed`
  (params (DestroyedActor :type "Actor Object Reference")))

(event `self.Sphere_0.OnComponentBeginOverlap`
  (params (OverlappedComponent :type "PrimitiveComponent Object Reference") (OtherActor :type "Actor Object Reference") (OtherComp :type "PrimitiveComponent Object Reference") (OtherBodyIndex :type Integer) (bFromSweep :type Boolean) (SweepResult :type "HitResult Structure (by ref)"))
  (`self.K2_DestroyActor`))

(fn `UserConstructionScript`
  (`parent.UserConstructionScript`))
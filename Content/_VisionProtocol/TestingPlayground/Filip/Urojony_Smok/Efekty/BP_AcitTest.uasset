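; BP_AcitTest is a test acid attack actor that bursts into a venom effect on hit and damages a player standing in it.
; On hit it hides its mesh, spawns the Niagara effect, levels AcidArea and destroys itself after seven seconds.
; AcidArea overlaps, plus a distance check at impact, drive a looping damage timer.
; SCQuantum and the player's visor state govern actor and effect visibility.
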(event `self.ReceiveBeginPlay`
  (add `/Game/_VisionProtocol/TestingPlayground/Filip/Visors/QuantumVisor/SC_Quantum.OnPlayerActivatedQ` (`self.SC_Quantum`) (`|CreateDelegate` :!event `UnhideNiagara`))
  (add `/Game/_VisionProtocol/TestingPlayground/Filip/Visors/QuantumVisor/SC_Quantum.OnPlayerDeactivatedQ` (`self.SC_Quantum`) (`|CreateDelegate` :!event `HideNiagara`))
  (if (`/Game/_VisionProtocol/TestingPlayground/Filip/Visors/C_Visors.Q_Active` (`/Game/_VisionProtocol/TestingPlayground/Filip/Visors/QuantumVisor/SC_Quantum.Player Visor` (`self.SC_Quantum`)))
    (set `/Game/_VisionProtocol/TestingPlayground/Filip/Visors/QuantumVisor/SC_Quantum.Q_Hidden` true (`self.SC_Quantum`))
    (`self.SetActorHiddenInGame` false)))

(event `HideNiagara`
  (`/Engine/EditorBlueprintResources/StandardMacros.IsValid` (stale `self.Box.OnComponentHit` _returnvalue)
    (:`Is Valid`
      (`SceneComponent.SetHiddenInGame` (stale `self.Box.OnComponentHit` _returnvalue) true true))))

(event `UnhideNiagara`
  (`/Engine/EditorBlueprintResources/StandardMacros.IsValid` (stale `self.Box.OnComponentHit` _returnvalue)
    (:`Is Valid`
      (`SceneComponent.SetHiddenInGame` (stale `self.Box.OnComponentHit` _returnvalue) false true))))

(event `self.Box.OnComponentHit`
  (params (HitComponent :type "PrimitiveComponent Object Reference") (OtherActor :type "Actor Object Reference") (OtherComp :type "PrimitiveComponent Object Reference") (NormalImpulse :type "Vector Structure") (Hit :type "HitResult Structure (by ref)"))
  (`PrimitiveComponent.SetCollisionEnabled` (`self.Box`) "NoCollision")
  (`SceneComponent.SetHiddenInGame` (`self.StaticMesh`) true false)
  (bind _returnvalue (`NiagaraFunctionLibrary.SpawnSystemAtLocation` "/Game/_VisionProtocol/TestingPlayground/Filip/Urojony_Smok/Efekty/NS_VenomAttack.NS_VenomAttack" Hit_Location))
  (if (not (`/Game/_VisionProtocol/TestingPlayground/Filip/Visors/C_Visors.Q_Active` (`/Game/_VisionProtocol/TestingPlayground/Filip/Visors/QuantumVisor/SC_Quantum.Player Visor` (`self.SC_Quantum`))))
    (`SceneComponent.SetHiddenInGame` _returnvalue true true))
  (`|ExecutionSequence`
    (:`then_0`
      (`KismetSystemLibrary.Delay` 7.0)
      (`ActorComponent.K2_DestroyComponent` _returnvalue)
      (`self.K2_DestroyActor`))
    (:`then_1`
      (`SceneComponent.K2_SetWorldRotation` :`self` (`self.AcidArea`))
      (if (<= (`KismetMathLibrary.Vector_Distance` (`self.K2_GetActorLocation`) (`self.K2_GetActorLocation` (`GameplayStatics.GetPlayerCharacter` 0))) 100.0)
        (`self.ShortCut`)))))

(event `AcidDmg`
  (message `/Game/_VisionProtocol/Core/DMG-HP/BPI_Damageable.TakeDamage` (stale `self.AcidArea.OnComponentBeginOverlap` OtherActor) 1.0))

(event `ShortCut`
  (bind _returnvalue (`KismetSystemLibrary.K2_SetTimerDelegate` (delegate `AcidDmg`) 0.1 true :!label _label))
  (`KismetSystemLibrary.PrintString` "Gracz w srodku"))

(event `self.AcidArea.OnComponentBeginOverlap`
  (params (OverlappedComponent :type "PrimitiveComponent Object Reference") (OtherActor :type "Actor Object Reference") (OtherComp :type "PrimitiveComponent Object Reference") (OtherBodyIndex :type Integer) (bFromSweep :type Boolean) (SweepResult :type "HitResult Structure (by ref)"))
  (if (== (`GameplayStatics.GetObjectClass` OtherActor) (`self.PlayerRef`))
    (goto _label)))

(event `self.AcidArea.OnComponentEndOverlap`
  (params (OverlappedComponent :type "PrimitiveComponent Object Reference") (OtherActor :type "Actor Object Reference") (OtherComp :type "PrimitiveComponent Object Reference") (OtherBodyIndex :type Integer))
  (if (== (`GameplayStatics.GetObjectClass` OtherActor) (`self.PlayerRef`))
    (`KismetSystemLibrary.K2_ClearAndInvalidateTimerHandle` (stale `ShortCut` _returnvalue))
    (`KismetSystemLibrary.PrintString` "Nie ma gracza")))

(fn `UserConstructionScript`)
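; Spawned quantum object, apparently for the Smok (dragon) encounter, that damages the player on contact before becoming an interactable, moveable weighted prop.
; A looping timer traces vertically from the mesh until it hits a non-"Smok" actor; that or a trigger overlap enables the quantum flags and destroys the damage trigger.
; Quantum state syncs with the player's QVisor status.
; A second, never-cleared timer keeps forcing the mesh to block WorldStatic.
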(event `BetterTick`
  (bind _returnvalue (`SceneComponent.K2_GetComponentLocation` (`self.StaticMesh`)))
  (bind (_outhit _returnvalue_2) (`KismetSystemLibrary.LineTraceSingleForObjects` :`Start` _returnvalue :`End` (+ _returnvalue (`KismetMathLibrary.MakeVector` 0.0 0.0 (`self.Z_Level`))) :`ObjectTypes` (`|MakeArray` "ObjectTypeQuery1" "ObjectTypeQuery2" :!type "EObjectTypeQuery Enum") :`DrawDebugType` "ForDuration"))
  (if _returnvalue_2
    (if (not (`self.ActorHasTag` (`.HitActor` (`GameplayStatics.BreakHitResult` _outhit)) "Smok"))
      (`self.ShortCut`)
      (`KismetSystemLibrary.K2_ClearAndInvalidateTimerHandle` (stale `self.ReceiveBeginPlay` _returnvalue)))))

(event `self.ReceiveBeginPlay`
  (bind _sc_quantum (`self.SC_Quantum`))
  (bind _returnvalue (`KismetSystemLibrary.K2_SetTimerDelegate` (delegate `BetterTick`) 0.1 true))
  (`KismetSystemLibrary.K2_SetTimerDelegate` (delegate `KillMyPc`) 0.1 true)
  (bind _activated (message `/Game/_VisionProtocol/TestingPlayground/Filip/Urojony_Smok/BPI_ToPlayer.Get Q Visor Status` (`GameplayStatics.GetPlayerCharacter` 0)))
  (if _activated
    (`/Game/_VisionProtocol/Core/Visors/Quantovisor/SC_Quantum.Q Activated` _sc_quantum)
    (`/Game/_VisionProtocol/Core/Visors/Quantovisor/SC_Quantum.Refresh` _sc_quantum)))

(event `KillMyPc`
  ;[1 1 1] Update Collision channel
  (`PrimitiveComponent.SetCollisionResponseToChannel` (`self.StaticMesh`) "ECC_WorldStatic" "ECR_Block"))

(event `self.DmgTrigger.OnComponentBeginOverlap`
  (params (OverlappedComponent :type "PrimitiveComponent Object Reference") (OtherActor :type "Actor Object Reference") (OtherComp :type "PrimitiveComponent Object Reference") (OtherBodyIndex :type Integer) (bFromSweep :type Boolean) (SweepResult :type "HitResult Structure (by ref)"))
  (bind _dmgtrigger (`self.DmgTrigger`))
  (bind _sc_quantum (`self.SC_Quantum`))
  (bind _sc_quantum_2 (`self.SC_Quantum`))
  (if (not (== OtherActor self))
    (if (== (`GameplayStatics.GetObjectClass` OtherActor) (`self.PlayerRefSoft`))
      (set `/Game/_VisionProtocol/Core/Visors/Quantovisor/SC_Quantum.Q_Interactable` true (`self.SC_Quantum`))
      (message `/Game/_VisionProtocol/Core/DMG-HP/BPI_Damageable.TakeDamage` OtherActor 20.0)
      (else
        (set `/Game/_VisionProtocol/Core/Visors/Quantovisor/SC_Quantum.Q_Interactable` true _sc_quantum :!label _label)))
    (set `/Game/_VisionProtocol/Core/Visors/Quantovisor/SC_Quantum.QF_Moveable` true _sc_quantum)
    (`BlueprintGameplayTagLibrary.AddGameplayTag` (`/Game/_VisionProtocol/Core/Visors/Quantovisor/SC_Quantum.GTC` _sc_quantum_2) (`self.WeightTag`))
    (bind _activated (message `/Game/_VisionProtocol/TestingPlayground/Filip/Urojony_Smok/BPI_ToPlayer.Get Q Visor Status` (`GameplayStatics.GetPlayerCharacter` 0)))
    (if _activated
      (`/Game/_VisionProtocol/Core/Visors/Quantovisor/SC_Quantum.Refresh` _sc_quantum_2))
    (`/Engine/EditorBlueprintResources/StandardMacros.IsValid` _dmgtrigger
      (:`Is Valid`
        (`ActorComponent.K2_DestroyComponent` _dmgtrigger)))))

(event `ShortCut`
  (goto _label))

(fn `UserConstructionScript`)
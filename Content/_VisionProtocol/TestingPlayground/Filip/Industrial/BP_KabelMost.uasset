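; BP_KabelMost is a test-playground industrial actor, by name a cable bridge piece, that destroys itself on any TakeDamage call.
; Its other health functions are stubs returning zero or false, so no health is tracked.
; The Box overlap casts to BP_DragonbloodKatana but does nothing afterwards.
; Debug prints and creation of an InduMost level sequence player are left unconnected, so the sequence never plays from here.
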(event `self.ReceiveActorBeginOverlap`
  (params (OtherActor :type "Actor Object Reference")))

(event `self.Box.OnComponentBeginOverlap`
  (params (OverlappedComponent :type "PrimitiveComponent Object Reference") (OtherActor :type "Actor Object Reference") (OtherComp :type "PrimitiveComponent Object Reference") (OtherBodyIndex :type Integer) (bFromSweep :type Boolean) (SweepResult :type "HitResult Structure (by ref)"))
  (cast `/Game/_VisionProtocol/Core/Melee/Weapons/BP_DragonbloodKatana` OtherActor))

(fn `GetCurrentHealth`
  (returns (Health :type "Float (double-precision)"))
  (return 0.0))

(fn `GetMaxHealth`
  (returns (MaxHealth :type "Float (double-precision)"))
  (return 0.0))

(fn `Heal`
  (params (HP_Amount :type "Float (double-precision)"))
  (returns (`New Health` :type "Float (double-precision)"))
  (return 0.0))

(fn `IsDead`
  (returns (Dead :type Boolean))
  (return false))

(fn `TakeDamage`
  (params (Amount :type "Float (double-precision)"))
  (returns (`Was Damaged` :type Boolean))
  (`self.K2_DestroyActor`)
  (return false))

(fn `UserConstructionScript`)
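; BP_ProjectileCube is a test turret that the player toggles on and off through interaction, with a prompt that reflects its current state.
; A looping timer set on BeginPlay fires StepsNoise every ShootDelay, which, despite its name, spawns the Projectile while Activated.
; Projectiles take the cube's rotation and scale, but spawn at a fixed world-space +X offset rather than along its forward vector.
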(event `self.ReceiveBeginPlay`
  (`KismetSystemLibrary.K2_SetTimerDelegate` (delegate `Steps Noise`) (`self.ShootDelay`) true true 2.0))

(event `Steps Noise`
  (bind (_returnvalue_location _returnvalue_rotation _returnvalue_scale) (`KismetMathLibrary.BreakTransform` (`self.GetTransform`)))
  (if (`self.Activated`)
    (`|SpawnActorFromClass` (`self.Projectile`) (`KismetMathLibrary.MakeTransform` (+ _returnvalue_location (100.0 0.0 0.0)) _returnvalue_rotation _returnvalue_scale) "Undefined" "MultiplyWithRoot" self null)))

(event `self.Interact`
  (params (Interactor :type "Actor Object Reference") (InteracteeComponent :type "PrimitiveComponent Object Reference"))
  (set `self.Activated` (not (`self.Activated`))))

(fn `GetInteractionName`
  (returns (InteractionName :type Text))
  (return (`KismetMathLibrary.SelectText` "Deactivate turret" "Activate turret" (`self.Activated`))))

(fn `GetIsInteractKeyWidgetVisible`
  (returns (IsInteractKeyWidgetVisible :type Boolean))
  (return true))

(fn `UserConstructionScript`)